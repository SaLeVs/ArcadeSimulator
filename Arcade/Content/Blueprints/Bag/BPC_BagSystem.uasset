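; Player component that manages a carried coin bag, used to collect coins from machines and drop the bag off.
; AddBag and RemoveBag track the held bag and toggle the bag's Enhanced Input mapping context, with removal destroying the bag actor.
; Use input line-traces from the camera to take one coin from a BP_BuildMachineMaster while below capacity.
; Put-down input traces for a component tagged DeliverBagBox to remove the bag.
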(event Custom|AddBag
  (params (bagRef :type Actor%20Object%20Reference))
  ;[1 1 1] Add Bag on Hand
  (Variables|Default|SetBP_BagRef bagRef)
  (Variables|Default|SetisWithBag true)
  (Input|AddMappingContext (PlayerController|LocalPlayerSubsystems|GetEnhancedInputLocalPlayerSubsystem (Game|GetPlayerController 0)) "/Game/Inputs/InputsBag/IMC_Bag.IMC_Bag" 0 "(bIgnoreAllPressedKeysUntilRelease=True,bForceImmediately=False,bNotifyUserSettings=False)"))

(event Custom|RemoveBag
  ;[1 1 1] Remove Bag on Hand
  (Variables|Default|SetisWithBag false)
  (Actor|DestroyActor (Variables|Default|GetBP_BagRef))
  (Variables|Default|SetBP_BagRef 0)
  (Default|RemoveItemonHand (Variables|Default|GetBP_Player))
  (Input|RemoveMappingContext (PlayerController|LocalPlayerSubsystems|GetEnhancedInputLocalPlayerSubsystem (Game|GetPlayerController 0)) "/Game/Inputs/InputsBag/IMC_Bag.IMC_Bag" "(bIgnoreAllPressedKeysUntilRelease=True,bForceImmediately=False,bNotifyUserSettings=False)"))

(event Input|EnhancedActionEvents|EnhancedInputActionIA_PutDownBag
  (params (ActionValue :type Boolean) (ElapsedSeconds :type Float%20%28double-precision%29) (TriggeredSeconds :type Float%20%28double-precision%29) (InputAction :type Input%20Action%20Object%20Reference :default "/Game/Inputs/InputsBag/IA_PutDownBag.IA_PutDownBag"))
  (bind _camera (Variables|Default|GetCamera))
  (bind _returnvalue (Transformation|GetWorldTransform _camera))
  ;[1 1 1] Put the Bag Away
  (:Started
    (bind (_outhit _returnvalue_2) (Collision|LineTraceByChannel (.location _returnvalue) (+ (.location _returnvalue) (* (Math|Vector|GetForwardVector (.rotation _returnvalue)) 7e+02)) "TraceTypeQuery1" false 0 "ForDuration" true "(R=0.000000,G=0.235957,B=1.000000,A=1.000000)" "(R=0.608986,G=0.566361,B=1.000000,A=1.000000)"))
    (if _returnvalue_2
      (if (Components|ComponentHasTag (.HitComponent (Collision|BreakHitResult _outhit)) "DeliverBagBox")
        (CallFunction|RemoveBag)))))

(event Input|EnhancedActionEvents|EnhancedInputActionIA_UseBag
  (params (ActionValue :type Boolean) (ElapsedSeconds :type Float%20%28double-precision%29) (TriggeredSeconds :type Float%20%28double-precision%29) (InputAction :type Input%20Action%20Object%20Reference :default "/Game/Inputs/InputsBag/IA_UseBag.IA_UseBag"))
  (bind _camera (Variables|Default|GetCamera))
  (bind _returnvalue (Transformation|GetWorldTransform _camera))
  ;[1 1 1] Interact with Machine
  (:Started
    (if (< (Variables|Default|GetcoinsInBag) (Variables|Default|GetmaxCoinsInBag))
      (bind (_outhit _returnvalue_2) (Collision|LineTraceByChannel (.location _returnvalue) (+ (.location _returnvalue) (* (Math|Vector|GetForwardVector (.rotation _returnvalue)) 7e+02)) "TraceTypeQuery1" false 0 "ForDuration" true "(R=0.546875,G=0.093750,B=1.000000,A=1.000000)" "(R=1.000000,G=0.224885,B=0.855494,A=1.000000)")) ; Can Add More Coins
      (if _returnvalue_2
        (bind _asbp_build_machine_master (Utilities|Casting|CastToBP_BuildMachineMaster (.HitActor (Collision|BreakHitResult _outhit))))
        (bind _takencoin (Default|PlayerGetCoins _asbp_build_machine_master))
        (if _takencoin
          (Variables|Default|SetcoinsInBag (+ (Variables|Default|GetcoinsInBag) 1)) ; Taken one Coin
          (else
            (Development|PrintString "Empty Machine") ; No more coins in Machine
          ))))))

(event EventBeginPlay
  ;[1 1 1] Get Camera
  (bind _asbp_player (Utilities|Casting|CastToBP_Player (Components|GetOwner)))
  (Variables|Default|SetBP_Player _asbp_player)
  (Variables|Default|SetCamera (Variables|/Game/Blueprints/Player/BP_Player.BP_Player_C|GetCamera _asbp_player)))