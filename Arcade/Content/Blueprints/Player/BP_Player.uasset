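; BP_Player is the player character, handling movement, camera look, jumping and interaction with world objects.
; On BeginPlay it adds the IMC_PlayerMovement Enhanced Input context, whose actions drive those controls.
; While the hands are empty, interact line-traces forward from the camera, with debug drawing, and sends InteractMessage to hit actors implementing BPI_InteractAction.
; Two functions set and clear the held-item flag that gates interaction.
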(event Input|EnhancedActionEvents|EnhancedInputActionIA_PlayerCam
  (params (ActionValue :type Vector%202D%20Structure) (ElapsedSeconds :type Float%20%28double-precision%29) (TriggeredSeconds :type Float%20%28double-precision%29) (InputAction :type Input%20Action%20Object%20Reference :default "/Game/Inputs/InputsPlayerMove/IA_PlayerCam.IA_PlayerCam"))
  ;[0.8714 0.03434 0.03434] Cam Player Control
  (Pawn|Input|AddControllerPitchInput (.y ActionValue))
  (Pawn|Input|AddControllerYawInput (.x ActionValue)))

(event Input|EnhancedActionEvents|EnhancedInputActionIA_PlayerJump
  (params (ActionValue :type Boolean) (ElapsedSeconds :type Float%20%28double-precision%29) (TriggeredSeconds :type Float%20%28double-precision%29) (InputAction :type Input%20Action%20Object%20Reference :default "/Game/Inputs/InputsPlayerMove/IA_PlayerJump.IA_PlayerJump"))
  ;[0.8714 0.03434 0.03434] Movement Player Control
  (:Triggered
    (Character|Jump))
  (:Completed
    (Character|StopJumping)))

(event Input|EnhancedActionEvents|EnhancedInputActionIA_PlayerMove
  (params (ActionValue :type Vector%202D%20Structure) (ElapsedSeconds :type Float%20%28double-precision%29) (TriggeredSeconds :type Float%20%28double-precision%29) (InputAction :type Input%20Action%20Object%20Reference :default "/Game/Inputs/InputsPlayerMove/IA_PlayerMove.IA_PlayerMove"))
  ;[0.8714 0.03434 0.03434] Movement Player Control
  (Pawn|Input|AddMovementInput (Transformation|GetActorRightVector) (.x ActionValue) false)
  (Pawn|Input|AddMovementInput (Transformation|GetActorForwardVector) (.y ActionValue) false))

(event Input|EnhancedActionEvents|EnhancedInputActionIA_Interactable
  (params (ActionValue :type Boolean) (ElapsedSeconds :type Float%20%28double-precision%29) (TriggeredSeconds :type Float%20%28double-precision%29) (InputAction :type Input%20Action%20Object%20Reference :default "/Game/Inputs/InputsPlayerMove/IA_Interactable.IA_Interactable"))
  (bind _camera (Variables|Default|GetCamera))
  (bind _returnvalue (Transformation|GetWorldTransform _camera))
  (:Started
    (if (not (Variables|Default|GethaveItemOnHand))
      (bind _outhit (Collision|LineTraceByChannel (.location _returnvalue) (+ (.location _returnvalue) (* (Math|Vector|GetForwardVector (.rotation _returnvalue)) 7e+02)) "TraceTypeQuery1" false 0 "ForDuration"))
      (if (Utilities|DoesObjectImplementInterface (.HitActor (Collision|BreakHitResult _outhit)) "/Game/Blueprints/Interfaces/BPI_InteractAction.BPI_InteractAction_C")
        (Class|BPIInteractAction|Interact(Message) (.HitActor (Collision|BreakHitResult _outhit)) self)))))

(event EventBeginPlay
  ;[0.8714 0.03434 0.03434] Adding Maping context for Player
  (bind _asplayer_controller (Utilities|Casting|CastToPlayerController (Pawn|GetController)))
  (Utilities|IsValid (PlayerController|LocalPlayerSubsystems|GetEnhancedInputLocalPlayerSubsystem _asplayer_controller)
    (:Is%20Valid
      (Input|AddMappingContext (PlayerController|LocalPlayerSubsystems|GetEnhancedInputLocalPlayerSubsystem _asplayer_controller) "/Game/Inputs/InputsPlayerMove/IMC_PlayerMovement.IMC_PlayerMovement" 0 "(bIgnoreAllPressedKeysUntilRelease=True,bForceImmediately=False,bNotifyUserSettings=False)"))))

(fn ConstructionScript)

(fn AddItemonHand
  (Variables|Default|SethaveItemOnHand true))

(fn RemoveItemonHand
  (Variables|Default|SethaveItemOnHand false))