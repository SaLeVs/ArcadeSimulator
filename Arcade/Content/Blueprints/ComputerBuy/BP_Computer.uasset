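; Interactable computer that seats the player at a screen widget, in a folder suggesting an in-game buying station.
; Interact saves the player's transform, teleports them to the construction-placed Arrow and disables capsule collision.
; For player 0, it swaps Enhanced Input contexts, shows the cursor, focuses the widget and blends the view to the computer.
; BPCComputerSystem's left-PC event restores position, collision, movement input and camera.
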(event Custom|PlayerExitPc
  (bind _returnvalue (Game|GetPlayerController 0))
  (bind _bp_player (Variables|Default|GetBp%20Player))
  (bind _returnvalue_2 (PlayerController|LocalPlayerSubsystems|GetEnhancedInputLocalPlayerSubsystem _returnvalue))
  (Input|RemoveMappingContext _returnvalue_2 "/Game/Inputs/InputsComputer/IMC_PlayerOnComputer.IMC_PlayerOnComputer" "(bIgnoreAllPressedKeysUntilRelease=True,bForceImmediately=False,bNotifyUserSettings=False)")
  (Input|AddMappingContext _returnvalue_2 "/Game/Inputs/InputsPlayerMove/IMC_PlayerMovement.IMC_PlayerMovement" 0 "(bIgnoreAllPressedKeysUntilRelease=True,bForceImmediately=False,bNotifyUserSettings=False)")
  (Transformation|SetWorldTransform (Variables|/Script/Engine.Actor|GetRootComponent (Variables|Default|GetBp%20Player)) (Math|Transform|MakeTransform (Variables|Default|GetplayerLastLocation) (Variables|Default|GetplayerLastRotation) "1.000000,1.000000,1.000000") false false) ; Teletransport player
  (Collision|SetCollisionEnabled (Variables|/Script/Engine.Character|GetCapsuleComponent _bp_player) "QueryAndPhysics") ; player can walk on ground
  (Default|RemoveItemonHand _bp_player)
  (Utilities|IsValid (Game|GetPlayerController 0)
    (:Is%20Valid
      (Input|SetInputModeGameOnly (Variables|Default|GetPlayerController) false)
      (Variables|/Script/Engine.PlayerController|SetbShowMouseCursor (Variables|Default|GetPlayerController) false)
      (Game|Player|SetViewTargetwithBlend (Variables|Default|GetPlayerController) (Game|GetPlayerCharacter 0) 0.0 "VTBlend_Linear" 0.0 false))))

(event EventInteract
  (params (bpPlayer :type BP%20Player%20Object%20Reference))
  (bind _returnvalue (Game|GetPlayerController 0))
  (bind _returnvalue_2 (Game|GetPlayerCharacter 0))
  (bind _arrow (Variables|Default|GetArrow))
  (bind _returnvalue_3 (Transformation|GetWorldTransform _arrow))
  (bind _returnvalue_4 (PlayerController|LocalPlayerSubsystems|GetEnhancedInputLocalPlayerSubsystem _returnvalue))
  (Variables|Default|SetBp%20Player bpPlayer)
  (Default|AddItemonHand bpPlayer)
  (Utilities|FlowControl|Sequence
    (:then_0
      (Variables|Default|SetplayerLastLocation (.location (Transformation|GetWorldTransform (Variables|/Script/Engine.Actor|GetRootComponent (Variables|Default|GetBp%20Player)))))
      (Variables|Default|SetplayerLastRotation (.rotation (Transformation|GetWorldTransform (Variables|/Script/Engine.Actor|GetRootComponent (Variables|Default|GetBp%20Player)))))
      (Transformation|SetWorldTransform (Variables|/Script/Engine.Actor|GetRootComponent (Variables|Default|GetBp%20Player)) (Math|Transform|MakeTransform (.location _returnvalue_3) (.rotation _returnvalue_3) "1.000000,1.000000,1.000000") false false) ; Teletransport player
      (Collision|SetCollisionEnabled (Variables|/Script/Engine.Character|GetCapsuleComponent (Variables|Default|GetBp%20Player)) "NoCollision") ; Allow player enter on the groud
      (if (== (Variables|Default|GetBp%20Player) _returnvalue_2)
        (Pawn|SetControlRotation (Game|GetPlayerController 0) (Transformation|GetActorRotation _returnvalue_2)) ; Set player to look foward
        (Variables|/Script/Engine.MovementComponent|SetVelocity (Variables|/Script/Engine.Character|GetCharacterMovement _returnvalue_2) "0, 0, 0")
        (Input|RemoveMappingContext _returnvalue_4 "/Game/Inputs/InputsPlayerMove/IMC_PlayerMovement.IMC_PlayerMovement" "(bIgnoreAllPressedKeysUntilRelease=True,bForceImmediately=False,bNotifyUserSettings=False)") ; Switch the mapping context for cashier
        (Input|AddMappingContext _returnvalue_4 "/Game/Inputs/InputsComputer/IMC_PlayerOnComputer.IMC_PlayerOnComputer" 0 "(bIgnoreAllPressedKeysUntilRelease=True,bForceImmediately=False,bNotifyUserSettings=False)")
        (Utilities|IsValid self
          (:Is%20Valid
            (bind _output_get (Variables|Default|SetPlayerController (Game|GetPlayerController 0)))
            (Input|SetInputModeGameandUI _output_get (UserInterface|GetUserWidgetObject (Variables|Default|GetWidget)) "DoNotLock" true false)
            (Variables|/Script/Engine.PlayerController|SetbShowMouseCursor (Variables|Default|GetPlayerController) true)
            (Game|Player|SetViewTargetwithBlend (Variables|Default|GetPlayerController) self 0.0 "VTBlend_Linear" 0.0 false)))))
    (:then_1
      (EventDispatchers|BindEventtoOnPlayerLeftPc (Variables|/Game/Blueprints/Player/BP_Player.BP_Player_C|GetBPC_ComputerSystem (Variables|Default|GetBp%20Player)) (delegate Custom|PlayerExitPc)))))

(fn ConstructionScript
  (Transformation|SetRelativeTransform (Variables|Default|GetArrow) (Variables|Default|GetteleportLocation) false false))