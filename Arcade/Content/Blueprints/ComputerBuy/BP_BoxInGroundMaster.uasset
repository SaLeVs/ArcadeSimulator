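; Master Blueprint for a box on the ground that the player picks up by interacting with it.
; Interact prints a debug "Hello", then proceeds only if the player's hands are empty, setting the player's HaveBoxInHands flag.
; It swaps itself for a BP_BoxInHand spawned at the player's BoxInHandPoint, which receives the player reference, runs Setup and attaches there before the ground box destroys itself.
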(event EventInteract
  (params (bpPlayer :type BP%20Player%20Object%20Reference))
  ;[1 1 1] Touched player, spawn a box in hand
  (Development|PrintString "Hello")
  (bind _output_get (Variables|Default|SetBP_Player bpPlayer))
  (if (not (Variables|/Game/Blueprints/Player/BP_Player.BP_Player_C|GethaveBoxInHands _output_get)) ; If hands empty
    (Variables|/Game/Blueprints/Player/BP_Player.BP_Player_C|SethaveBoxInHands (Variables|Default|GetBP_Player) true) ; Now, have box in hands
    (bind _returnvalue (Game|SpawnActorfromClass "/Game/Blueprints/Itens/BP_BoxInHand.BP_BoxInHand_C" (Transformation|GetWorldTransform (Variables|/Game/Blueprints/Player/BP_Player.BP_Player_C|GetBoxInHandPoint (Variables|Default|GetBP_Player))) "AlwaysSpawn" "MultiplyWithRoot" 0 0)) ; Spawn Box
    (Variables|/Game/Blueprints/Itens/BP_BoxInHand.BP_BoxInHand_C|SetBP_Player _returnvalue (Variables|Default|GetBP_Player)) ; Pass ref to box
    (Default|Setup _returnvalue)
    (Transformation|AttachComponentToComponent _returnvalue (Variables|/Game/Blueprints/Player/BP_Player.BP_Player_C|GetBoxInHandPoint (Variables|Default|GetBP_Player)) "None" "SnapToTarget" "SnapToTarget" "KeepRelative" true)
    (Actor|DestroyActor) ; Destroy this obj
  ))

(fn ConstructionScript)