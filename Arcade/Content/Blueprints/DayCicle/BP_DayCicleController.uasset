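; Day cycle controller that runs the arcade's open/closed state, in-game clock and day count.
; The sign's TriggerDay toggles the arcade by day; at night it shows the end-day widget once no NPCs remain.
; Opening starts a looping one-second timer that advances minutes until night forces closing, broadcasting changes through dispatchers.
; NextDay increments the day, resets the clock and saves through the GameInstance, which also supplies the saved day on BeginPlay.
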(event Custom|PassDayTime
  ;[1 1 1] Change hour
  (if (>= (Variables|Default|GetcurrentDayTimeInMinutes) (Variables|Default|GetmaxDayTimeInMinutes)) ; if true = no more time, night time\nif  false = day, can play
    (CallFunction|FinishDay)
    (else
      (Variables|Default|SetcurrentDayTimeInMinutes (+ (Variables|Default|GetcurrentDayTimeInMinutes) 1)) ; have time to play
      (Default|CallOnTimeChanged))))

(event Custom|NextDay
  ;[1 1 1] Change Day
  (Utilities|FlowControl|Sequence
    (:then_0
      (Variables|Default|SetcurrentDay (+ (Variables|Default|GetcurrentDay) 1)) ; Add Day
      (Default|CallOnDayChanged))
    (:then_1
      (Variables|Default|SetisDay true) ; Reset to next day
      (Variables|Default|SetisArcadeOpen false)
      (Variables|Default|SetcurrentDayTimeInMinutes 0) ; Reset hour time
      (Default|CallOnTimeChanged)
      (Default|CallOnDayStateChanged true false))
    (:then_2
      (Class|BPISaveGame|SaveAll(Message) (Game|GetGameInstance) true))))

(event Custom|TriggerDay
  ;[1 1 1] Interact with sign
  (if (Variables|Default|GetisDay) ; if day = open\nif night = finish day, save and next day
    (if (Variables|Default|GetisArcadeOpen) ; if closed = open\nif open = close
      (CallFunction|CloseArcade) ; Stop Spawning, but timer still going
      (else
        (CallFunction|OpenArcade) ; Start spawning, start timer
      ))
    (else
      (bind _returnvalue (Actor|GetActorOfClass "/Game/Blueprints/AI/BP_NpcSpawnerController.BP_NpcSpawnerController_C"))
      (bind _thereisanynpc (Default|CheckAnyNPCinArcade _returnvalue))
      (if (not _thereisanynpc) ; false = no npc and night
        (CallFunction|CreateFinishDayWB)))))

(event Custom|OpenArcade
  ;[1 1 1] Start Day (start spawn npcs)
  (Variables|Default|SetisArcadeOpen true)
  (bind _returnvalue (Utilities|Time|SetTimerbyEvent (delegate Custom|PassDayTime) 1.0 true))
  (Variables|Default|SetpassDayTimeTimer _returnvalue)
  (Default|CallOnDayStateChanged (Variables|Default|GetisDay) (Variables|Default|GetisArcadeOpen)))

(event Custom|CloseArcade
  ;[1 1 1] Close arcade (stop spawning npcs)
  (Variables|Default|SetisArcadeOpen false)
  (Default|CallOnDayStateChanged (Variables|Default|GetisDay) (Variables|Default|GetisArcadeOpen)))

(event Custom|FinishDay
  ;[1 1 1] Time of the day ended
  (CallFunction|CloseArcade)
  (Variables|Default|SetisDay false) ; set to night
  (Utilities|Time|ClearandInvalidateTimerbyHandle (Variables|Default|GetpassDayTimeTimer)) ; Stop time Timer
  (Default|CallOnDayStateChanged false false))

(event EventBeginPlay
  (Utilities|FlowControl|Delay 0.1) ; delay to some refs
  (CallFunction|UseDaySave))

(fn ConstructionScript)

(fn UseDaySave
  (bind _savegamedata (Class|BPISaveGame|GetGameData(Message) (Game|GetGameInstance)))
  (Utilities|IsValid _savegamedata
    (:Is%20Valid
      (Variables|Default|SetcurrentDay (Variables|/Game/Blueprints/SaveLoad/BP_SaveLoadGame.BP_SaveLoadGame_C|GetdaySave _savegamedata))
      (Default|CallOnDayChanged))))

(fn CreateFinishDayWB
  (bind _returnvalue (Game|GetPlayerController 0))
  (bind _returnvalue_2 (UserInterface|CreateWidget "/Game/Widgets/UI/WB_EndDay.WB_EndDay_C" _returnvalue))
  (UserInterface|Viewport|AddtoViewport _returnvalue_2 0)
  (Input|SetInputModeUIOnly _returnvalue _returnvalue_2 "DoNotLock" false)
  (Variables|/Script/Engine.PlayerController|SetbShowMouseCursor (Game|GetPlayerController 0) true))