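; Interactable arcade open/closed sign that lets the player trigger the day cycle on BP_DayCicleController.
; Interacting plays a click sound through the game instance and calls TriggerDay.
; Day-state change events toggle between the open/closed and next-day meshes, showing next-day at night only if the NPC spawner reports the arcade empty at that moment.
; Tick polls the controller's IsArcadeOpen into AnimDayCicle.
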(event Custom|DayStateChanged
  (params (isDay :type Boolean) (isArcadeOpen :type Boolean))
  (if isDay ; true = its day\nfalse = its night
    (Rendering|SetVisibility (Variables|Default|GetNextDayMesh) false false)
    (Rendering|SetVisibility (Variables|Default|GetOpenClosed) true false)
    (else
      (bind _returnvalue (Actor|GetActorOfClass "/Game/Blueprints/AI/BP_NpcSpawnerController.BP_NpcSpawnerController_C"))
      (bind _thereisanynpc (Default|CheckAnyNPCinArcade _returnvalue))
      (if (not _thereisanynpc) ; false = can change day
        (Rendering|SetVisibility (Variables|Default|GetNextDayMesh) true false)
        (Rendering|SetVisibility (Variables|Default|GetOpenClosed) false false)))))

(event EventBeginPlay
  ;[1 1 1] Get Controller ref
  (bind _returnvalue (Actor|GetActorOfClass "/Game/Blueprints/DayCicle/BP_DayCicleController.BP_DayCicleController_C"))
  (bind _output_get (Variables|Default|SetBP_DayCicleController _returnvalue))
  (EventDispatchers|BindEventtoOnDayStateChanged _output_get (delegate Custom|DayStateChanged)))

(event Collision|EventActorBeginOverlap
  (params (OtherActor :type Actor%20Object%20Reference)))

(event EventInteract
  (params (bpPlayer :type BP%20Player%20Object%20Reference))
  (Class|BPIPlaySound|PlaySoundLocation(Message) (Game|GetGameInstance) "/Game/SFX/D4_Open_closed_object/ui_button_simple_click_02_-_2º_Opção.ui_button_simple_click_02_-_2º_Opção" (Transformation|GetActorTransform))
  (Default|TriggerDay (Variables|Default|GetBP_DayCicleController)) ; hit the sign, trigger func
)

(event EventTick
  (params (DeltaSeconds :type Float%20%28single-precision%29))
  ;[1 1 1] Crime
  (bind _bp_dayciclecontroller (Variables|Default|GetBP_DayCicleController)
    (:then
      (Variables|Default|SetanimDayCicle (Variables|/Game/Blueprints/DayCicle/BP_DayCicleController.BP_DayCicleController_C|GetisArcadeOpen _bp_dayciclecontroller)))
    (:else)))

(fn ConstructionScript)