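; BP_Atm is an interactable ATM or cashier station that locks the player in place at a teleport spot.
; Interact moves the player to an Arrow positioned by TeleportLocation, disables capsule collision, and swaps the local player's movement input context for the cashier one.
; It binds to the player's BPCAtmSystem events: exit restores input and collision, while interact line-traces from the camera and only prints the hit component's name.
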(event Custom|OnPlayerLeftCashier
  (bind _returnvalue (Game|GetPlayerController 0))
  (bind _returnvalue_2 (PlayerController|LocalPlayerSubsystems|GetEnhancedInputLocalPlayerSubsystem _returnvalue))
  (Input|RemoveMappingContext _returnvalue_2 "/Game/Inputs/InputsAtm/IMC_PlayerOnCashier.IMC_PlayerOnCashier" "(bIgnoreAllPressedKeysUntilRelease=True,bForceImmediately=False,bNotifyUserSettings=False)")
  (Input|AddMappingContext _returnvalue_2 "/Game/Inputs/InputsPlayerMove/IMC_PlayerMovement.IMC_PlayerMovement" 0 "(bIgnoreAllPressedKeysUntilRelease=True,bForceImmediately=False,bNotifyUserSettings=False)")
  (Collision|SetCollisionEnabled (Variables|/Script/Engine.Character|GetCapsuleComponent (Variables|Default|GetBp%20Player)) "QueryAndPhysics"))

(event Custom|OnPlayerInteractOnCashier
  (bind _bp_player (Variables|Default|GetBp%20Player))
  (bind _camera (Variables|/Game/Blueprints/Player/BP_Player.BP_Player_C|GetCamera _bp_player))
  (bind _returnvalue (Transformation|GetWorldTransform _camera))
  (bind _outhit (Collision|LineTraceByChannel (.location _returnvalue) (+ (.location _returnvalue) (* (Math|Vector|GetForwardVector (.rotation _returnvalue)) 7e+02)) "TraceTypeQuery1" false 0 "ForDuration"))
  (Development|PrintString (Utilities|GetDisplayName (.HitComponent (Collision|BreakHitResult _outhit)))))

(event EventInteract
  (params (bpPlayer :type BP%20Player%20Object%20Reference))
  (bind _returnvalue (Game|GetPlayerController 0))
  (bind _returnvalue_2 (Game|GetPlayerCharacter 0))
  (bind _arrow (Variables|Default|GetArrow))
  (bind _returnvalue_3 (Transformation|GetWorldTransform _arrow))
  (bind _returnvalue_4 (PlayerController|LocalPlayerSubsystems|GetEnhancedInputLocalPlayerSubsystem _returnvalue))
  (Default|AddItemonHand bpPlayer)
  (Variables|Default|SetBp%20Player bpPlayer)
  (Utilities|FlowControl|Sequence
    (:then_0
      (Transformation|SetWorldTransform (Variables|/Script/Engine.Actor|GetRootComponent (Variables|Default|GetBp%20Player)) (Math|Transform|MakeTransform (.location _returnvalue_3) (.rotation _returnvalue_3) "1.000000,1.000000,1.000000") false false)
      (Collision|SetCollisionEnabled (Variables|/Script/Engine.Character|GetCapsuleComponent (Variables|Default|GetBp%20Player)) "NoCollision")
      (if (== (Variables|Default|GetBp%20Player) _returnvalue_2)
        (Pawn|SetControlRotation (Game|GetPlayerController 0) (Transformation|GetActorRotation _returnvalue_2))
        (Variables|/Script/Engine.MovementComponent|SetVelocity (Variables|/Script/Engine.Character|GetCharacterMovement _returnvalue_2) "0, 0, 0")
        (Input|RemoveMappingContext _returnvalue_4 "/Game/Inputs/InputsPlayerMove/IMC_PlayerMovement.IMC_PlayerMovement" "(bIgnoreAllPressedKeysUntilRelease=True,bForceImmediately=False,bNotifyUserSettings=False)")
        (Input|AddMappingContext _returnvalue_4 "/Game/Inputs/InputsAtm/IMC_PlayerOnCashier.IMC_PlayerOnCashier" 0 "(bIgnoreAllPressedKeysUntilRelease=True,bForceImmediately=False,bNotifyUserSettings=False)")))
    (:then_1
      (EventDispatchers|BindEventtoOnPlayerExitCashier (Variables|/Game/Blueprints/Player/BP_Player.BP_Player_C|GetBPC_AtmSystem (Variables|Default|GetBp%20Player)) (delegate Custom|OnPlayerLeftCashier)))
    (:then_2
      (EventDispatchers|BindEventtoOnPlayerInteractinCashier (Variables|/Game/Blueprints/Player/BP_Player.BP_Player_C|GetBPC_AtmSystem (Variables|Default|GetBp%20Player)) (delegate Custom|OnPlayerInteractOnCashier)))))

(fn ConstructionScript
  (Transformation|SetRelativeTransform (Variables|Default|GetArrow) (Variables|Default|GetteleportLocation) false false))