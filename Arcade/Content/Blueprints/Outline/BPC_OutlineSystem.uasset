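; Actor component for BP_Player that outlines the interactable mesh the player looks at.
; A looping timer runs a short visibility line trace from the player camera instead of checking every tick.
; Hit actors implementing BPI_Outline get custom depth enabled on the hit mesh component, tracking the last one so only one is highlighted.
; The outline clears when nothing valid is hit or the player holds an item.
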(event Custom|CheckOutline
  (bind _camera (Variables|Components|GetCamera))
  (bind _returnvalue (Transformation|GetWorldTransform _camera))
  (if (Variables|/Game/Blueprints/Player/BP_Player.BP_Player_C|GethaveItemOnHand (Variables|Default|GetBP_Player))
    (CallFunction|RemoveOutline)
    (else
      (bind _outhit (Collision|LineTraceByChannel (.location _returnvalue) (+ (.location _returnvalue) (* (Math|Vector|GetForwardVector (.rotation _returnvalue)) 2.5e+02)) "TraceTypeQuery1" false 0 "None" true "(R=1.000000,G=0.222171,B=0.740750,A=1.000000)"))
      (Utilities|Casting|CastToBPI_Outline (.HitActor (Collision|BreakHitResult _outhit)) ; only change outline if have interface
        (:then
          (bind _asmesh_component (Utilities|Casting|CastToMeshComponent (.HitComponent (Collision|BreakHitResult _outhit))) ; Have interface
            (:then
              (if (!= (Variables|Default|GetlastObjOutline) _asmesh_component)
                (Utilities|FlowControl|Sequence ; Different obj, change mat
                  (:then_0
                    (CallFunction|RemoveOutline))
                  (:then_1
                    (CallFunction|AddOutline _asmesh_component)))))
            (:CastFailed
              (CallFunction|RemoveOutline :!label _label) ; hit nothing, remove it
            )))
        (:CastFailed
          (goto _label))))))

(event EventBeginPlay
  (Utilities|FlowControl|Sequence
    (:then_0
      (CallFunction|GetCamera))
    (:then_1
      (bind _returnvalue (Utilities|Time|SetTimerbyEvent (delegate Custom|CheckOutline) 0.15 true))
      (Variables|Default|SetCheckOutlineTimer _returnvalue) ; Save if needs to stop
    )))

(fn AddOutline
  (params (meshParam :type Mesh%20Component%20Object%20Reference))
  (bind _output_get (Variables|Default|SetlastObjOutline meshParam))
  (Rendering|SetRenderCustomDepth _output_get true))

(fn RemoveOutline
  (bind _lastobjoutline (Variables|Default|GetlastObjOutline)
    (:then
      (Rendering|SetRenderCustomDepth _lastobjoutline false)
      (Variables|Default|SetlastObjOutline 0))
    (:else)))

(fn GetCamera
  (bind _asbp_player (Utilities|Casting|CastToBP_Player (Components|GetOwner)))
  (Variables|Default|SetBP_Player _asbp_player)
  (Variables|Components|SetCamera (Variables|/Game/Blueprints/Player/BP_Player.BP_Player_C|GetCamera _asbp_player)))