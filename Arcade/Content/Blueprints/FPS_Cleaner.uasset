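; First-person cleaner player Blueprint that washes A_Target actors by painting onto their render targets.
; BeginPlay adds the movement input context, and IA_Wash fires a symmetrical row of camera-forward multi line traces, spaced by brush radius.
; The row follows the camera's right vector, rotated around the view axis by Rotation, like an adjustable flat nozzle.
; Each target hit draws a brush-sized mark at its impact point.
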(event Input|EnhancedActionEvents|EnhancedInputActionIA_Wash
  (params (ActionValue :type Boolean) (ElapsedSeconds :type Float%20%28double-precision%29) (TriggeredSeconds :type Float%20%28double-precision%29) (InputAction :type Input%20Action%20Object%20Reference :default "/Game/Inputs/IA_Wash.IA_Wash"))
  (CallFunction|CreateLineTraces))

(event Collision|EventActorBeginOverlap
  (params (OtherActor :type Actor%20Object%20Reference)))

(event EventTick
  (params (DeltaSeconds :type Float%20%28single-precision%29)))

(event EventBeginPlay
  (Input|AddMappingContext (PlayerController|LocalPlayerSubsystems|GetEnhancedInputLocalPlayerSubsystem (Game|GetPlayerController 0)) "/Game/Inputs/IMC_PlayerMovement.IMC_PlayerMovement" 0 "(bIgnoreAllPressedKeysUntilRelease=True,bForceImmediately=False,bNotifyUserSettings=False)"))

(fn ConstructionScript
  (|CallParentFunction))

(fn OnRepRotation)

(fn CreateLineTraces
  (for _index (range 0 (Variables|Default|GetLength))
    (LocalVariables|SetL-Index _index)
    (Utilities|FlowControl|Sequence
      (:then_0
        (CallFunction|LineTraceforTargets (.Start (Utilities|LineTraceForward (* (Utilities|MakeLineVector) (* (LocalVariables|GetL-Index) (* (Variables|Default|GetBrushRadius) 2.2))) 1.5e+03)) (.End (Utilities|LineTraceForward (* (Utilities|MakeLineVector) (* (LocalVariables|GetL-Index) (* (Variables|Default|GetBrushRadius) 2.2))) 1.5e+03))))
      (:then_1
        (if (!= (LocalVariables|GetL-Index) 0)
          (CallFunction|LineTraceforTargets (.Start (Utilities|LineTraceForward (* (Utilities|MakeLineVector) (* (LocalVariables|GetL-Index) (* (Variables|Default|GetBrushRadius) -2.2))) 1.5e+03)) (.End (Utilities|LineTraceForward (* (Utilities|MakeLineVector) (* (LocalVariables|GetL-Index) (* (Variables|Default|GetBrushRadius) -2.2))) 1.5e+03))))))))

(fn LineTraceforTargets
  (params (Start :type Vector) (End :type Vector))
  (bind _outhits (Collision|MultiLineTraceByChannel Start End "TraceTypeQuery1" false 0 "None"))
  (for _array_element _outhits
    (bind _asa_target (Utilities|Casting|CastToA_Target (.HitActor (Collision|BreakHitResult _array_element))))
    (Default|DrawtoRenderTarget _asa_target (.ImpactPoint (Collision|BreakHitResult _array_element)) (Variables|Default|GetBrushRadius))))