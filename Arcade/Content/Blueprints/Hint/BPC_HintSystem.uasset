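; BPC_HintSystem is an unfinished hint component that looks for hints in front of the player's camera.
; On BeginPlay it caches the owning BP_Player and its camera, then starts a looping 0.1-second timer.
; While DoHintTrace is set, each timer call runs a short, debug-drawn Visibility line trace along the camera's forward vector, avoiding Tick.
; Trace hits currently trigger nothing.
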(event Custom|HintTrace
  (bind _camera (Variables|Default|GetCamera))
  (bind _returnvalue (Transformation|GetWorldTransform _camera))
  (if (Variables|Default|GetdoHintTrace)
    (bind (_outhit _returnvalue_2) (Collision|LineTraceByChannel (.location _returnvalue) (+ (.location _returnvalue) (* (Math|Vector|GetForwardVector (.rotation _returnvalue)) 2.5e+02)) "TraceTypeQuery1" false 0 "ForDuration" true "(R=0.062269,G=0.980104,B=1.000000,A=1.000000)"))
    (if _returnvalue_2
      _)))

(event EventBeginPlay
  (Utilities|FlowControl|Sequence
    (:then_0
      (CallFunction|GetCamera))
    (:then_1
      (bind _returnvalue (Utilities|Time|SetTimerbyEvent (delegate Custom|HintTrace) 0.1 true))
      (Variables|Default|SetHintTraceTimer _returnvalue))))

(event EventTick
  (params (DeltaSeconds :type Float%20%28single-precision%29)))

(fn GetCamera
  (bind _asbp_player (Utilities|Casting|CastToBP_Player (Components|GetOwner)))
  (Variables|Default|SetBP_Player _asbp_player)
  (Variables|Default|SetCamera (Variables|/Game/Blueprints/Player/BP_Player.BP_Player_C|GetCamera _asbp_player)))