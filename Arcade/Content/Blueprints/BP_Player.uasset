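; BP_Player is the player character, handling Enhanced Input movement, camera look and jumping, plus picking up and using a mop.
; On BeginPlay it registers the player movement mapping context.
; If the player has no mop, overlapping a BP_Mop with the capsule destroys it and spawns a replacement attached to MopPoint.
; Pressing and releasing the use input calls MopUseMessage and MopDisuse on the stored mop.
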(event OnComponentBeginOverlap(CapsuleComponent)
  (params (OverlappedComponent :type Primitive%20Component%20Object%20Reference) (OtherActor :type Actor%20Object%20Reference) (OtherComp :type Primitive%20Component%20Object%20Reference) (OtherBodyIndex :type Integer) (bFromSweep :type Boolean) (SweepResult :type Hit%20Result%20Structure%20%28by%20ref%29))
  ;[0.8714 0.03434 0.03434] Player colliding with Mop
  (if (not (Variables|Default|GetIsPlayerHaveMop?))
    (bind _asbp_mop (Utilities|Casting|CastToBP_Mop OtherActor))
    (Actor|DestroyActor _asbp_mop)
    (Variables|Default|SetIsPlayerHaveMop? true)
    (bind _returnvalue (Game|SpawnActorfromClass "/Game/Blueprints/BP_Mop.BP_Mop_C" (Transformation|GetWorldTransform (Variables|Default|GetMopPoint)) "Undefined" "MultiplyWithRoot" 0 0))
    (bind _output_get (Variables|Default|SetMop _returnvalue))
    (Transformation|AttachComponentToComponent _output_get (Variables|Default|GetMopPoint) "None" "SnapToTarget" "SnapToTarget" "KeepRelative" true)))

(event Input|EnhancedActionEvents|EnhancedInputActionIA_PlayerCam
  (params (ActionValue :type Vector%202D%20Structure) (ElapsedSeconds :type Float%20%28double-precision%29) (TriggeredSeconds :type Float%20%28double-precision%29) (InputAction :type Input%20Action%20Object%20Reference :default "/Game/Inputs/IA_PlayerCam.IA_PlayerCam"))
  ;[0.8714 0.03434 0.03434] Cam Player Control
  (Pawn|Input|AddControllerPitchInput (.y ActionValue))
  (Pawn|Input|AddControllerYawInput (.x ActionValue)))

(event Input|EnhancedActionEvents|EnhancedInputActionIA_PlayerJump
  (params (ActionValue :type Boolean) (ElapsedSeconds :type Float%20%28double-precision%29) (TriggeredSeconds :type Float%20%28double-precision%29) (InputAction :type Input%20Action%20Object%20Reference :default "/Game/Inputs/IA_PlayerJump.IA_PlayerJump"))
  ;[0.8714 0.03434 0.03434] Movement Player Control
  (:Triggered
    (Character|Jump))
  (:Completed
    (Character|StopJumping)))

(event Input|EnhancedActionEvents|EnhancedInputActionIA_PlayerMove
  (params (ActionValue :type Vector%202D%20Structure) (ElapsedSeconds :type Float%20%28double-precision%29) (TriggeredSeconds :type Float%20%28double-precision%29) (InputAction :type Input%20Action%20Object%20Reference :default "/Game/Inputs/IA_PlayerMove.IA_PlayerMove"))
  ;[0.8714 0.03434 0.03434] Movement Player Control
  (Pawn|Input|AddMovementInput (Transformation|GetActorRightVector) (.x ActionValue) false)
  (Pawn|Input|AddMovementInput (Transformation|GetActorForwardVector) (.y ActionValue) false))

(event Input|EnhancedActionEvents|EnhancedInputActionIA_PlayerUses
  (params (ActionValue :type Boolean) (ElapsedSeconds :type Float%20%28double-precision%29) (TriggeredSeconds :type Float%20%28double-precision%29) (InputAction :type Input%20Action%20Object%20Reference :default "/Game/Inputs/IA_PlayerUses.IA_PlayerUses"))
  (bind _mop (Variables|Default|GetMop))
  ;[0.8714 0.03434 0.03434] Player Pressing For Pick the Mop
  (:Started
    (Class|BPIMop|MopUse(Message) _mop))
  (:Completed
    (Default|MopDisuse _mop)))

(event Input|EnhancedActionEvents|EnhancedInputActionIA_Wash
  (params (ActionValue :type Boolean) (ElapsedSeconds :type Float%20%28double-precision%29) (TriggeredSeconds :type Float%20%28double-precision%29) (InputAction :type Input%20Action%20Object%20Reference :default "/Game/Inputs/IA_Wash.IA_Wash")))

(event EventBeginPlay
  ;[0.8714 0.03434 0.03434] Adding Maping context for Player
  (bind _asplayer_controller (Utilities|Casting|CastToPlayerController (Pawn|GetController)))
  (Utilities|IsValid (PlayerController|LocalPlayerSubsystems|GetEnhancedInputLocalPlayerSubsystem _asplayer_controller)
    (:Is%20Valid
      (Input|AddMappingContext (PlayerController|LocalPlayerSubsystems|GetEnhancedInputLocalPlayerSubsystem _asplayer_controller) "/Game/Inputs/IMC_PlayerMovement.IMC_PlayerMovement" 0 "(bIgnoreAllPressedKeysUntilRelease=True,bForceImmediately=False,bNotifyUserSettings=False)"))))

(fn ConstructionScript)