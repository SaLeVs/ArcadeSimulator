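; BP_NPC is an AI-driven NPC, apparently an arcade visitor, that shows thought bubbles and occasionally litters.
; A looping timer gives it a small chance to spawn BP_Dirt near a random reachable point around it.
; Helper functions write the state machine index to the AI controller's blackboard and set exclusive animation flags for paying, thumbs-up and game machines.
; Bubble functions show or hide a WB_ToughBubble widget, passing it an index and coin count.
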(event Custom|TrySpawnDirt
  (bind _returnvalue (Transformation|GetActorLocation))
  (bind _randomlocation (AI|Navigation|GetRandomReachablePointinRadius _returnvalue 2e+02 0 0))
  (if (> (Math|Random|RandomIntegerinRange 0 9) 8)
    (Game|SpawnActorfromClass "/Game/Blueprints/Mop/BP_Dirt.BP_Dirt_C" (Math|Transform|MakeTransform (Math|Vector|MakeVector (.x _randomlocation) (.y _randomlocation) (.z (Transformation|GetWorldLocation (Variables|Default|GetTrashSpawnPoint)))) "0, 0, 0" "1.000000,1.000000,1.000000") "AdjustIfPossibleButAlwaysSpawn" "OverrideRootScale" 0 0)))

(event EventBeginPlay
  (CallFunction|ResetBubble)
  (bind _returnvalue (Utilities|Time|SetTimerbyEvent (delegate Custom|TrySpawnDirt) 1e+01 true))
  (Variables|Default|SettrySpawnDirtTimer _returnvalue))

(fn ConstructionScript)

(fn SetStateMachineIndex
  (params (aiController :type Pawn%20Object%20Reference) (intValue :type Integer))
  (Class|BlackboardComponent|SetValueasInt (AI|GetBlackboard (AI|GetAIController aiController)) (Variables|Default|GetstateMachineIndexName) intValue))

(fn ChangeAnim
  (params (indexAnim :type Integer))
  (Utilities|FlowControl|Sequence ; if = 0, just reset
    (:then_0
      (Variables|Default|SetisPay false)
      (Variables|Default|SetisThumbUp false)
      (Variables|Default|SetisArcade false)
      (Variables|Default|SetisClaw false)
      (Variables|Default|SetisPinball false))
    (:then_1
      (if (== indexAnim 1)
        (Variables|Default|SetisPay true)))
    (:then_2
      (if (== indexAnim 2)
        (Variables|Default|SetisThumbUp true)))
    (:then_3
      (if (== indexAnim 3)
        (Variables|Default|SetisArcade true)))
    (:then_4
      (if (== indexAnim 4)
        (Variables|Default|SetisClaw true)))
    (:then_5
      (if (== indexAnim 5)
        (Variables|Default|SetisPinball true)))))

(fn PassValuesforBubble
  (params (indexForBubble :type Integer))
  (Rendering|SetVisibility (Variables|Default|GetThoughtBubble) true false)
  (bind _aswb_tough_bubble (Utilities|Casting|CastToWB_ToughBubble (UserInterface|GetUserWidgetObject (Variables|Default|GetThoughtBubble))))
  (Default|UpdateToughtBubble _aswb_tough_bubble indexForBubble (Variables|Default|GetquantityOfCoins)))

(fn ResetBubble
  (Rendering|SetVisibility (Variables|Default|GetThoughtBubble) false false)
  (bind _aswb_tough_bubble (Utilities|Casting|CastToWB_ToughBubble (UserInterface|GetUserWidgetObject (Variables|Default|GetThoughtBubble))))
  (Default|DisableToughtBubble _aswb_tough_bubble))