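; NPC spawner controller that fills the arcade with customers while it is open and tracks how many are inside.
; It binds to BP_DayCicleController's day-state event to start or clear a looping, randomized-interval spawn timer.
; Each tick spawns a random NPC class under a cap that grows with the current day, incrementing the GameInstance's daily customer count.
; When the last NPC leaves at night, it stops spawning and broadcasts the arcade as closed.
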(event Custom|SpawnNPC
  ;[1 1 1] Spawn npc
  (if (not (>= (Variables|Default|GetspawnedNPCs) (+ (Variables|Default|GetbaseMaxSpawnedNPC) (* (Variables|/Game/Blueprints/DayCicle/BP_DayCicleController.BP_DayCicleController_C|GetcurrentDay (Variables|Default|GetBP_DayCicleController)) (Variables|Default|GetmaxSpawnNPCIncreasePerDay))))) ; true = full\nfalse = can spawn more
    (Game|SpawnActorfromClass (Utilities|Array|Get(acopy) (Variables|Default|GetnpcsToSpawn) (Math|Random|RandomIntegerinRange 0 (- (Utilities|Array|Length (Variables|Default|GetnpcsToSpawn)) 1))) (Transformation|GetWorldTransform (Variables|Default|GetspawnPointNPC)) "AdjustIfPossibleButAlwaysSpawn" "OverrideRootScale" 0 0)
    (Math|Integer|IncrementInt (Variables|Default|GetspawnedNPCs)
      (:%20%20
        (bind _asmy_game_instance (Utilities|Casting|CastToMyGameInstance (Game|GetGameInstance)))
        (Math|Integer|IncrementInt (Variables|/Game/Blueprints/Interfaces/MyGameInstance.MyGameInstance_C|GetthisCustomersDay _asmy_game_instance))))))

(event Custom|OnDayStateChanged
  (params (isDay :type Boolean) (isArcadeOpen :type Boolean))
  (if isArcadeOpen ; true = start timer\nfalse = stop timer
    (bind _returnvalue (Utilities|Time|SetTimerbyEvent (delegate Custom|SpawnNPC) (Math|Random|RandomFloatinRange 9.5 11.0) true))
    (Variables|Default|SetSpawnNPCTimer _returnvalue)
    (else
      (Utilities|Time|ClearandInvalidateTimerbyHandle (Variables|Default|GetSpawnNPCTimer)))))

(event EventBeginPlay
  ;[1 1 1] Bind
  (bind _returnvalue (Actor|GetActorOfClass "/Game/Blueprints/DayCicle/BP_DayCicleController.BP_DayCicleController_C"))
  (bind _output_get (Variables|Default|SetBP_DayCicleController _returnvalue))
  (EventDispatchers|BindEventtoOnDayStateChanged _output_get (delegate Custom|OnDayStateChanged)))

(fn ConstructionScript)

(fn NPCLeaved
  (Math|Integer|DecrementInt (Variables|Default|GetspawnedNPCs)
    (:%20%20
      (bind _thereisanynpc (CallFunction|CheckAnyNPCinArcade))
      (if (and (not _thereisanynpc) (not (Variables|/Game/Blueprints/DayCicle/BP_DayCicleController.BP_DayCicleController_C|GetisDay (Variables|Default|GetBP_DayCicleController)))) ; true = no more npcs and is night
        (Utilities|Time|ClearandInvalidateTimerbyHandle (Variables|Default|GetSpawnNPCTimer)) ; stop spawning npcs
        (Default|CallOnDayStateChanged (Variables|Default|GetBP_DayCicleController) false false) ; need to call to updt openclose obj
      ))))

(fn CheckAnyNPCinArcade
  (if (<= (Variables|Default|GetspawnedNPCs) 0) ; true = no more npcs
    (return false)
    (else
      (return true))))