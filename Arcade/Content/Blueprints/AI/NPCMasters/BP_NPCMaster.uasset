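; BP_NPCMaster is the master NPC Blueprint, providing shared AI-state, animation, thought-bubble and littering behavior.
; Helpers write the state-machine index to the Blackboard and set mutually exclusive animation flags for pay, thumbs-up and machine interactions.
; The thought-bubble widget shows images or token progress, with a looping timer yawing it toward the player until reset.
; Another looping timer occasionally spawns BP_Dirt at random reachable points nearby.
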(event Custom|TrySpawnDirt
  (bind _returnvalue (Transformation|GetActorLocation))
  (bind _randomlocation (AI|Navigation|GetRandomReachablePointinRadius _returnvalue 2e+02 0 0))
  (if (> (Math|Random|RandomIntegerinRange 0 9) 8)
    (Game|SpawnActorfromClass "/Game/Blueprints/Mop/BP_Dirt.BP_Dirt_C" (Math|Transform|MakeTransform (Math|Vector|MakeVector (.x _randomlocation) (.y _randomlocation) (.z (Transformation|GetWorldLocation (Variables|Default|GetTrashSpawnPoint)))) "0, 0, 0" "1.000000,1.000000,1.000000") "AdjustIfPossibleButAlwaysSpawn" "OverrideRootScale" 0 0)))

(event EventBeginPlay
  (CallFunction|ResetBubble)
  (bind _returnvalue (Utilities|Time|SetTimerbyEvent (delegate Custom|TrySpawnDirt) 1e+01 true))
  (Variables|Default|SettrySpawnDirtTimer _returnvalue))

(fn ConstructionScript)

(fn SetStateMachineIndex
  (params (aiController :type Pawn%20Object%20Reference) (intValue :type Integer))
  (Class|BlackboardComponent|SetValueasInt (AI|GetBlackboard (AI|GetAIController aiController)) (Variables|Default|GetstateMachineIndexName) intValue))

(fn ChangeAnim
  (params (indexAnim :type Integer))
  (Utilities|FlowControl|Sequence ; if = 0, idle
    (:then_0
      (Variables|Default|SetisPay false)
      (Variables|Default|SetisThumbUp false)
      (Variables|Default|SetisArcade false)
      (Variables|Default|SetisClaw false)
      (Variables|Default|SetisPinball false)
      (Variables|Default|SetisToken false))
    (:then_1
      (if (== indexAnim 1)
        (Variables|Default|SetisPay true)))
    (:then_2
      (if (== indexAnim 2)
        (Variables|Default|SetisThumbUp true)))
    (:then_3
      (if (== indexAnim 3)
        (Variables|Default|SetisArcade true)))
    (:then_4
      (if (== indexAnim 4)
        (Variables|Default|SetisClaw true)))
    (:then_5
      (if (== indexAnim 5)
        (Variables|Default|SetisPinball true)))
    (:then_6
      (if (== indexAnim 6)
        (Variables|Default|SetisToken true)))))

(fn PassImgforBubble
  (params (imageForBubble :type Texture%20Object%20Reference))
  (bind _returnvalue (Utilities|Time|SetTimerbyFunctionName 0 "BubbleLookAtPlayer" 0.1 true))
  (Variables|Default|SetupdateBubbleLookTIimer _returnvalue)
  (Rendering|SetVisibility (Variables|Default|GetThoughtBubble) true false) ; Enable the ballon
  (bind _aswb_tough_bubble (Utilities|Casting|CastToWB_ToughBubble (UserInterface|GetUserWidgetObject (Variables|Default|GetThoughtBubble))))
  (Default|UpdateBubbleImg _aswb_tough_bubble imageForBubble))

(fn ResetBubble
  (Rendering|SetVisibility (Variables|Default|GetThoughtBubble) false false)
  (bind _aswb_tough_bubble (Utilities|Casting|CastToWB_ToughBubble (UserInterface|GetUserWidgetObject (Variables|Default|GetThoughtBubble))))
  (Default|DisableToughtBubble _aswb_tough_bubble)
  (Utilities|Time|ClearandInvalidateTimerbyHandle (Variables|Default|GetupdateBubbleLookTIimer)))

(fn BubbleLookatPlayer
  (bind _thoughtbubble (Variables|Default|GetThoughtBubble))
  (bind _returnvalue (Transformation|GetWorldLocation _thoughtbubble))
  (bind _asmy_game_instance (Utilities|Casting|CastToMyGameInstance (Game|GetGameInstance)))
  (Utilities|IsValid _thoughtbubble
    (:Is%20Valid
      (Transformation|SetWorldRotation _thoughtbubble (Math|Rotator|FindLookatRotation (Math|Vector|MakeVector (.x _returnvalue) (.y _returnvalue) (.z _returnvalue)) (Math|Vector|MakeVector (.x (Transformation|GetWorldLocation (Variables|/Script/Engine.Actor|GetRootComponent (Variables|/Game/Blueprints/Interfaces/MyGameInstance.MyGameInstance_C|GetbpPlayer _asmy_game_instance)))) (.y (Transformation|GetWorldLocation (Variables|/Script/Engine.Actor|GetRootComponent (Variables|/Game/Blueprints/Interfaces/MyGameInstance.MyGameInstance_C|GetbpPlayer _asmy_game_instance)))) (.z _returnvalue))) false false))))

(fn PassTokensforBubble
  (bind _returnvalue (Utilities|Time|SetTimerbyFunctionName 0 "BubbleLookAtPlayer" 0.1 true))
  (Variables|Default|SetupdateBubbleLookTIimer _returnvalue)
  (Variables|Default|SettokensForRecieve 0) ; reset cuz if move the terminal
  (Rendering|SetVisibility (Variables|Default|GetThoughtBubble) true false) ; Enable the ballon
  (bind _aswb_tough_bubble (Utilities|Casting|CastToWB_ToughBubble (UserInterface|GetUserWidgetObject (Variables|Default|GetThoughtBubble))))
  (Default|UpdateBubbleToken _aswb_tough_bubble (Variables|Default|GetquantityOfCoins) (Variables|Default|GettokensForRecieve)) ; Execute the function that you need on widget
)

(fn UpdateBubbleValue
  (bind _aswb_tough_bubble (Utilities|Casting|CastToWB_ToughBubble (UserInterface|GetUserWidgetObject (Variables|Default|GetThoughtBubble))))
  (Default|UpdateBubbleToken _aswb_tough_bubble (Variables|Default|GetquantityOfCoins) (Variables|Default|GettokensForRecieve)) ; Execute the function that you need on widget
)