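; BP_AutomaticDoor is a door actor meant to open automatically for characters derived from BP_NPCMaster.
; Overlap begin and end events on InteractWithDoorCollision maintain a count of the NPCs inside.
; CheckDoorCollisionCount passes whether that count is above zero to ToggleDoor, which snaps DoorMesh to the open or closed point without interpolation.
; Nothing in these graphs calls CheckDoorCollisionCount.
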(event OnComponentBeginOverlap(InteractWithDoorCollision)
  (params (OverlappedComponent :type Primitive%20Component%20Object%20Reference) (OtherActor :type Actor%20Object%20Reference) (OtherComp :type Primitive%20Component%20Object%20Reference) (OtherBodyIndex :type Integer) (bFromSweep :type Boolean) (SweepResult :type Hit%20Result%20Structure%20%28by%20ref%29))
  (Utilities|Casting|CastToBP_NPCMaster OtherActor)
  (Math|Integer|IncrementInt (Variables|Default|GetdoorCollisionCount)))

(event OnComponentEndOverlap(InteractWithDoorCollision)
  (params (OverlappedComponent :type Primitive%20Component%20Object%20Reference) (OtherActor :type Actor%20Object%20Reference) (OtherComp :type Primitive%20Component%20Object%20Reference) (OtherBodyIndex :type Integer))
  (Utilities|Casting|CastToBP_NPCMaster OtherActor)
  (Math|Integer|DecrementInt (Variables|Default|GetdoorCollisionCount)))

(event EventBeginPlay)

(event Collision|EventActorBeginOverlap
  (params (OtherActor :type Actor%20Object%20Reference)))

(event EventTick
  (params (DeltaSeconds :type Float%20%28single-precision%29)))

(fn ConstructionScript)

(fn ToggleDoor
  (params (openDoor :type Boolean))
  (if openDoor
    (Transformation|SetWorldLocation (Variables|Default|GetDoorMesh) (Transformation|GetWorldLocation (Variables|Default|GetDoorOpenPoint)) false false)
    (else
      (Transformation|SetWorldLocation (Variables|Default|GetDoorMesh) (Transformation|GetWorldLocation (Variables|Default|GetDoorClosePoint)) false false))))

(fn CheckDoorCollisionCount
  (CallFunction|ToggleDoor (> (Variables|Default|GetdoorCollisionCount) 0)))