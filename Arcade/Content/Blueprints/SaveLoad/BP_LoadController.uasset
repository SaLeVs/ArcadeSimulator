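; BP_LoadController is an actor that restores saved player buildables when the level begins play.
; On BeginPlay it reads the BuildablesSave array from the Game Instance's game data and spawns each entry's class at its saved transform, ignoring collisions.
; Each spawned actor is cast to BP_BuildablesMaster to restore its build index.
; An unconnected older path that spawned only the master class from a transform array never runs.
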(event EventBeginPlay
  (bind _savegamedata (Class|BPISaveGame|GetGameData(Message) (Game|GetGameInstance)))
  (if (> (Utilities|Array|Length (Variables|/Game/Blueprints/SaveLoad/BP_SaveLoadGame.BP_SaveLoadGame_C|GetBuildablesSave _savegamedata)) 0)
    (for _array_element (Variables|/Game/Blueprints/SaveLoad/BP_SaveLoadGame.BP_SaveLoadGame_C|GetBuildablesSave _savegamedata)
      (bind _returnvalue (Game|SpawnActorfromClass (.type _array_element) (.transform _array_element) "AlwaysSpawn" "MultiplyWithRoot" 0 0))
      (bind _asbp_buildables_master (Utilities|Casting|CastToBP_BuildablesMaster _returnvalue))
      (Variables|/Game/Blueprints/Builder/BP_BuildablesMaster.BP_BuildablesMaster_C|SetthisBuildableIndex _asbp_buildables_master (.buildindex _array_element))
      (Development|PrintString "Spawned Buildable"))))

(event Collision|EventActorBeginOverlap
  (params (OtherActor :type Actor%20Object%20Reference)))

(event EventTick
  (params (DeltaSeconds :type Float%20%28single-precision%29)))

(fn ConstructionScript)