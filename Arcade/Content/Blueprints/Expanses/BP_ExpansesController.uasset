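; Manages the player's timed expenses ("Expanses"): each day adds a random one, and any expense past its expiration ends the game.
; Loads templates from DT_Expanses and active expenses from the GameInstance save on BeginPlay, then binds to BP_DayCicleController's day change.
; Day changes decrement expirations; expiry deletes the save and opens the main menu.
; New or supplied saved expenses become slots in the WB_Computer widget on the PC buy terminal.
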(event Custom|OnDayChanged
  (CallFunction|UpdateCurrentExpansesDay)
  (CallFunction|AddNewExpanse (Math|Random|RandomIntegerinRange 0 (Utilities|Array|LastIndex (Variables|Default|GetDT_Expanses)))))

(event EventBeginPlay
  (Utilities|FlowControl|Sequence
    (:then_0
      (bind _outrownames (DataTable|GetDataTableRowNames "/Game/Blueprints/Expanses/DT_Expanses.DT_Expanses")) ; Get data bank
      (for _array_element _outrownames
        (bind _returnvalue (Utilities|GetDataTableRow "/Game/Blueprints/Expanses/DT_Expanses.DT_Expanses" _array_element)
          (:then
            (Utilities|Array|Add (Variables|Default|GetDT_Expanses) _returnvalue)))))
    (:then_1
      (bind _savegamedata (Class|BPISaveGame|GetGameData(Message) (Game|GetGameInstance))) ; LoadSave
      (Utilities|IsValid _savegamedata
        (:Is%20Valid
          (Variables|Default|SetcurrentExpanses (Variables|/Game/Blueprints/SaveLoad/BP_SaveLoadGame.BP_SaveLoadGame_C|GetexpansesSave _savegamedata)))))
    (:then_2
      (Utilities|FlowControl|Delay 0.2)
      (bind _returnvalue_2 (Actor|GetActorOfClass "/Game/Blueprints/DayCicle/BP_DayCicleController.BP_DayCicleController_C")) ; get day cicle controller for more expanses
      (EventDispatchers|BindEventtoOnDayChanged _returnvalue_2 (delegate Custom|OnDayChanged)))))

(fn ConstructionScript)

(fn AddNewExpanse
  (params (expanseIndex :type Integer))
  (bind _returnvalue (Utilities|Array|Add (Variables|Default|GetcurrentExpanses) (Utilities|Array|Get(acopy) (Variables|Default|GetDT_Expanses) expanseIndex)))
  (bind _returnvalue_2 (Actor|GetActorOfClass "/Game/Blueprints/Builder/Terminals/TerminalBuilds/BP_BuildTerminal_PcBuy.BP_BuildTerminal_PcBuy_C")) ; get pc for wb
  (bind _aswb_computer (Utilities|Casting|CastToWB_Computer (UserInterface|GetUserWidgetObject (Variables|/Game/Blueprints/Builder/Terminals/TerminalBuilds/BP_BuildTerminal_PcBuy.BP_BuildTerminal_PcBuy_C|GetWidget _returnvalue_2))))
  (Default|CreateExpanseSlot _aswb_computer (Utilities|Array|Get(acopy) (Variables|Default|GetcurrentExpanses) _returnvalue)))

(fn UpdateCurrentExpansesDay
  (bind _returnvalue (Game|GetPlayerController 0))
  (bind (_array_element _array_index) (Utilities|Array|ForEachLoopwithBreak (Variables|Default|GetcurrentExpanses) :!label _label)
    (:LoopBody
      (bind _result (Math|Integer|DecrementInt (.currentexpirationdate _array_element))
        (:%20%20
          (Utilities|Array|SetArrayElem (Variables|Default|GetcurrentExpanses) _array_index (Utilities|Struct|MakeS_Expanses (.tittle _array_element) (.imageexpanse _array_element) (.cost _array_element) _result))
          (if (< _result 0) ; True = Expanse expired
            (Development|PrintString "game over")
            (Class|BPISaveGame|DeleteSave(Message) (Game|GetGameInstance))
            (Input|SetInputModeUIOnly _returnvalue 0 "DoNotLock" false)
            (Variables|/Script/Engine.PlayerController|SetbShowMouseCursor _returnvalue true)
            (Game|OpenLevel(byName) "MainMenu_lvl")
            (goto _label Break)
            (else
              (Development|PrintString "can pay"))))))))

(fn UseExpansesSaveData
  (params (s_expanses :type Array%20of%20S%20Expanses%20Structures))
  (for _array_element s_expanses
    (bind _returnvalue (Actor|GetActorOfClass "/Game/Blueprints/Builder/Terminals/TerminalBuilds/BP_BuildTerminal_PcBuy.BP_BuildTerminal_PcBuy_C")) ; get pc for wb
    (bind _aswb_computer (Utilities|Casting|CastToWB_Computer (UserInterface|GetUserWidgetObject (Variables|/Game/Blueprints/Builder/Terminals/TerminalBuilds/BP_BuildTerminal_PcBuy.BP_BuildTerminal_PcBuy_C|GetWidget _returnvalue))))
    (Default|CreateExpanseSlot _aswb_computer _array_element)))

(fn GetExpansesSaveData
  (params (expanseIndex :type Integer))
  (return (Utilities|Array|Get(acopy) (Variables|Default|GetcurrentExpanses) expanseIndex)))