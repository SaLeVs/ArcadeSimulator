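; BP_BuildablesMaster is the base actor for placed buildables, handling their saving and pickup.
; On BeginPlay it caches controller and player references, loads DT_BuildParts rows, and saves itself through the GameInstance.
; A builder-controller event toggles its collision mesh visibility with build mode.
; Hold-interact replaces it with a small or big box attached to the player's hand, passing along its index and any machine coins, then destroys it.
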(event Custom|OnBuildModeChanged
  (params (InBuildMode :type Boolean))
  ;[1 1 1] Listen OnBuildModeChanged
  ;[1 1 1] Turn ON CollisionMesh
  (Rendering|SetVisibility (Variables|Default|GetCollisionMesh) InBuildMode false))

(event EventBeginPlay
  (Utilities|FlowControl|Sequence
    (:then_0
      ;[1 1 1] Get builder controller
      (bind _outactors (Actor|GetAllActorsOfClass "/Game/Blueprints/Builder/BuilderStuff/BP_BuilderController.BP_BuilderController_C"))
      (if (> (Utilities|Array|Length _outactors) 0)
        (Variables|Default|SetBP_BuilderController (Utilities|Array|Get(acopy) _outactors))))
    (:then_1
      ;[1 1 1] Turn OFF CollisionMesh
      (Rendering|SetVisibility (Variables|Default|GetCollisionMesh) false false))
    (:then_2
      ;[1 1 1] Listen OnBuildModeChanged
      (EventDispatchers|BindEventtoOnBuildModeChanged (Variables|Default|GetBP_BuilderController) (delegate Custom|OnBuildModeChanged)))
    (:then_3
      ;[1 1 1] Box Array
      (Variables|Default|SetBP_BoxInHand (Utilities|Array|MakeArray "/Game/Blueprints/BoxInHand/BP_BoxInHand_Small.BP_BoxInHand_Small_C" "/Game/Blueprints/BoxInHand/BP_BoxInHand_Big.BP_BoxInHand_Big_C")))
    (:then_4
      ;[1 1 1] Get Data Table
      (bind _outrownames (DataTable|GetDataTableRowNames "/Game/Blueprints/Builder/BuilderStuff/DT_BuildParts.DT_BuildParts"))
      (for _array_element _outrownames
        (bind _returnvalue (Utilities|GetDataTableRow "/Game/Blueprints/Builder/BuilderStuff/DT_BuildParts.DT_BuildParts" _array_element)
          (:then
            (Utilities|Array|Add (Variables|Default|GetDT_Buildables) _returnvalue)))))
    (:then_5
      ;[1 1 1] Get Player Ref
      (bind _asmy_game_instance (Utilities|Casting|CastToMyGameInstance (Game|GetGameInstance)))
      (Variables|Default|SetBP%20Player (Variables|/Game/Blueprints/Interfaces/MyGameInstance.MyGameInstance_C|GetbpPlayer _asmy_game_instance)))
    (:then_6
      ;[1 1 1] Save this buildable
      (bind _buildablesave (CallFunction|GetBuildableSaveData))
      (Class|BPISaveGame|SaveBuildables(Message) (Game|GetGameInstance) _buildablesave false))))

(event Collision|EventActorBeginOverlap
  (params (OtherActor :type Actor%20Object%20Reference)))

(event EventTick
  (params (DeltaSeconds :type Float%20%28single-precision%29)))

(event EventInteractHold
  (params (bpPlayer :type BP%20Player%20Object%20Reference))
  (bind _bp_player (Variables|Default|GetBP%20Player))
  (bind _boxinhandpoint (Variables|/Game/Blueprints/Player/BP_Player.BP_Player_C|GetBoxInHandPoint _bp_player))
  ;[1 1 1] Replace Buildable
  (Default|AddItemonHand (Variables|Default|GetBP%20Player))
  (bind _returnvalue (Game|SpawnActorfromClass (Utilities|Array|Get(acopy) (Variables|Default|GetBP_BoxInHand) (.ThisItemBoxIndex (Utilities|Struct|BreakS_BuildParts (Utilities|Array|Get(acopy) (Variables|Default|GetDT_Buildables) (Variables|Default|GetthisBuildableIndex))))) (Transformation|GetWorldTransform _boxinhandpoint) "AlwaysSpawn" "MultiplyWithRoot" 0 0)) ; Spawn Box
  (Variables|/Game/Blueprints/BoxInHand/BP_BoxInHandMaster.BP_BoxInHandMaster_C|SetBP_Player _returnvalue (Variables|Default|GetBP%20Player)) ; Pass ref to box
  (Default|Setup _returnvalue (Variables|Default|GetthisBuildableIndex))
  (Transformation|AttachComponentToComponent _returnvalue _boxinhandpoint "None" "SnapToTarget" "SnapToTarget" "KeepRelative" true)
  (Utilities|FlowControl|Sequence
    (:then_0
      ;[1 1 1] If I'm a Machine, ref coins to bpc
      (bind _asbp_build_machine_master (Utilities|Casting|CastToBP_BuildMachineMaster self))
      (Variables|/Game/Blueprints/Builder/BuilderStuff/BPC_BuildSystem.BPC_BuildSystem_C|SetcoinsInMachineHolding (Variables|/Game/Blueprints/Player/BP_Player.BP_Player_C|GetBPC_BuildSystem (Variables|Default|GetBP%20Player)) (Variables|/Game/Blueprints/Builder/Machines/MachineBuilds/BP_BuildMachineMaster.BP_BuildMachineMaster_C|GetcurrentCoins _asbp_build_machine_master)))
    (:then_1
      (Actor|DestroyActor) ; Destroy this obj
    )))

(fn ConstructionScript)

(fn GetBuildableSaveData
  (return (Utilities|Struct|MakeS_BuildablesSave (Transformation|GetActorTransform) self (Variables|Default|GetthisBuildableIndex))))

(fn UseBuildableSaveData
  (params (BuildableSave :type S%20Buildables%20Save%20Structure))
  (Utilities|FlowControl|Sequence
    (:then_0
      (Transformation|SetActorTransform (.transform BuildableSave)))
    (:then_1
      (Variables|Default|SetthisBuildableIndex (.buildindex BuildableSave)))))