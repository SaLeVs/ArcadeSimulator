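; Base Blueprint for buildable, coin-operated machines that hold an NPC queue and a coin store the player can empty.
; NPCs take one of four queue points by count, step forward through them, and leaving fires a queue-exit dispatcher.
; Plays add the machine's cost to its coins, while the player withdraws one coin at a time.
; A widget shows the machine as stuck when another play would exceed coin capacity.
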(event EventBeginPlay
  (|CallParentFunction)
  (CallFunction|UpdateStuckMachineUi))

(event Collision|EventActorBeginOverlap
  (params (OtherActor :type Actor%20Object%20Reference))
  (|CallParentFunction OtherActor) ; This node is disabled and will not be called.\nDrag off pins to build functionality.
)

(event EventTick
  (params (DeltaSeconds :type Float%20%28single-precision%29))
  (|CallParentFunction DeltaSeconds))

(fn ConstructionScript
  (|CallParentFunction)
  (Variables|Default|SetqueuePoints (Utilities|Array|MakeArray (Variables|Default|GetQueuePoint1) (Variables|Default|GetQueuePoint2) (Variables|Default|GetQueuePoint3) (Variables|Default|GetQueuePoint4))))

(fn PlayerGetCoins
  (if (> (Variables|Default|GetcurrentCoins) 0)
    (Variables|Default|SetcurrentCoins (- (Variables|Default|GetcurrentCoins) 1)) ; Can Subtract, Take One
    (CallFunction|UpdateStuckMachineUi)
    (return true)
    (else
      (return false) ; Cant Subtract, Empty
    )))

(fn CheckQueueLenght
  (if (>= (Variables|Default|GetnpcsOnQueue) (Utilities|Array|Length (Variables|Default|GetqueuePoints)))
    (return false)
    (else
      (return true))))

(fn JoinonQueue
  (bind _output_get (Variables|Default|SetnpcsOnQueue (+ (Variables|Default|GetnpcsOnQueue) 1)))
  (return (Utilities|Array|Get(acopy) (Variables|Default|GetqueuePoints) (- _output_get 1)) (- _output_get 1)))

(fn ExitonQueue
  (Variables|Default|SetnpcsOnQueue (- (Variables|Default|GetnpcsOnQueue) 1))
  (Default|CallOnQueueExit))

(fn PasstheQueu
  (params (MyPosOnQueue :type Integer))
  (bind _returnvalue (- MyPosOnQueue 1))
  (bind _returnvalue_2 (Math|Integer|Absolute(Integer) _returnvalue))
  (return (Utilities|Array|Get(acopy) (Variables|Default|GetqueuePoints) _returnvalue_2) _returnvalue_2))

(fn CheckTokens
  (if (<= (+ (Variables|Default|GetcurrentCoins) (Variables|Default|GetcostToPlayMachine)) (Variables|Default|GetmaxCoins))
    (return true)
    (else
      (return false))))

(fn AddTokenonMachine
  (Variables|Default|SetcurrentCoins (+ (Variables|Default|GetcurrentCoins) (Variables|Default|GetcostToPlayMachine)))
  (CallFunction|UpdateStuckMachineUi))

(fn UpdateStuckMachineUi
  (bind _aswb_machine_stuck (Utilities|Casting|CastToWB_MachineStuck (UserInterface|GetUserWidgetObject (Variables|Default|GetWidget))))
  (bind _can_add_more_tokens (CallFunction|CheckTokens))
  (Default|ToggleUiMachineStuck _aswb_machine_stuck (not _can_add_more_tokens)) ; true here = stuck machine
)