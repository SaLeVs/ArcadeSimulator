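; BP_MachineBuildMaster appears to be the base Blueprint for buildable machines, showing its CollisionMesh only while build mode is active.
; On BeginPlay it caches the first BP_BuilderController in the level, hides the mesh and binds to that controller's OnBuildModeChanged event.
; The event sets mesh visibility from the build mode flag, without touching collision settings or child components.
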(event Custom|OnBuildModeChanged
  (params (InBuildMode :type Boolean))
  ;[1 1 1] Listen OnBuildModeChanged
  ;[1 1 1] Turn ON CollisionMesh
  (Rendering|SetVisibility (Variables|Default|GetCollisionMesh) InBuildMode false))

(event EventBeginPlay
  (Utilities|FlowControl|Sequence
    (:then_0
      ;[1 1 1] Get builder controller
      (bind _outactors (Actor|GetAllActorsOfClass "/Game/Blueprints/Builder/BuilderStuff/BP_BuilderController.BP_BuilderController_C"))
      (if (> (Utilities|Array|Length _outactors) 0)
        (Variables|Default|SetBP_BuilderController (Utilities|Array|Get(acopy) _outactors))))
    (:then_1
      ;[1 1 1] Turn OFF CollisionMesh
      (Rendering|SetVisibility (Variables|Default|GetCollisionMesh) false false))
    (:then_2
      ;[1 1 1] Listen OnBuildModeChanged
      (EventDispatchers|BindEventtoOnBuildModeChanged (Variables|Default|GetBP_BuilderController) (delegate Custom|OnBuildModeChanged)))))

(fn ConstructionScript)