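; Master Blueprint for placed builder machines that collect coins from NPCs and let the player take them.
; NPC interaction adds a coin up to MaxCoins, while PlayerGetCoins removes one and reports success.
; Holding interact picks the machine up for re-placement, spawning its data-table box attached to the player's hand point, then destroying the machine.
; BeginPlay still randomizes and prints the coin count for debugging.
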(event Custom|NPC_INTERACT
  (if (< (Variables|Default|GetcurrentCoins) (Variables|Default|GetmaxCoins))
    (Variables|Default|SetcurrentCoins (+ (Variables|Default|GetcurrentCoins) 1))))

(event EventBeginPlay
  (|CallParentFunction)
  ;[0.1219 0 1] DEBUG ( TIRAR )
  (bind _output_get (Variables|Default|SetcurrentCoins (Math|Random|RandomInteger (Variables|Default|GetmaxCoins))))
  (Development|PrintString (Utilities|String|ToString(Integer) _output_get)))

(event Collision|EventActorBeginOverlap
  (params (OtherActor :type Actor%20Object%20Reference))
  (|CallParentFunction OtherActor) ; This node is disabled and will not be called.\nDrag off pins to build functionality.
)

(event EventTick
  (params (DeltaSeconds :type Float%20%28single-precision%29))
  (|CallParentFunction DeltaSeconds) ; This node is disabled and will not be called.\nDrag off pins to build functionality.
)

(event EventInteractHold
  (params (bpPlayer :type BP%20Player%20Object%20Reference))
  ;[1 1 1] Replace Machine
  (bind _output_get (Variables|Default|SetBP_Player bpPlayer))
  (Default|AddItemonHand _output_get)
  (bind _returnvalue (Game|SpawnActorfromClass (Utilities|Array|Get(acopy) (Variables|Default|GetBP_BoxInHand) (.ThisItemBoxIndex (Utilities|Struct|BreakS_BuildParts (Utilities|Array|Get(acopy) (Variables|Default|GetDT_Buildables) (Variables|Default|GetthisBuildableIndex))))) (Transformation|GetWorldTransform (Variables|/Game/Blueprints/Player/BP_Player.BP_Player_C|GetBoxInHandPoint (Variables|Default|GetBP_Player))) "AlwaysSpawn" "MultiplyWithRoot" 0 0)) ; Spawn Box
  (Variables|/Game/Blueprints/BoxInHand/BP_BoxInHandMaster.BP_BoxInHandMaster_C|SetBP_Player _returnvalue (Variables|Default|GetBP_Player)) ; Pass ref to box
  (Default|Setup _returnvalue (Variables|Default|GetthisBuildableIndex))
  (Transformation|AttachComponentToComponent _returnvalue (Variables|/Game/Blueprints/Player/BP_Player.BP_Player_C|GetBoxInHandPoint (Variables|Default|GetBP_Player)) "None" "SnapToTarget" "SnapToTarget" "KeepRelative" true)
  (Actor|DestroyActor) ; Destroy this obj
)

(fn ConstructionScript
  (|CallParentFunction))

(fn PlayerGetCoins
  (if (> (Variables|Default|GetcurrentCoins) 0)
    (Variables|Default|SetcurrentCoins (- (Variables|Default|GetcurrentCoins) 1)) ; Can Subtract, Take One
    (return true)
    (else
      (return false) ; Cant Subtract, Empty
    )))