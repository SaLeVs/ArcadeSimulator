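; BP_BuildMachinePreviewMaster is a machine placement preview for the builder that shows whether the current spot is free to build on.
; BeginPlay caches the first BP_BuilderController found in the level.
; BuildCollision counts overlapping components tagged "BuildCollision" as they enter and leave.
; Each count change reports buildability to the controller via CanBuildEvent and swaps BuildMesh between the valid and blocked preview materials.
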(event OnComponentBeginOverlap(BuildCollision)
  (params (OverlappedComponent :type Primitive%20Component%20Object%20Reference) (OtherActor :type Actor%20Object%20Reference) (OtherComp :type Primitive%20Component%20Object%20Reference) (OtherBodyIndex :type Integer) (bFromSweep :type Boolean) (SweepResult :type Hit%20Result%20Structure%20%28by%20ref%29))
  (bind _bp_buildercontroller (Variables|Default|GetBP_BuilderController))
  (bind _buildmesh (Variables|Default|GetBuildMesh))
  ;[1 1 1] Collided with build, add count
  (if (Components|ComponentHasTag OtherComp "BuildCollision")
    (bind _output_get (Variables|Default|SetcountColl (+ (Variables|Default|GetcountColl) 1)))
    (if (> _output_get 0)
      (Default|CanBuildEvent _bp_buildercontroller false) ; cant build
      (Rendering|Material|SetMaterial _buildmesh 0 "/Game/Materials/M_CantBuildingPreview.M_CantBuildingPreview")
      (else
        (Default|CanBuildEvent _bp_buildercontroller true) ; can build
        (Rendering|Material|SetMaterial _buildmesh 0 "/Game/Materials/M_BuildingPreview.M_BuildingPreview")))))

(event OnComponentEndOverlap(BuildCollision)
  (params (OverlappedComponent :type Primitive%20Component%20Object%20Reference) (OtherActor :type Actor%20Object%20Reference) (OtherComp :type Primitive%20Component%20Object%20Reference) (OtherBodyIndex :type Integer))
  (bind _bp_buildercontroller (Variables|Default|GetBP_BuilderController))
  (bind _buildmesh (Variables|Default|GetBuildMesh))
  ;[1 1 1] Stop Colliding with one build
  (if (Components|ComponentHasTag OtherComp "BuildCollision")
    (Variables|Default|SetcountColl (- (Variables|Default|GetcountColl) 1))
    (if (> (stale OnComponentBeginOverlap(BuildCollision) _output_get) 0)
      (Default|CanBuildEvent _bp_buildercontroller false) ; cant build
      (Rendering|Material|SetMaterial _buildmesh 0 "/Game/Materials/M_CantBuildingPreview.M_CantBuildingPreview")
      (else
        (Default|CanBuildEvent _bp_buildercontroller true) ; can build
        (Rendering|Material|SetMaterial _buildmesh 0 "/Game/Materials/M_BuildingPreview.M_BuildingPreview")))))

(event EventBeginPlay
  (|CallParentFunction)
  ;[1 1 1] Get Builder Controller
  (bind _outactors (Actor|GetAllActorsOfClass "/Game/Blueprints/Builder/BuilderStuff/BP_BuilderController.BP_BuilderController_C"))
  (if (> (Utilities|Array|Length _outactors) 0)
    (Variables|Default|SetBP_BuilderController (Utilities|Array|Get(acopy) _outactors))))

(event EventTick
  (params (DeltaSeconds :type Float%20%28single-precision%29))
  (|CallParentFunction DeltaSeconds) ; This node is disabled and will not be called.\nDrag off pins to build functionality.
)

(event Collision|EventActorBeginOverlap
  (params (OtherActor :type Actor%20Object%20Reference))
  (|CallParentFunction OtherActor) ; This node is disabled and will not be called.\nDrag off pins to build functionality.
)

(fn ConstructionScript
  (|CallParentFunction))