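; Buildable cashier station (named ATM machine) where the player takes an NPC's payment and hands back change and tokens.
; Interact snaps the player to the station, swaps input to the cashier mapping context, opens the drawer and binds BPCAtmSystem events.
; Camera traces pick up money, add or remove tagged bills and coins on the WB_AtmMonitor widget, and outline the aimed piece on a timer.
; Correct change credits PlayerMoney; CallOnMoneyDelivered2 fires once money and tokens are both delivered.
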(event Custom|OnPlayerLeftCashier2
  (bind _returnvalue (Game|GetPlayerController 0))
  (bind _bp_player1 (Variables|Default|GetBp%20Player1))
  (bind _returnvalue_2 (PlayerController|LocalPlayerSubsystems|GetEnhancedInputLocalPlayerSubsystem _returnvalue))
  ;[0.2622 1 0.6244] Teleport player for atm
  (Input|RemoveMappingContext _returnvalue_2 "/Game/Inputs/InputsAtm/IMC_PlayerOnCashier.IMC_PlayerOnCashier" "(bIgnoreAllPressedKeysUntilRelease=True,bForceImmediately=False,bNotifyUserSettings=False)")
  (Input|AddMappingContext _returnvalue_2 "/Game/Inputs/InputsPlayerMove/IMC_PlayerMovement.IMC_PlayerMovement" 0 "(bIgnoreAllPressedKeysUntilRelease=True,bForceImmediately=False,bNotifyUserSettings=False)")
  (Collision|SetCollisionEnabled (Variables|/Script/Engine.Character|GetCapsuleComponent _bp_player1) "QueryAndPhysics") ; player can walk on ground
  (Default|RemoveItemonHand _bp_player1))

(event Custom|OnPlayerInteractOnCashier2
  (bind _moneyoncashier (Variables|Default|GetmoneyOnCashier))
  (bind _wbatm (Variables|Default|GetwbAtm))
  (bind _wbatm_2 (Variables|Default|GetwbAtm))
  (bind _wbatm_3 (Variables|Default|GetwbAtm))
  (bind _wbatm_4 (Variables|Default|GetwbAtm))
  (bind _tokensmeshforcashier (Variables|Default|GetTokensMeshForCashier))
  (bind _wbatm_5 (Variables|Default|GetwbAtm))
  (bind _bp_player1 (Variables|Default|GetBp%20Player1))
  (bind _wbatm_6 (Variables|Default|GetwbAtm))
  (bind _returnvalue (Transformation|GetWorldTransform _tokensmeshforcashier))
  (bind _camera (Variables|/Game/Blueprints/Player/BP_Player.BP_Player_C|GetCamera _bp_player1))
  (bind _returnvalue_2 (Transformation|GetWorldTransform _camera))
  (bind _outhit (Collision|LineTraceByChannel (.location _returnvalue_2) (+ (.location _returnvalue_2) (* (Math|Vector|GetForwardVector (.rotation _returnvalue_2)) 7e+02)) "TraceTypeQuery2" false 0 "ForDuration" false))
  (bind _caninteract (CallFunction|InteractMoney (.HitActor (Collision|BreakHitResult _outhit)))) ; Verify if player picked money of npc
  (Development|PrintString "passou por auqi")
  (if _caninteract
    (Utilities|FlowControl|Sequence
      (:then_0
        ;[0.2622 1 0.6244] Add money if hit on money component
        (if (Variables|Default|GetdrawerOpen)
          (bind _moneyvalue (CallFunction|SendMoneyValue (Variables|Default|GetmoneyArray) (.HitComponent (Collision|BreakHitResult _outhit)))) ; Pass the value according the array function
          (Utilities|FlowControl|Sequence
            (:then_0
              (if (not (Variables|Default|GetMoneyDelivered))
                (Variables|/Game/Widgets/WB_AtmMonitor.WB_AtmMonitor_C|SetmoneyGiving _wbatm_3 (+ _moneyvalue (Variables|/Game/Widgets/WB_AtmMonitor.WB_AtmMonitor_C|GetmoneyGiving _wbatm_3)))
                (Default|UpdateMoneyValues _wbatm_3)))
            (:then_1
              (if (not (Variables|Default|GetcoinsDelivered))
                (Default|UpdateMoneyValues _wbatm_3))))))
      (:then_1
        ;[0.2622 1 0.6244] calculating how many tokens we need to send
        (Utilities|IsValid (.HitComponent (Collision|BreakHitResult _outhit))
          (:Is%20Valid
            (if (Components|ComponentHasTag (.HitComponent (Collision|BreakHitResult _outhit)) "TipsMesh") ; True = Player hit tipSuport
              (if (> (- (Variables|/Game/Widgets/WB_AtmMonitor.WB_AtmMonitor_C|GetTokensRecieved _wbatm_2) (Variables|/Game/Widgets/WB_AtmMonitor.WB_AtmMonitor_C|GetTokensRecieving _wbatm_2)) 0) ; Player cant pay negative coins for npc
                (bind _outputpin (CallFunction|SendTokensValue))
                (Default|TokensUpdate _outputpin) ; Update tokens value on monitor
                (bind _outactors (Actor|GetAllActorsOfClass "/Game/Blueprints/Cashier/BP_CashierTokens.BP_CashierTokens_C"))
                (if (Utilities|Array|IsEmpty _outactors) ; Checks if the currency mesh already exists
                  (Game|SpawnActorfromClass "/Game/Blueprints/Cashier/BP_CashierTokens.BP_CashierTokens_C" (Math|Transform|MakeTransform (.location _returnvalue) (.rotation _returnvalue) "3.000000,3.000000,3.000000") "Undefined" "MultiplyWithRoot" 0 0)))))))
      (:then_2
        ;[0.2622 1 0.6244] calculating how many tokens we need to send
        (Utilities|IsValid (.HitActor (Collision|BreakHitResult _outhit))
          (:Is%20Valid
            (if (== (.HitActor (Collision|BreakHitResult _outhit)) _moneyoncashier) ; Compare if player hit on money on table for npc
              (if (Utilities|Enum|Equal(Enum) (Utilities|String|ToString(Float) (Variables|/Game/Widgets/WB_AtmMonitor.WB_AtmMonitor_C|GetmoneyChange _wbatm_6)) (Utilities|String|ToString(Float) (Variables|/Game/Widgets/WB_AtmMonitor.WB_AtmMonitor_C|GetmoneyGiving _wbatm_6))) ; If the change is correct
                (Actor|DestroyActor _moneyoncashier) ; Destroy the mesh on table
                (bind _asmy_game_instance (Utilities|Casting|CastToMyGameInstance (Game|GetGameInstance)))
                (Variables|/Game/Blueprints/Interfaces/MyGameInstance.MyGameInstance_C|SetplayerMoney _asmy_game_instance (- (+ (Variables|/Game/Widgets/WB_AtmMonitor.WB_AtmMonitor_C|GetmoneyRecieved (Variables|Default|GetwbAtm)) (Variables|/Game/Blueprints/Interfaces/MyGameInstance.MyGameInstance_C|GetplayerMoney _asmy_game_instance)) (Variables|/Game/Widgets/WB_AtmMonitor.WB_AtmMonitor_C|GetmoneyGiving _wbatm))) ; Set money on game instance
                (Variables|/Game/Widgets/WB_AtmMonitor.WB_AtmMonitor_C|SetmoneyRecieved _wbatm 0.0)
                (Variables|/Game/Widgets/WB_AtmMonitor.WB_AtmMonitor_C|SetmoneyGiving _wbatm 0.0)
                (Variables|/Game/Widgets/WB_AtmMonitor.WB_AtmMonitor_C|SetmoneyChange _wbatm 0.0) ; Reset values for other npc
                (bind _output_get (Variables|Default|SetMoneyDelivered true))
                (Default|NpcDeliveryAnything _wbatm)
                ;[0.2622 1 0.6244] Verify if player delivery money and tokens
                (if (and _output_get (stale _output_get_2)) :!label _label ; True = Call event that npc left off cashier
                  (Variables|Default|SetMoneyDelivered false)
                  (Variables|Default|SetcoinsDelivered false)
                  (Default|CallOnMoneyDelivered2)))))))
      (:then_3
        (Utilities|IsValid (.HitActor (Collision|BreakHitResult _outhit))
          (:Is%20Valid
            (if (Actor|ActorHasTag (.HitActor (Collision|BreakHitResult _outhit)) "tipsOnCashier") ; Compare if player hit on tokens on table for npc
              (if (<= (Variables|/Game/Widgets/WB_AtmMonitor.WB_AtmMonitor_C|GetTokensRecieved _wbatm_5) (Variables|/Game/Widgets/WB_AtmMonitor.WB_AtmMonitor_C|GetTokensRecieving _wbatm_5)) ; If the quantity of tokens is correct
                (Actor|DestroyActor (.HitActor (Collision|BreakHitResult _outhit)))
                (Variables|/Game/Widgets/WB_AtmMonitor.WB_AtmMonitor_C|SetTokensRecieving _wbatm_4 0)
                (Variables|/Game/Widgets/WB_AtmMonitor.WB_AtmMonitor_C|SetTokensRecieved _wbatm_4 0)
                (Variables|Default|SetCoinsGiving 0) ; Reset values
                (bind _output_get_2 (Variables|Default|SetcoinsDelivered true))
                (Default|NpcDeliveryAnything (Variables|Default|GetwbAtm))
                (goto _label)))))))))

(event Custom|PlayerRemoveMoney2
  (bind _wbatm (Variables|Default|GetwbAtm))
  (bind _bp_player1 (Variables|Default|GetBp%20Player1))
  (bind _camera (Variables|/Game/Blueprints/Player/BP_Player.BP_Player_C|GetCamera _bp_player1))
  (bind _returnvalue (Transformation|GetWorldTransform _camera))
  ;[0.2622 1 0.6244] Retire money off cashier
  (bind _outhit (Collision|LineTraceByChannel (.location _returnvalue) (+ (.location _returnvalue) (* (Math|Vector|GetForwardVector (.rotation _returnvalue)) 7e+02)) "TraceTypeQuery1" false 0 "ForDuration" false))
  (if (Variables|Default|GetdrawerOpen)
    (bind _moneyvalue (CallFunction|SendMoneyValueBack (Variables|Default|GetmoneyArray) (.HitComponent (Collision|BreakHitResult _outhit))))
    (Variables|/Game/Widgets/WB_AtmMonitor.WB_AtmMonitor_C|SetmoneyGiving _wbatm (+ _moneyvalue (Variables|/Game/Widgets/WB_AtmMonitor.WB_AtmMonitor_C|GetmoneyGiving _wbatm)))
    (Default|UpdateMoneyValues _wbatm)))

(event Custom|UpdateLineTrace2
  (bind _bp_player1 (Variables|Default|GetBp%20Player1))
  (bind _camera (Variables|/Game/Blueprints/Player/BP_Player.BP_Player_C|GetCamera _bp_player1))
  (bind _returnvalue (Transformation|GetWorldTransform _camera))
  ;[0.2622 1 0.6244] Update line trace for outline money
  (Utilities|Time|SetTimerbyEvent (delegate Custom|UpdateLineTrace2) 0.05)
  (if (Variables|Default|GetdrawerOpen)
    (bind _outhit (Collision|LineTraceByChannel (.location _returnvalue) (+ (.location _returnvalue) (* (Math|Vector|GetForwardVector (.rotation _returnvalue)) 7e+02)) "TraceTypeQuery1" false 0 "None" false))
    (CallFunction|ActiveandDisableOutline (Variables|Default|GetmoneyArray) (.HitComponent (Collision|BreakHitResult _outhit)))))

(event EventInteract
  (params (bpPlayer :type BP%20Player%20Object%20Reference))
  (bind _returnvalue (Game|GetPlayerController 0))
  (bind _returnvalue_2 (Game|GetPlayerCharacter 0))
  (bind _drawer (Variables|Default|GetDrawer))
  (bind _arrow (Variables|Default|GetArrow))
  (bind _returnvalue_3 (Transformation|GetWorldTransform _arrow))
  (bind _returnvalue_4 (PlayerController|LocalPlayerSubsystems|GetEnhancedInputLocalPlayerSubsystem _returnvalue))
  (Default|AddItemonHand bpPlayer)
  (Variables|Default|SetBp%20Player1 bpPlayer)
  (Utilities|FlowControl|Sequence
    (:then_0
      ;[0.2622 1 0.6244] Teleport player for atm
      (Transformation|SetWorldTransform (Variables|/Script/Engine.Actor|GetRootComponent (Variables|Default|GetBp%20Player1)) (Math|Transform|MakeTransform (.location _returnvalue_3) (.rotation _returnvalue_3) "1.000000,1.000000,1.000000") false false) ; Teletransport player
      (Collision|SetCollisionEnabled (Variables|/Script/Engine.Character|GetCapsuleComponent (Variables|Default|GetBp%20Player1)) "NoCollision") ; Allow player enter on the groud
      (if (== (Variables|Default|GetBp%20Player1) _returnvalue_2)
        (Pawn|SetControlRotation (Game|GetPlayerController 0) (Transformation|GetActorRotation _returnvalue_2)) ; Set player to look foward
        (Variables|/Script/Engine.MovementComponent|SetVelocity (Variables|/Script/Engine.Character|GetCharacterMovement _returnvalue_2) "0, 0, 0")
        (Input|RemoveMappingContext _returnvalue_4 "/Game/Inputs/InputsPlayerMove/IMC_PlayerMovement.IMC_PlayerMovement" "(bIgnoreAllPressedKeysUntilRelease=True,bForceImmediately=False,bNotifyUserSettings=False)") ; Switch the mapping context for cashier
        (Input|AddMappingContext _returnvalue_4 "/Game/Inputs/InputsAtm/IMC_PlayerOnCashier.IMC_PlayerOnCashier" 0 "(bIgnoreAllPressedKeysUntilRelease=True,bForceImmediately=False,bNotifyUserSettings=False)")))
    (:then_1
      (EventDispatchers|BindEventtoOnPlayerExitCashier (Variables|/Game/Blueprints/Player/BP_Player.BP_Player_C|GetBPC_AtmSystem (Variables|Default|GetBp%20Player1)) (delegate Custom|OnPlayerLeftCashier2)))
    (:then_2
      (EventDispatchers|BindEventtoOnPlayerInteractinCashier (Variables|/Game/Blueprints/Player/BP_Player.BP_Player_C|GetBPC_AtmSystem (Variables|Default|GetBp%20Player1)) (delegate Custom|OnPlayerInteractOnCashier2)))
    (:then_3
      (EventDispatchers|BindEventtoOnPlayerRemoveMoney (Variables|/Game/Blueprints/Player/BP_Player.BP_Player_C|GetBPC_AtmSystem (Variables|Default|GetBp%20Player1)) (delegate Custom|PlayerRemoveMoney2)))
    (:then_4
      ;[0.2622 1 0.6244] Open Drawer
      (if (not (Variables|Default|GetdrawerOpen))
        (Transformation|SetRelativeLocation _drawer (+ (Variables|/Script/Engine.SceneComponent|GetRelativeLocation _drawer) "0.000000,34.000000,0.000000") false false)
        (Variables|Default|SetdrawerOpen true)
        (CallFunction|UpdateLineTrace2) ; Call the event for interact with all
      ))))

(event EventBeginPlay
  ;[0.2622 1 0.6244] Pass the reference for widget
  (|CallParentFunction)
  (bind _aswb_atm_monitor (Utilities|Casting|CastToWB_AtmMonitor (UserInterface|GetUserWidgetObject (Variables|Default|GetWidget))))
  (Variables|Default|SetwbAtm _aswb_atm_monitor))

(event EventTick
  (params (DeltaSeconds :type Float%20%28single-precision%29))
  (|CallParentFunction DeltaSeconds) ; This node is disabled and will not be called.\nDrag off pins to build functionality.
)

(event Collision|EventActorBeginOverlap
  (params (OtherActor :type Actor%20Object%20Reference))
  (|CallParentFunction OtherActor) ; This node is disabled and will not be called.\nDrag off pins to build functionality.
)

(fn ConstructionScript
  (|CallParentFunction)
  (Transformation|SetRelativeTransform (Variables|Default|GetArrow) (Variables|Default|GetteleportLocation) false false)
  (Variables|Default|SetmoneyArray (Utilities|Array|MakeArray (Variables|Default|Get50_Dolar) (Variables|Default|Get20_Dolar) (Variables|Default|Get10_Dolar) (Variables|Default|Get5_Dolar) (Variables|Default|Get1_Dolar) (Variables|Default|Get50_Cent) (Variables|Default|Get25_Cent) (Variables|Default|Get10_Cent) (Variables|Default|Get5_Cent) (Variables|Default|Get1_Cent) (Variables|Default|GetSuportForTokens)))
  (Variables|Default|SetqueuePoints (Utilities|Array|MakeArray (Variables|Default|GetQueu1) (Variables|Default|GetQueu2) (Variables|Default|GetQueu3) (Variables|Default|GetQueu4))))

(fn ActiveandDisableOutline
  (params (MoneyComponent :type Array%20of%20Static%20Mesh%20Component%20Object%20References) (HitComponent :type Primitive%20Component%20Object%20Reference))
  (if (not (Utilities|Array|IsEmpty MoneyComponent))
    (for _array_element MoneyComponent
      (Utilities|IsValid _array_element
        (:Is%20Valid
          (bind _output_get (Variables|Components|SetArray%20Element _array_element))
          (if (== _output_get HitComponent)
            (Rendering|SetRenderCustomDepth (Variables|Components|GetArray%20Element) true)
            (else
              (Rendering|SetRenderCustomDepth (Variables|Components|GetArray%20Element) false))))))
    (Variables|Components|SetArray%20Element 0)))

(fn SendMoneyValue
  (params (moneyComponent :type Array%20of%20Static%20Mesh%20Component%20Object%20References) (hitComponent :type Primitive%20Component%20Object%20Reference))
  (Variables|Components|SetArray%20Element 0)
  (Variables|Default|SetmoneyValeuForSend 0.0) ; Reset values
  (if (not (Utilities|Array|IsEmpty moneyComponent))
    (for _array_element moneyComponent
      (Utilities|IsValid _array_element
        (:Is%20Valid
          (bind _output_get (Variables|Components|SetArray%20Element _array_element))
          (if (== _output_get hitComponent)
            (for _array_element_2 (Variables|/Script/Engine.ActorComponent|GetComponentTags (Variables|Components|GetArray%20Element))
              (switch string (Utilities|String|ToString(Name) _array_element_2) ; Pass the value according the tag off object hitted
                (:1Dolar
                  (Variables|Default|SetmoneyValeuForSend 1.0))
                (:5Dolar
                  (Variables|Default|SetmoneyValeuForSend 5.0))
                (:10Dolar
                  (Variables|Default|SetmoneyValeuForSend 1e+01))
                (:20Dolar
                  (Variables|Default|SetmoneyValeuForSend 2e+01))
                (:50Dolar
                  (Variables|Default|SetmoneyValeuForSend 5e+01))
                (:1Cent
                  (Variables|Default|SetmoneyValeuForSend 0.01))
                (:5Cent
                  (Variables|Default|SetmoneyValeuForSend 0.05))
                (:10Cent
                  (Variables|Default|SetmoneyValeuForSend 0.1))
                (:25Cent
                  (Variables|Default|SetmoneyValeuForSend 0.25))
                (:50Cent
                  (Variables|Default|SetmoneyValeuForSend 0.5))))))))
    (Variables|Components|SetArray%20Element 0)
    (Variables|Components|SetArray%20Element 0)
    (return (Variables|Default|GetmoneyValeuForSend))))

(fn SendMoneyValueBack
  (params (moneyComponent :type Array%20of%20Static%20Mesh%20Component%20Object%20References) (hitComponent :type Primitive%20Component%20Object%20Reference))
  (Variables|Components|SetArray%20Element 0)
  (Variables|Default|SetmoneyValeuForSend 0.0)
  (if (not (Utilities|Array|IsEmpty moneyComponent))
    (for _array_element moneyComponent
      (Utilities|IsValid _array_element
        (:Is%20Valid
          (bind _output_get (Variables|Components|SetArray%20Element _array_element))
          (if (== _output_get hitComponent)
            (for _array_element_2 (Variables|/Script/Engine.ActorComponent|GetComponentTags (Variables|Components|GetArray%20Element))
              (switch string (Utilities|String|ToString(Name) _array_element_2)
                (:1Dolar
                  (Variables|Default|SetmoneyValeuForSend -1.0))
                (:5Dolar
                  (Variables|Default|SetmoneyValeuForSend -5.0))
                (:10Dolar
                  (Variables|Default|SetmoneyValeuForSend -1e+01))
                (:20Dolar
                  (Variables|Default|SetmoneyValeuForSend -2e+01))
                (:50Dolar
                  (Variables|Default|SetmoneyValeuForSend -5e+01))
                (:1Cent
                  (Variables|Default|SetmoneyValeuForSend -0.01))
                (:5Cent
                  (Variables|Default|SetmoneyValeuForSend -0.05))
                (:10Cent
                  (Variables|Default|SetmoneyValeuForSend -0.1))
                (:25Cent
                  (Variables|Default|SetmoneyValeuForSend -0.25))
                (:50Cent
                  (Variables|Default|SetmoneyValeuForSend -0.5))))))))
    (Variables|Components|SetArray%20Element 0)
    (Variables|Components|SetArray%20Element 0)
    (return (Variables|Default|GetmoneyValeuForSend))))

(fn SendTokensValue
  (bind _wbatm (Variables|Default|GetwbAtm))
  (bind _result (Math|Integer|IncrementInt (Variables|Default|GetCoinsGiving))
    (:%20%20
      (Variables|/Game/Widgets/WB_AtmMonitor.WB_AtmMonitor_C|SetTokensRecieving _wbatm _result)
      (return _wbatm))))

(fn InteractMoney
  (params (hitComponent :type Actor%20Object%20Reference))
  (bind _moneymeshforcashier (Variables|Default|GetMoneyMeshForCashier))
  (bind _wbatm (Variables|Default|GetwbAtm))
  (bind _returnvalue (Transformation|GetWorldTransform _moneymeshforcashier))
  (Utilities|IsValid hitComponent
    (:Is%20Valid
      (if (Components|ComponentHasTag (Variables|/Script/Engine.Actor|GetRootComponent hitComponent) "MoneyMesh")
        (bind _returnvalue_2 (Actor|GetActorOfClass "/Game/Blueprints/Cashier/BP_NpcMoney.BP_NpcMoney_C"))
        (Variables|/Game/Widgets/WB_AtmMonitor.WB_AtmMonitor_C|SetmoneyChange _wbatm (Variables|/Game/Blueprints/Cashier/BP_NpcMoney.BP_NpcMoney_C|GetchangeNpc _returnvalue_2))
        (Variables|/Game/Widgets/WB_AtmMonitor.WB_AtmMonitor_C|SetmoneyRecieved _wbatm (Variables|/Game/Blueprints/Cashier/BP_NpcMoney.BP_NpcMoney_C|GetmoneyNpc _returnvalue_2))
        (Variables|/Game/Widgets/WB_AtmMonitor.WB_AtmMonitor_C|SetTokensRecieved _wbatm (Variables|/Game/Blueprints/Cashier/BP_NpcMoney.BP_NpcMoney_C|GetcoinsNpc _returnvalue_2))
        (Actor|DestroyActor hitComponent)
        (bind _returnvalue_3 (Game|SpawnActorfromClass "/Game/Blueprints/Cashier/BP_CashierMoney.BP_CashierMoney_C" (Math|Transform|MakeTransform (.location _returnvalue) (.rotation _returnvalue) "0.200000,0.200000,0.200000") "Undefined" "MultiplyWithRoot" 0 0))
        (Variables|Default|SetmoneyOnCashier _returnvalue_3)
        (Default|UpdateMoneyValues _wbatm)
        (Default|TokensUpdate _wbatm)
        (return true)))))