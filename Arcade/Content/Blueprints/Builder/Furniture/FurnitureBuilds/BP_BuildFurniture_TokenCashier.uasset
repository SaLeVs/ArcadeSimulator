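; Buildable token cashier station where the player hands out tokens to customers.
; Interact snaps the player to an arrow, disables capsule collision and swaps to cashier input until BPCAtmSystem signals exit.
; Interact presses line trace tagged meshes to count tokens up to the required amount, then hand them over and fire OnTokenDelivered.
; A looping timer traces from the camera to custom-depth outline hovered items; construction fills four queue points.
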(event Custom|OnPlayerLeftCashier
  (bind _returnvalue (Game|GetPlayerController 0))
  (bind _bp_player (Variables|Default|GetBP%20Player))
  (bind _returnvalue_2 (PlayerController|LocalPlayerSubsystems|GetEnhancedInputLocalPlayerSubsystem _returnvalue))
  ;[0.2622 1 0.6244] Teleport player for atm
  (Input|RemoveMappingContext _returnvalue_2 "/Game/Inputs/InputsAtm/IMC_PlayerOnCashier.IMC_PlayerOnCashier" "(bIgnoreAllPressedKeysUntilRelease=True,bForceImmediately=False,bNotifyUserSettings=False)")
  (Input|AddMappingContext _returnvalue_2 "/Game/Inputs/InputsPlayerMove/IMC_PlayerMovement.IMC_PlayerMovement" 0 "(bIgnoreAllPressedKeysUntilRelease=True,bForceImmediately=False,bNotifyUserSettings=False)")
  (Collision|SetCollisionEnabled (Variables|/Script/Engine.Character|GetCapsuleComponent _bp_player) "QueryAndPhysics") ; player can walk on ground
  (Default|RemoveItemonHand _bp_player)
  (Utilities|Time|ClearandInvalidateTimerbyHandle (Variables|Default|GetupdateLineTraceTimer)))

(event Custom|OnPlayerInteractOnCashier
  (bind _bp_player (Variables|Default|GetBP%20Player))
  (bind _camera (Variables|/Game/Blueprints/Player/BP_Player.BP_Player_C|GetCamera _bp_player))
  (bind _returnvalue (Transformation|GetWorldTransform _camera))
  (bind _outhit (Collision|LineTraceByChannel (.location _returnvalue) (+ (.location _returnvalue) (* (Math|Vector|GetForwardVector (.rotation _returnvalue)) 7e+02)) "TraceTypeQuery1" false 0 "ForDuration" false))
  (Utilities|FlowControl|Sequence
    (:then_0
      ;[0.2622 1 0.6244] calculating how many tokens we need to send
      (Utilities|IsValid (.HitComponent (Collision|BreakHitResult _outhit))
        (:Is%20Valid
          (if (Components|ComponentHasTag (.HitComponent (Collision|BreakHitResult _outhit)) "TipsMesh") ; True = Player hit tipSuport
            (if (< (Variables|Default|GetgivedTokens) (Variables|Default|GettokensToGive)) ; true = can give more\nfalse = cant give more
              (Math|Integer|IncrementInt (Variables|Default|GetgivedTokens)
                (:%20%20
                  (Rendering|SetVisibility (Variables|Default|GetTokensDeliver) true true))))))))
    (:then_1
      ;[0.2622 1 0.6244] Verify if player delivery money and tokens
      (Utilities|IsValid (.HitComponent (Collision|BreakHitResult _outhit))
        (:Is%20Valid
          (if (Components|ComponentHasTag (.HitComponent (Collision|BreakHitResult _outhit)) "tipsOnCashier") ; Compare if player hit on tokens on table for npc
            (if (>= (Variables|Default|GetgivedTokens) (Variables|Default|GettokensToGive)) ; true = can give more\nfalse = cant give more, give to npc
              (Variables|Default|SetgivedTokens 0)
              (Variables|Default|SettokensToGive 0)
              (Rendering|SetVisibility (Variables|Default|GetTokensDeliver) false true)
              (Default|CallOnTokenDelivered))))))))

(event Custom|UpdateLineTrace
  (bind _bp_player (Variables|Default|GetBP%20Player))
  (bind _camera (Variables|/Game/Blueprints/Player/BP_Player.BP_Player_C|GetCamera _bp_player))
  (bind _returnvalue (Transformation|GetWorldTransform _camera))
  ;[0.2622 1 0.6244] Update line trace for outline money (Need to exist cuz have item on hand)
  (bind (_outhit _returnvalue_2) (Collision|LineTraceByChannel (.location _returnvalue) (+ (.location _returnvalue) (* (Math|Vector|GetForwardVector (.rotation _returnvalue)) 7e+02)) "TraceTypeQuery1" false 0 "None" false))
  (if _returnvalue_2
    (CallFunction|ActiveandDisableOutline (.HitComponent (Collision|BreakHitResult _outhit)))))

(event EventBeginPlay
  (|CallParentFunction))

(event EventTick
  (params (DeltaSeconds :type Float%20%28single-precision%29))
  (|CallParentFunction DeltaSeconds))

(event EventInteract
  (params (bpPlayer :type BP%20Player%20Object%20Reference))
  (bind _returnvalue (Game|GetPlayerController 0))
  (bind _returnvalue_2 (Game|GetPlayerCharacter 0))
  (bind _bp_player (Variables|Default|GetBP%20Player))
  (bind _arrow (Variables|Default|GetArrow))
  (bind _returnvalue_3 (Transformation|GetWorldTransform _arrow))
  (bind _returnvalue_4 (PlayerController|LocalPlayerSubsystems|GetEnhancedInputLocalPlayerSubsystem _returnvalue))
  (bind _bpc_atmsystem (Variables|/Game/Blueprints/Player/BP_Player.BP_Player_C|GetBPC_AtmSystem _bp_player))
  (Default|AddItemonHand bpPlayer)
  (Utilities|FlowControl|Sequence
    (:then_0
      ;[0.2622 1 0.6244] Teleport player for atm
      (Transformation|SetWorldTransform (Variables|/Script/Engine.Actor|GetRootComponent (Variables|Default|GetBP%20Player)) (Math|Transform|MakeTransform (.location _returnvalue_3) (.rotation _returnvalue_3) "1.000000,1.000000,1.000000") false false) ; Teletransport player
      (Collision|SetCollisionEnabled (Variables|/Script/Engine.Character|GetCapsuleComponent (Variables|Default|GetBP%20Player)) "NoCollision") ; Allow player enter on the groud
      (Pawn|SetControlRotation (Game|GetPlayerController 0) (Transformation|GetActorRotation _returnvalue_2)) ; Set player to look foward
      (Variables|/Script/Engine.MovementComponent|SetVelocity (Variables|/Script/Engine.Character|GetCharacterMovement _returnvalue_2) "0, 0, 0")
      (Input|RemoveMappingContext _returnvalue_4 "/Game/Inputs/InputsPlayerMove/IMC_PlayerMovement.IMC_PlayerMovement" "(bIgnoreAllPressedKeysUntilRelease=True,bForceImmediately=False,bNotifyUserSettings=False)") ; Switch the mapping context for cashier
      (Input|AddMappingContext _returnvalue_4 "/Game/Inputs/InputsAtm/IMC_PlayerOnCashier.IMC_PlayerOnCashier" 0 "(bIgnoreAllPressedKeysUntilRelease=True,bForceImmediately=False,bNotifyUserSettings=False)"))
    (:then_1
      (EventDispatchers|BindEventtoOnPlayerExitCashier _bpc_atmsystem (delegate Custom|OnPlayerLeftCashier)))
    (:then_2
      (EventDispatchers|BindEventtoOnPlayerInteractinCashier _bpc_atmsystem (delegate Custom|OnPlayerInteractOnCashier)))
    (:then_3
      (bind _returnvalue_5 (Utilities|Time|SetTimerbyEvent (delegate Custom|UpdateLineTrace) 0.05 true))
      (Variables|Default|SetupdateLineTraceTimer _returnvalue_5))))

(event Collision|EventActorBeginOverlap
  (params (OtherActor :type Actor%20Object%20Reference))
  (|CallParentFunction OtherActor) ; This node is disabled and will not be called.\nDrag off pins to build functionality.
)

(fn ConstructionScript
  (|CallParentFunction)
  (Transformation|SetRelativeTransform (Variables|Default|GetArrow) (Variables|Default|GetteleportLocation) false false)
  (Variables|Default|SetqueuePoints (Utilities|Array|MakeArray (Variables|Default|GetQueu1) (Variables|Default|GetQueu2) (Variables|Default|GetQueu3) (Variables|Default|GetQueu4))))

(fn ActiveandDisableOutline
  (params (HitComponent :type Primitive%20Component%20Object%20Reference))
  (if (Components|ComponentHasTag HitComponent "outlineTag")
    (if (!= HitComponent (Variables|Default|GetlastComponentOutline))
      (Utilities|FlowControl|Sequence
        (:then_0
          (bind _lastcomponentoutline (Variables|Default|GetlastComponentOutline)
            (:then
              (Rendering|SetRenderCustomDepth _lastcomponentoutline false)
              (Variables|Default|SetlastComponentOutline 0))
            (:else)))
        (:then_1
          (bind _output_get (Variables|Default|SetlastComponentOutline HitComponent))
          (Rendering|SetRenderCustomDepth _output_get true))))
    (else
      (bind _lastcomponentoutline_2 (Variables|Default|GetlastComponentOutline)
        (:then
          (Rendering|SetRenderCustomDepth _lastcomponentoutline_2 false)
          (Variables|Default|SetlastComponentOutline 0))
        (:else)))))