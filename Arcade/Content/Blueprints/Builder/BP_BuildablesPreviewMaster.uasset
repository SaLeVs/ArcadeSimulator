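; Base preview actor for the building system that shows whether a buildable can be placed at its current spot.
; Its BuildCollision counts overlaps with components tagged BuildCollision, so placement stays blocked until every overlap ends.
; The count drives the valid or invalid preview material on BuildMesh and reports buildability to the builder controller through CanBuildEvent.
; BeginPlay starts it as buildable and makes CollisionMesh visible.
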(event OnComponentBeginOverlap(BuildCollision)
  (params (OverlappedComponent :type Primitive%20Component%20Object%20Reference) (OtherActor :type Actor%20Object%20Reference) (OtherComp :type Primitive%20Component%20Object%20Reference) (OtherBodyIndex :type Integer) (bFromSweep :type Boolean) (SweepResult :type Hit%20Result%20Structure%20%28by%20ref%29))
  (bind _bp_buildercontroller (Variables|Default|GetBP_BuilderController))
  (bind _buildmesh (Variables|Default|GetBuildMesh))
  ;[1 1 1] Collided with build, add count
  (if (Components|ComponentHasTag OtherComp "BuildCollision")
    (Default|CanBuildEvent (Variables|Default|GetBP_BuilderController) false) ; cant build
    (Math|Integer|IncrementInt (Variables|Default|GetcountColl)
      (:%20%20
        (if (> (Variables|Default|GetcountColl) 0)
          (Default|CanBuildEvent _bp_buildercontroller false) ; cant build
          (Rendering|Material|SetMaterial _buildmesh 0 "/Game/Materials/M_CantBuildingPreview.M_CantBuildingPreview")
          (else
            (Default|CanBuildEvent _bp_buildercontroller true) ; can build
            (Rendering|Material|SetMaterial _buildmesh 0 "/Game/Materials/M_BuildingPreview.M_BuildingPreview")))))))

(event OnComponentEndOverlap(BuildCollision)
  (params (OverlappedComponent :type Primitive%20Component%20Object%20Reference) (OtherActor :type Actor%20Object%20Reference) (OtherComp :type Primitive%20Component%20Object%20Reference) (OtherBodyIndex :type Integer))
  (bind _bp_buildercontroller (Variables|Default|GetBP_BuilderController))
  (bind _buildmesh (Variables|Default|GetBuildMesh))
  ;[1 1 1] Stop Colliding with one build
  (if (Components|ComponentHasTag OtherComp "BuildCollision")
    (Math|Integer|DecrementInt (Variables|Default|GetcountColl)
      (:%20%20
        ;[1 1 1] Collided with build, add count
        (if (> (Variables|Default|GetcountColl) 0)
          (Default|CanBuildEvent _bp_buildercontroller false) ; cant build
          (Rendering|Material|SetMaterial _buildmesh 0 "/Game/Materials/M_CantBuildingPreview.M_CantBuildingPreview")
          (else
            (Default|CanBuildEvent _bp_buildercontroller true) ; can build
            (Rendering|Material|SetMaterial _buildmesh 0 "/Game/Materials/M_BuildingPreview.M_BuildingPreview")))))))

(event EventBeginPlay
  (|CallParentFunction)
  (Default|CanBuildEvent (Variables|Default|GetBP_BuilderController) true) ; can build
  (Rendering|SetVisibility (Variables|Default|GetCollisionMesh) true false))

(event EventTick
  (params (DeltaSeconds :type Float%20%28single-precision%29))
  (|CallParentFunction DeltaSeconds))

(event Collision|EventActorBeginOverlap
  (params (OtherActor :type Actor%20Object%20Reference))
  (|CallParentFunction OtherActor) ; This node is disabled and will not be called.\nDrag off pins to build functionality.
)

(fn ConstructionScript
  (|CallParentFunction))