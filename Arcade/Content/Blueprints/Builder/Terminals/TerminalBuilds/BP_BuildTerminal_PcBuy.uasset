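; Buildable PC terminal, apparently for buying, that the player interacts with to use an on-screen computer widget.
; Interact snaps the player to an arrow placed by TeleportLocation, disables capsule collision, switches to the computer input context with cursor, and makes the terminal the view target.
; The player computer component's leave event restores movement input, collision, camera and crosshair, placing the player slightly below the arrow.
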(event Custom|PlayerExitPc
  (bind _returnvalue (Game|GetPlayerController 0))
  (bind _returnvalue_2 (PlayerController|LocalPlayerSubsystems|GetEnhancedInputLocalPlayerSubsystem _returnvalue))
  (Input|RemoveMappingContext _returnvalue_2 "/Game/Inputs/InputsComputer/IMC_PlayerOnComputer.IMC_PlayerOnComputer" "(bIgnoreAllPressedKeysUntilRelease=True,bForceImmediately=False,bNotifyUserSettings=False)")
  (Input|AddMappingContext _returnvalue_2 "/Game/Inputs/InputsPlayerMove/IMC_PlayerMovement.IMC_PlayerMovement" 0 "(bIgnoreAllPressedKeysUntilRelease=True,bForceImmediately=False,bNotifyUserSettings=False)")
  (CallFunction|TeletransportPlayerBackPc)
  (Default|RemoveItemonHand (Variables|Default|GetBp%20Player))
  (Utilities|IsValid (Game|GetPlayerController 0)
    (:Is%20Valid
      (Input|SetInputModeGameOnly (Variables|Default|GetPlayerController) false)
      (Variables|/Script/Engine.PlayerController|SetbShowMouseCursor (Variables|Default|GetPlayerController) false)
      (Game|Player|SetViewTargetwithBlend (Variables|Default|GetPlayerController) (Game|GetPlayerCharacter 0) 0.0 "VTBlend_Linear" 0.0 false)
      (Default|ShowCroshair (Variables|Default|GetBp%20Player) true) ; Function on player to display crosshair of viewport
    )))

(event EventInteract
  (params (bpPlayer :type BP%20Player%20Object%20Reference))
  (bind _returnvalue (Game|GetPlayerController 0))
  (bind _returnvalue_2 (PlayerController|LocalPlayerSubsystems|GetEnhancedInputLocalPlayerSubsystem _returnvalue))
  (Default|AddItemonHand bpPlayer)
  (Utilities|FlowControl|Sequence
    (:then_0
      (CallFunction|TeletransportPlayertoPc)
      (Input|RemoveMappingContext _returnvalue_2 "/Game/Inputs/InputsPlayerMove/IMC_PlayerMovement.IMC_PlayerMovement" "(bIgnoreAllPressedKeysUntilRelease=True,bForceImmediately=False,bNotifyUserSettings=False)") ; Switch the mapping context for cashier
      (Input|AddMappingContext _returnvalue_2 "/Game/Inputs/InputsComputer/IMC_PlayerOnComputer.IMC_PlayerOnComputer" 0 "(bIgnoreAllPressedKeysUntilRelease=True,bForceImmediately=False,bNotifyUserSettings=False)")
      (Utilities|IsValid self
        (:Is%20Valid
          (bind _output_get (Variables|Default|SetPlayerController (Game|GetPlayerController 0)))
          (Input|SetInputModeGameandUI _output_get (UserInterface|GetUserWidgetObject (Variables|Default|GetWidget)) "DoNotLock" true false)
          (Variables|/Script/Engine.PlayerController|SetbShowMouseCursor (Variables|Default|GetPlayerController) true)
          (Game|Player|SetViewTargetwithBlend (Variables|Default|GetPlayerController) self 0.0 "VTBlend_Linear" 0.0 false)
          (Default|ShowCroshair (Variables|Default|GetBp%20Player) false) ; Function on player to remove crosshair of viewport
          (Default|ChangeHint (Variables|/Game/Blueprints/Player/BP_Player.BP_Player_C|GetBPC_HintSystem (Variables|Default|GetBP%20Player)) "/Game/UI_Assets/Hints/Hint7PC.Hint7PC"))))
    (:then_1
      (EventDispatchers|BindEventtoOnPlayerLeftPc (Variables|/Game/Blueprints/Player/BP_Player.BP_Player_C|GetBPC_ComputerSystem (Variables|Default|GetBp%20Player)) (delegate Custom|PlayerExitPc)))))

(event Collision|EventActorBeginOverlap
  (params (OtherActor :type Actor%20Object%20Reference))
  (|CallParentFunction OtherActor) ; This node is disabled and will not be called.\nDrag off pins to build functionality.
)

(event EventTick
  (params (DeltaSeconds :type Float%20%28single-precision%29))
  (|CallParentFunction DeltaSeconds) ; This node is disabled and will not be called.\nDrag off pins to build functionality.
)

(event EventBeginPlay
  (|CallParentFunction) ; This node is disabled and will not be called.\nDrag off pins to build functionality.
)

(fn ConstructionScript
  (|CallParentFunction)
  (Transformation|SetRelativeTransform (Variables|Default|GetArrow) (Variables|Default|GetteleportLocation) false false))

(fn TeletransportPlayertoPc
  (bind _returnvalue (Game|GetPlayerCharacter 0))
  (bind _bp_player (Variables|Default|GetBp%20Player))
  (bind _arrow (Variables|Default|GetArrow))
  (bind _returnvalue_2 (Transformation|GetWorldTransform _arrow))
  (Transformation|SetWorldTransform (Variables|/Script/Engine.Actor|GetRootComponent _bp_player) (Math|Transform|MakeTransform (.location _returnvalue_2) (.rotation _returnvalue_2) "1.000000,1.000000,1.000000") false false) ; Teletransport player
  (Collision|SetCollisionEnabled (Variables|/Script/Engine.Character|GetCapsuleComponent _bp_player) "NoCollision") ; Allow player enter on the groud
  (if (== _bp_player _returnvalue)
    (Pawn|SetControlRotation (Game|GetPlayerController 0) (Transformation|GetActorRotation _returnvalue)) ; Set player to look foward
    (Variables|/Script/Engine.MovementComponent|SetVelocity (Variables|/Script/Engine.Character|GetCharacterMovement _returnvalue) "0, 0, 0")))

(fn TeletransportPlayerBackPc
  (bind _arrow (Variables|Default|GetArrow))
  (bind _returnvalue (Transformation|GetWorldTransform _arrow))
  (Transformation|SetWorldTransform (Variables|/Script/Engine.Actor|GetRootComponent (Variables|Default|GetBp%20Player)) (Math|Transform|MakeTransform (- (.location _returnvalue) "0.000000,0.000000,30.000000") (.rotation _returnvalue) "1.000000,1.000000,1.000000") false false) ; Teletransport player
  (Collision|SetCollisionEnabled (Variables|/Script/Engine.Character|GetCapsuleComponent (Variables|Default|GetBp%20Player)) "QueryAndPhysics") ; player can walk on ground
)