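; Cashier terminal where the player takes an NPC's payment and counts out change from an open drawer to earn money.
; Interacting locks the player at the register, swaps input mapping contexts and binds the player's ATM component events.
; Camera line traces collect NPC cash, add or remove tagged denominations on the monitor widget, and a timed trace outlines hovered money.
; Handing over correct change, compared as strings to dodge float error, credits the game instance.
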(event Custom|OnPlayerLeftCashier
  (bind _returnvalue (Game|GetPlayerController 0))
  (bind _returnvalue_2 (PlayerController|LocalPlayerSubsystems|GetEnhancedInputLocalPlayerSubsystem _returnvalue))
  ;[0.2622 1 0.6244] Teleport player for atm
  (Input|RemoveMappingContext _returnvalue_2 "/Game/Inputs/InputsAtm/IMC_PlayerOnCashier.IMC_PlayerOnCashier" "(bIgnoreAllPressedKeysUntilRelease=True,bForceImmediately=False,bNotifyUserSettings=False)")
  (Input|AddMappingContext _returnvalue_2 "/Game/Inputs/InputsPlayerMove/IMC_PlayerMovement.IMC_PlayerMovement" 0 "(bIgnoreAllPressedKeysUntilRelease=True,bForceImmediately=False,bNotifyUserSettings=False)")
  (CallFunction|TeletransportPlayerBackCashier)
  (Default|SetPlayerinATM (Variables|Default|GetBP%20Player) false)
  (Default|RemoveItemonHand (Variables|Default|GetBP%20Player))
  (Utilities|Time|ClearandInvalidateTimerbyHandle (Variables|Default|GetupdateLineTraceTimer)) ; stop line trace timer
  (CallFunction|UnbindAll) ; unbind events
  (CallFunction|ToggleDrawer false) ; close drawer
  (CallFunction|ActiveandDisableOutline (Variables|Default|GetmoneyArray)) ; turn off all outlines when exit
)

(event Custom|OnPlayerInteractOnCashier
  (bind _wbatm (Variables|Default|GetwbAtm))
  (bind _wbatm_2 (Variables|Default|GetwbAtm))
  (bind _bp_player (Variables|Default|GetBP%20Player))
  (bind _wbatm_3 (Variables|Default|GetwbAtm))
  (bind _camera (Variables|/Game/Blueprints/Player/BP_Player.BP_Player_C|GetCamera _bp_player))
  (bind _returnvalue (Transformation|GetWorldTransform _camera))
  (bind _outhit (Collision|LineTraceByChannel (.location _returnvalue) (+ (.location _returnvalue) (* (Math|Vector|GetForwardVector (.rotation _returnvalue)) 7e+02)) "TraceTypeQuery2" false 0 "ForDuration" false))
  (bind _caninteract (CallFunction|InteractMoney (.HitActor (Collision|BreakHitResult _outhit)))) ; Verify if player picked money of npc
  (if _caninteract
    (Utilities|FlowControl|Sequence
      (:then_0
        ;[0.2622 1 0.6244] Add money if hit on money component
        (bind _moneyvalue (CallFunction|SendMoneyValue (Variables|Default|GetmoneyArray) (.HitComponent (Collision|BreakHitResult _outhit)))) ; Pass the value according the array function
        (Variables|/Game/Widgets/WB_AtmMonitor.WB_AtmMonitor_C|SetmoneyGiving _wbatm (+ _moneyvalue (Variables|/Game/Widgets/WB_AtmMonitor.WB_AtmMonitor_C|GetmoneyGiving _wbatm)))
        (Default|UpdateMoneyValues _wbatm))
      (:then_1
        ;[0.2622 1 0.6244] calculating how many tokens we need to send
        (Utilities|IsValid (.HitComponent (Collision|BreakHitResult _outhit))
          (:Is%20Valid
            (if (Components|ComponentHasTag (.HitComponent (Collision|BreakHitResult _outhit)) "MoneyOnCashier") ; Compare if player hit on money on table for npc
              (if (Utilities|Enum|Equal(Enum) (Utilities|String|ToString(Float) (Variables|/Game/Widgets/WB_AtmMonitor.WB_AtmMonitor_C|GetmoneyChange _wbatm_3)) (Utilities|String|ToString(Float) (Variables|/Game/Widgets/WB_AtmMonitor.WB_AtmMonitor_C|GetmoneyGiving _wbatm_3))) ; If the change is correct
                (Rendering|SetVisibility (Variables|Default|GetMoneyDeliver) false true)
                (Variables|Default|SetmoneyToGain (- (Variables|/Game/Widgets/WB_AtmMonitor.WB_AtmMonitor_C|GetmoneyRecieved (Variables|Default|GetwbAtm)) (Variables|/Game/Widgets/WB_AtmMonitor.WB_AtmMonitor_C|GetmoneyGiving (Variables|Default|GetwbAtm))))
                (Variables|/Game/Widgets/WB_AtmMonitor.WB_AtmMonitor_C|SetmoneyRecieved _wbatm_2 0.0)
                (Variables|/Game/Widgets/WB_AtmMonitor.WB_AtmMonitor_C|SetmoneyGiving _wbatm_2 0.0)
                (Variables|/Game/Widgets/WB_AtmMonitor.WB_AtmMonitor_C|SetmoneyChange _wbatm_2 0.0) ; Reset values for other npc
                (Variables|/Game/Widgets/WB_AtmMonitor.WB_AtmMonitor_C|SetusedTokens (Variables|Default|GetwbAtm) 0)
                (Default|NpcDeliveryAnything _wbatm_2)
                (bind _asmy_game_instance (Utilities|Casting|CastToMyGameInstance (Game|GetGameInstance)))
                (Default|GainMoney _asmy_game_instance (Variables|Default|GetmoneyToGain))
                (Variables|Default|SetmoneyToGain 0.0)
                (Variables|Default|SettakenMoneyOnNPCHand false)
                (Default|CallOnMoneyDelivered2)))))))))

(event Custom|UnbindPlayerRemoveMoney
  (EventDispatchers|UnbindEventfromOnPlayerRemoveMoney (Variables|/Game/Blueprints/Player/BP_Player.BP_Player_C|GetBPC_AtmSystem (Variables|Default|GetBP%20Player)) (delegate Custom|PlayerRemoveMoney)))

(event Custom|PlayerRemoveMoney
  (bind _wbatm (Variables|Default|GetwbAtm))
  (bind _bp_player (Variables|Default|GetBP%20Player))
  (bind _camera (Variables|/Game/Blueprints/Player/BP_Player.BP_Player_C|GetCamera _bp_player))
  (bind _returnvalue (Transformation|GetWorldTransform _camera))
  ;[0.2622 1 0.6244] Retire money off cashier
  (bind _outhit (Collision|LineTraceByChannel (.location _returnvalue) (+ (.location _returnvalue) (* (Math|Vector|GetForwardVector (.rotation _returnvalue)) 7e+02)) "TraceTypeQuery1" false 0 "ForDuration" false))
  (bind _moneyvalue (CallFunction|SendMoneyValueBack (Variables|Default|GetmoneyArray) (.HitComponent (Collision|BreakHitResult _outhit))))
  (Variables|/Game/Widgets/WB_AtmMonitor.WB_AtmMonitor_C|SetmoneyGiving _wbatm (+ _moneyvalue (Variables|/Game/Widgets/WB_AtmMonitor.WB_AtmMonitor_C|GetmoneyGiving _wbatm)))
  (Default|UpdateMoneyValues _wbatm))

(event Custom|UpdateLineTrace2
  (bind _bp_player (Variables|Default|GetBP%20Player))
  (bind _camera (Variables|/Game/Blueprints/Player/BP_Player.BP_Player_C|GetCamera _bp_player))
  (bind _returnvalue (Transformation|GetWorldTransform _camera))
  ;[0.2622 1 0.6244] Update line trace for outline money
  (bind _outhit (Collision|LineTraceByChannel (.location _returnvalue) (+ (.location _returnvalue) (* (Math|Vector|GetForwardVector (.rotation _returnvalue)) 7e+02)) "TraceTypeQuery1" false 0 "None" false))
  (CallFunction|ActiveandDisableOutline (Variables|Default|GetmoneyArray) (.HitComponent (Collision|BreakHitResult _outhit))))

(event Custom|UnbindOnPlayerInteractOnCashier
  (EventDispatchers|UnbindEventfromOnPlayerInteractinCashier (Variables|/Game/Blueprints/Player/BP_Player.BP_Player_C|GetBPC_AtmSystem (Variables|Default|GetBP%20Player)) (delegate Custom|OnPlayerInteractOnCashier)))

(event Custom|UnbindOnPlayerLeftCashier
  (EventDispatchers|UnbindEventfromOnPlayerExitCashier (Variables|/Game/Blueprints/Player/BP_Player.BP_Player_C|GetBPC_AtmSystem (Variables|Default|GetBP%20Player)) (delegate Custom|OnPlayerLeftCashier)))

(event EventInteract
  (params (bpPlayer :type BP%20Player%20Object%20Reference))
  (bind _returnvalue (Game|GetPlayerController 0))
  (bind _bp_player (Variables|Default|GetBP%20Player))
  (bind _returnvalue_2 (PlayerController|LocalPlayerSubsystems|GetEnhancedInputLocalPlayerSubsystem _returnvalue))
  (bind _bpc_atmsystem (Variables|/Game/Blueprints/Player/BP_Player.BP_Player_C|GetBPC_AtmSystem _bp_player))
  (Default|AddItemonHand bpPlayer)
  (Utilities|FlowControl|Sequence
    (:then_0
      ;[0.2622 1 0.6244] Teleport player for atm
      (CallFunction|TeletransportPlayertoCashier)
      (Default|SetPlayerinATM (Variables|Default|GetBP%20Player) true)
      (Input|RemoveMappingContext _returnvalue_2 "/Game/Inputs/InputsPlayerMove/IMC_PlayerMovement.IMC_PlayerMovement" "(bIgnoreAllPressedKeysUntilRelease=True,bForceImmediately=False,bNotifyUserSettings=False)") ; Switch the mapping context for cashier
      (Input|AddMappingContext _returnvalue_2 "/Game/Inputs/InputsAtm/IMC_PlayerOnCashier.IMC_PlayerOnCashier" 0 "(bIgnoreAllPressedKeysUntilRelease=True,bForceImmediately=False,bNotifyUserSettings=False)"))
    (:then_1
      (EventDispatchers|BindEventtoOnPlayerExitCashier _bpc_atmsystem (delegate Custom|OnPlayerLeftCashier)))
    (:then_2
      (EventDispatchers|BindEventtoOnPlayerInteractinCashier _bpc_atmsystem (delegate Custom|OnPlayerInteractOnCashier)))
    (:then_3
      (EventDispatchers|BindEventtoOnPlayerRemoveMoney _bpc_atmsystem (delegate Custom|PlayerRemoveMoney)))
    (:then_4
      (CallFunction|ToggleDrawer true)
      (bind _returnvalue_3 (Utilities|Time|SetTimerbyEvent (delegate Custom|UpdateLineTrace2) 0.05 true))
      (Variables|Default|SetupdateLineTraceTimer _returnvalue_3))))

(event EventBeginPlay
  ;[0.2622 1 0.6244] Pass the reference for widget
  (|CallParentFunction)
  (bind _aswb_atm_monitor (Utilities|Casting|CastToWB_AtmMonitor (UserInterface|GetUserWidgetObject (Variables|Default|GetWidget))))
  (Variables|Default|SetwbAtm _aswb_atm_monitor))

(event EventTick
  (params (DeltaSeconds :type Float%20%28single-precision%29))
  (|CallParentFunction DeltaSeconds))

(event Collision|EventActorBeginOverlap
  (params (OtherActor :type Actor%20Object%20Reference))
  (|CallParentFunction OtherActor) ; This node is disabled and will not be called.\nDrag off pins to build functionality.
)

(fn ConstructionScript
  (|CallParentFunction)
  (Transformation|SetRelativeTransform (Variables|Default|GetArrow) (Variables|Default|GetteleportLocation) false false)
  (Variables|Default|SetmoneyArray (Utilities|Array|MakeArray (Variables|Default|Get50_Dolar) (Variables|Default|Get20_Dolar) (Variables|Default|Get10_Dolar) (Variables|Default|Get5_Dolar) (Variables|Default|Get1_Dolar) (Variables|Default|Get50_Cent) (Variables|Default|Get25_Cent) (Variables|Default|Get10_Cent) (Variables|Default|Get5_Cent) (Variables|Default|Get1_Cent) (Variables|Default|GetMoney1)))
  (Variables|Default|SetqueuePoints (Utilities|Array|MakeArray (Variables|Default|GetQueuePoint1) (Variables|Default|GetQueuePoint2) (Variables|Default|GetQueuePoint3) (Variables|Default|GetQueuePoint4))))

(fn ActiveandDisableOutline
  (params (MoneyComponent :type Array%20of%20Static%20Mesh%20Component%20Object%20References) (HitComponent :type Primitive%20Component%20Object%20Reference))
  (if (not (Utilities|Array|IsEmpty MoneyComponent))
    (for _array_element MoneyComponent
      (Utilities|IsValid _array_element
        (:Is%20Valid
          (bind _output_get (Variables|Components|SetArray%20Element_0 _array_element))
          (if (== _output_get HitComponent)
            (Rendering|SetRenderCustomDepth (Variables|Components|GetArray%20Element_0) true)
            (else
              (Rendering|SetRenderCustomDepth (Variables|Components|GetArray%20Element_0) false))))))
    (Variables|Components|SetArray%20Element_0 0)))

(fn SendMoneyValue
  (params (moneyComponent :type Array%20of%20Static%20Mesh%20Component%20Object%20References) (hitComponent :type Primitive%20Component%20Object%20Reference))
  (Variables|Components|SetArray%20Element_0 0)
  (Variables|Default|SetmoneyValeuForSend 0.0) ; Reset values
  (if (and (not (Utilities|Array|IsEmpty moneyComponent)) (Variables|Default|GettakenMoneyOnNPCHand))
    (for _array_element moneyComponent
      (Utilities|IsValid _array_element
        (:Is%20Valid
          (bind _output_get (Variables|Components|SetArray%20Element_0 _array_element))
          (if (== _output_get hitComponent)
            (for _array_element_2 (Variables|/Script/Engine.ActorComponent|GetComponentTags (Variables|Components|GetArray%20Element_0))
              (switch string (Utilities|String|ToString(Name) _array_element_2) ; Pass the value according the tag off object hitted
                (:1Dolar
                  (Variables|Default|SetmoneyValeuForSend 1.0))
                (:5Dolar
                  (Variables|Default|SetmoneyValeuForSend 5.0))
                (:10Dolar
                  (Variables|Default|SetmoneyValeuForSend 1e+01))
                (:20Dolar
                  (Variables|Default|SetmoneyValeuForSend 2e+01))
                (:50Dolar
                  (Variables|Default|SetmoneyValeuForSend 5e+01))
                (:1Cent
                  (Variables|Default|SetmoneyValeuForSend 0.01))
                (:5Cent
                  (Variables|Default|SetmoneyValeuForSend 0.05))
                (:10Cent
                  (Variables|Default|SetmoneyValeuForSend 0.1))
                (:25Cent
                  (Variables|Default|SetmoneyValeuForSend 0.25))
                (:50Cent
                  (Variables|Default|SetmoneyValeuForSend 0.5)))
              (Rendering|SetVisibility (Variables|Default|GetMoneyDeliver) true true))))))
    (Variables|Components|SetArray%20Element_0 0)
    (Variables|Components|SetArray%20Element_0 0)
    (return (Variables|Default|GetmoneyValeuForSend))))

(fn SendMoneyValueBack
  (params (moneyComponent :type Array%20of%20Static%20Mesh%20Component%20Object%20References) (hitComponent :type Primitive%20Component%20Object%20Reference))
  (Variables|Components|SetArray%20Element_0 0)
  (Variables|Default|SetmoneyValeuForSend 0.0)
  (if (not (Utilities|Array|IsEmpty moneyComponent))
    (for _array_element moneyComponent
      (Utilities|IsValid _array_element
        (:Is%20Valid
          (bind _output_get (Variables|Components|SetArray%20Element_0 _array_element))
          (if (== _output_get hitComponent)
            (for _array_element_2 (Variables|/Script/Engine.ActorComponent|GetComponentTags (Variables|Components|GetArray%20Element_0))
              (switch string (Utilities|String|ToString(Name) _array_element_2)
                (:1Dolar
                  (Variables|Default|SetmoneyValeuForSend -1.0))
                (:5Dolar
                  (Variables|Default|SetmoneyValeuForSend -5.0))
                (:10Dolar
                  (Variables|Default|SetmoneyValeuForSend -1e+01))
                (:20Dolar
                  (Variables|Default|SetmoneyValeuForSend -2e+01))
                (:50Dolar
                  (Variables|Default|SetmoneyValeuForSend -5e+01))
                (:1Cent
                  (Variables|Default|SetmoneyValeuForSend -0.01))
                (:5Cent
                  (Variables|Default|SetmoneyValeuForSend -0.05))
                (:10Cent
                  (Variables|Default|SetmoneyValeuForSend -0.1))
                (:25Cent
                  (Variables|Default|SetmoneyValeuForSend -0.25))
                (:50Cent
                  (Variables|Default|SetmoneyValeuForSend -0.5))))))))
    (Variables|Components|SetArray%20Element_0 0)
    (Variables|Components|SetArray%20Element_0 0)
    (return (Variables|Default|GetmoneyValeuForSend))))

(fn SendTokensValue
  (bind _wbatm (Variables|Default|GetwbAtm))
  (bind _result (Math|Integer|IncrementInt (Variables|Default|GetCoinsGiving))
    (:%20%20
      (Variables|/Game/Widgets/WB_AtmMonitor.WB_AtmMonitor_C|SetTokensRecieving _wbatm _result)
      (return _wbatm))))

(fn InteractMoney
  (params (hitComponent :type Actor%20Object%20Reference))
  (bind _wbatm (Variables|Default|GetwbAtm))
  (Utilities|IsValid hitComponent
    (:Is%20Valid
      (if (Components|ComponentHasTag (Variables|/Script/Engine.Actor|GetRootComponent hitComponent) "MoneyMesh")
        (Utilities|FlowControl|Sequence
          (:then_0
            (bind _asbp_npcmaster (Utilities|Casting|CastToBP_NPCMaster (Actor|GetAttachParentActor hitComponent)))
            (Default|ChangeAnim _asbp_npcmaster)
            (Variables|Default|SettakenMoneyOnNPCHand true))
          (:then_1
            (bind _returnvalue (Actor|GetActorOfClass "/Game/Blueprints/Cashier/BP_NpcMoney.BP_NpcMoney_C"))
            (Variables|/Game/Widgets/WB_AtmMonitor.WB_AtmMonitor_C|SetmoneyChange _wbatm (Variables|/Game/Blueprints/Cashier/BP_NpcMoney.BP_NpcMoney_C|GetchangeNpc _returnvalue))
            (Variables|/Game/Widgets/WB_AtmMonitor.WB_AtmMonitor_C|SetmoneyRecieved _wbatm (Variables|/Game/Blueprints/Cashier/BP_NpcMoney.BP_NpcMoney_C|GetmoneyNpc _returnvalue))
            (Variables|/Game/Widgets/WB_AtmMonitor.WB_AtmMonitor_C|SetusedTokens _wbatm (Variables|/Game/Blueprints/Cashier/BP_NpcMoney.BP_NpcMoney_C|GetcoinsNpc _returnvalue))
            (Actor|DestroyActor hitComponent)
            (Default|UpdateMoneyValues _wbatm)
            (Default|TokensUpdate _wbatm)
            (return true)))))))

(fn UnbindAll
  (Utilities|FlowControl|Sequence
    (:then_0
      (CallFunction|UnbindPlayerRemoveMoney))
    (:then_1
      (CallFunction|UnbindonPlayerInteractonCashier))
    (:then_2
      (CallFunction|UnbindonPlayerLeftCashier))))

(fn ToggleDrawer
  (params (toggle :type Boolean))
  (bind _drawer (Variables|Default|GetDrawer))
  (bind _relativelocation (Variables|/Script/Engine.SceneComponent|GetRelativeLocation _drawer))
  (if toggle
    (Transformation|SetRelativeLocation _drawer (+ _relativelocation "0.000000,34.000000,0.000000") false false)
    (Rendering|SetVisibility (Variables|Default|GetmoneyOnDrawer) true false)
    (else
      (Transformation|SetRelativeLocation _drawer (- _relativelocation "0.000000,34.000000,0.000000") false false)
      (Rendering|SetVisibility (Variables|Default|GetmoneyOnDrawer) false false))))

(fn TeletransportPlayertoCashier
  (bind _returnvalue (Game|GetPlayerCharacter 0))
  (bind _arrow (Variables|Default|GetArrow))
  (bind _returnvalue_2 (Transformation|GetWorldTransform _arrow))
  (Variables|/Script/Engine.CharacterMovementComponent|SetGravityScale (Variables|/Script/Engine.Character|GetCharacterMovement (Game|GetPlayerCharacter 0)) 0.0)
  (Transformation|SetWorldTransform (Variables|/Script/Engine.Actor|GetRootComponent (Variables|Default|GetBP%20Player)) (Math|Transform|MakeTransform (.location _returnvalue_2) (.rotation _returnvalue_2) "1.000000,1.000000,1.000000") false false) ; Teletransport player
  (Collision|SetCollisionEnabled (Variables|/Script/Engine.Character|GetCapsuleComponent (Variables|Default|GetBP%20Player)) "NoCollision") ; Allow player enter on the groud
  (if (== (Variables|Default|GetBP%20Player) _returnvalue)
    (Pawn|SetControlRotation (Game|GetPlayerController 0) (Transformation|GetActorRotation _returnvalue)) ; Set player to look foward
    (Variables|/Script/Engine.MovementComponent|SetVelocity (Variables|/Script/Engine.Character|GetCharacterMovement _returnvalue) "0, 0, 0")))

(fn TeletransportPlayerBackCashier
  (bind _arrow (Variables|Default|GetArrow))
  (bind _returnvalue (Transformation|GetWorldTransform _arrow))
  (Variables|/Script/Engine.CharacterMovementComponent|SetGravityScale (Variables|/Script/Engine.Character|GetCharacterMovement (Game|GetPlayerCharacter 0)) 1.0)
  (Transformation|SetWorldTransform (Variables|/Script/Engine.Actor|GetRootComponent (Variables|Default|GetBP%20Player)) (Math|Transform|MakeTransform (- (.location _returnvalue) "0.000000,0.000000,-30.000000") (.rotation _returnvalue) "1.000000,1.000000,1.000000") false false) ; Teletransport player
  (Collision|SetCollisionEnabled (Variables|/Script/Engine.Character|GetCapsuleComponent (Variables|Default|GetBP%20Player)) "QueryAndPhysics") ; player can walk on ground
)