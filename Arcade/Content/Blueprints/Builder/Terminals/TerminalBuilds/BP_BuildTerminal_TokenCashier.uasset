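; Token cashier terminal where the player hands out tokens to the first queued NPC.
; Interacting teleports the player to the counter without gravity or collision and swaps to a cashier input context until exit.
; Camera traces on interact use component tags to count tokens onto the counter, update the NPC's bubble, then broadcast thumbs-up and delivery events once the amount is met.
; A looping timer traces to outline targeted components through custom depth.
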(event Custom|OnPlayerLeftTokenCashier
  (bind _returnvalue (Game|GetPlayerController 0))
  (bind _returnvalue_2 (PlayerController|LocalPlayerSubsystems|GetEnhancedInputLocalPlayerSubsystem _returnvalue))
  ;[0.2622 1 0.6244] Teleport player for atm
  (Input|RemoveMappingContext _returnvalue_2 "/Game/Inputs/InputsTokenCashier/IMC_PlayerOnTokenCashier.IMC_PlayerOnTokenCashier" "(bIgnoreAllPressedKeysUntilRelease=True,bForceImmediately=False,bNotifyUserSettings=False)")
  (Input|AddMappingContext _returnvalue_2 "/Game/Inputs/InputsPlayerMove/IMC_PlayerMovement.IMC_PlayerMovement" 0 "(bIgnoreAllPressedKeysUntilRelease=True,bForceImmediately=False,bNotifyUserSettings=False)")
  (CallFunction|PlayerTeleportBackTokenCashier)
  (Default|RemoveItemonHand (Variables|Default|GetBP%20Player))
  (Utilities|Time|ClearandInvalidateTimerbyHandle (Variables|Default|GetupdateLineTraceTimer))
  (CallFunction|UnbindAll))

(event Custom|OnPlayerInteractOnTokenCashier
  (bind _bp_player (Variables|Default|GetBP%20Player))
  (bind _npconfirst (Variables|Default|GetNpcOnFirst))
  (bind _camera (Variables|/Game/Blueprints/Player/BP_Player.BP_Player_C|GetCamera _bp_player))
  (bind _returnvalue (Transformation|GetWorldTransform _camera))
  (bind _outhit (Collision|LineTraceByChannel (.location _returnvalue) (+ (.location _returnvalue) (* (Math|Vector|GetForwardVector (.rotation _returnvalue)) 7e+02)) "TraceTypeQuery1" false 0 "ForDuration" false))
  (Utilities|FlowControl|Sequence
    (:then_0
      ;[0.2622 1 0.6244] calculating how many tokens we need to send
      (Utilities|IsValid (.HitComponent (Collision|BreakHitResult _outhit))
        (:Is%20Valid
          (if (Components|ComponentHasTag (.HitComponent (Collision|BreakHitResult _outhit)) "TipsMesh") ; True = Player hit tipSuport
            (if (< (Variables|Default|GetgivedTokens) (Variables|Default|GettokensToGive)) ; true = can give more\nfalse = cant give more
              (bind _result (Math|Integer|IncrementInt (Variables|Default|GetgivedTokens))
                (:%20%20
                  (Variables|/Game/Blueprints/AI/BP_NPCMaster.BP_NPCMaster_C|SettokensForRecieve _npconfirst _result)
                  (Default|UpdateBubbleValue _npconfirst) ; Update the tokens value on bubble
                  (Rendering|SetVisibility (Variables|Default|GetTips) true true))))))))
    (:then_1
      ;[0.2622 1 0.6244] Verify if player delivery money and tokens
      (Utilities|IsValid (.HitComponent (Collision|BreakHitResult _outhit))
        (:Is%20Valid
          (if (Components|ComponentHasTag (.HitComponent (Collision|BreakHitResult _outhit)) "tipsOnCashier") ; Compare if player hit on tokens on table for npc
            (if (>= (Variables|Default|GetgivedTokens) (Variables|Default|GettokensToGive)) ; true = can give more\nfalse = cant give more, give to npc
              (Variables|Default|SetgivedTokens 0)
              (Variables|Default|SettokensToGive 0)
              (Rendering|SetVisibility (Variables|Default|GetTips) false true)
              (Default|CallOnThumbsUp)
              (Utilities|FlowControl|Delay 1.6) ; thumbs up anim
              (Default|CallOnTokenDelivered))))))))

(event Custom|UnbindOnPlayerInteractOnTokenCashier
  (EventDispatchers|UnbindEventfromOnPlayerInteractinTokenCashier (Variables|/Game/Blueprints/Player/BP_Player.BP_Player_C|GetBPC_AtmSystem (Variables|Default|GetBP%20Player)) (delegate Custom|OnPlayerInteractOnTokenCashier)))

(event Custom|UpdateLineTrace
  (bind _bp_player (Variables|Default|GetBP%20Player))
  (bind _camera (Variables|/Game/Blueprints/Player/BP_Player.BP_Player_C|GetCamera _bp_player))
  (bind _returnvalue (Transformation|GetWorldTransform _camera))
  ;[0.2622 1 0.6244] Update line trace for outline money (Need to exist cuz have item on hand)
  (bind (_outhit _returnvalue_2) (Collision|LineTraceByChannel (.location _returnvalue) (+ (.location _returnvalue) (* (Math|Vector|GetForwardVector (.rotation _returnvalue)) 7e+02)) "TraceTypeQuery1" false 0 "None" false))
  (if _returnvalue_2
    (CallFunction|ActiveandDisableOutline (.HitComponent (Collision|BreakHitResult _outhit)))))

(event Custom|UnbindOnPlayerLeftTokenCashier
  (EventDispatchers|UnbindEventfromOnPlayerExitTokenCashier (Variables|/Game/Blueprints/Player/BP_Player.BP_Player_C|GetBPC_AtmSystem (Variables|Default|GetBP%20Player)) (delegate Custom|OnPlayerLeftTokenCashier)))

(event EventBeginPlay
  (|CallParentFunction))

(event EventTick
  (params (DeltaSeconds :type Float%20%28single-precision%29))
  (|CallParentFunction DeltaSeconds))

(event EventInteract
  (params (bpPlayer :type BP%20Player%20Object%20Reference))
  (bind _returnvalue (Game|GetPlayerController 0))
  (bind _bp_player (Variables|Default|GetBP%20Player))
  (bind _returnvalue_2 (PlayerController|LocalPlayerSubsystems|GetEnhancedInputLocalPlayerSubsystem _returnvalue))
  (bind _bpc_atmsystem (Variables|/Game/Blueprints/Player/BP_Player.BP_Player_C|GetBPC_AtmSystem _bp_player))
  (Default|AddItemonHand bpPlayer)
  (Utilities|FlowControl|Sequence
    (:then_0
      ;[0.2622 1 0.6244] Teleport player for atm
      (CallFunction|PlayerTeleporttoTokenCashier)
      (Input|RemoveMappingContext _returnvalue_2 "/Game/Inputs/InputsPlayerMove/IMC_PlayerMovement.IMC_PlayerMovement" "(bIgnoreAllPressedKeysUntilRelease=True,bForceImmediately=False,bNotifyUserSettings=False)") ; Switch the mapping context for cashier
      (Input|AddMappingContext _returnvalue_2 "/Game/Inputs/InputsTokenCashier/IMC_PlayerOnTokenCashier.IMC_PlayerOnTokenCashier" 0 "(bIgnoreAllPressedKeysUntilRelease=True,bForceImmediately=False,bNotifyUserSettings=False)"))
    (:then_1
      (EventDispatchers|AssignOnPlayerExitTokenCashier _bpc_atmsystem (delegate Custom|OnPlayerLeftTokenCashier)))
    (:then_2
      (EventDispatchers|BindEventtoOnPlayerInteractinTokenCashier _bpc_atmsystem (delegate Custom|OnPlayerInteractOnTokenCashier)))
    (:then_3
      (bind _returnvalue_3 (Utilities|Time|SetTimerbyEvent (delegate Custom|UpdateLineTrace) 0.05 true))
      (Variables|Default|SetupdateLineTraceTimer _returnvalue_3))))

(event Collision|EventActorBeginOverlap
  (params (OtherActor :type Actor%20Object%20Reference))
  (|CallParentFunction OtherActor) ; This node is disabled and will not be called.\nDrag off pins to build functionality.
)

(fn ConstructionScript
  (|CallParentFunction)
  (Transformation|SetRelativeTransform (Variables|Default|GetArrow) (Variables|Default|GetteleportLocation) false false)
  (Variables|Default|SetqueuePoints (Utilities|Array|MakeArray (Variables|Default|GetQueuePoint1) (Variables|Default|GetQueuePoint2) (Variables|Default|GetQueuePoint3) (Variables|Default|GetQueuePoint4))))

(fn ActiveandDisableOutline
  (params (HitComponent :type Primitive%20Component%20Object%20Reference))
  (if (Components|ComponentHasTag HitComponent "outlineTag")
    (if (!= HitComponent (Variables|Default|GetlastComponentOutline))
      (Utilities|FlowControl|Sequence
        (:then_0
          (bind _lastcomponentoutline (Variables|Default|GetlastComponentOutline)
            (:then
              (Rendering|SetRenderCustomDepth _lastcomponentoutline false)
              (Variables|Default|SetlastComponentOutline 0))
            (:else)))
        (:then_1
          (bind _output_get (Variables|Default|SetlastComponentOutline HitComponent))
          (Rendering|SetRenderCustomDepth _output_get true))))
    (else
      (bind _lastcomponentoutline_2 (Variables|Default|GetlastComponentOutline)
        (:then
          (Rendering|SetRenderCustomDepth _lastcomponentoutline_2 false)
          (Variables|Default|SetlastComponentOutline 0))
        (:else)))))

(fn UnbindAll
  (Utilities|FlowControl|Sequence
    (:then_0
      (CallFunction|UnbindonPlayerInteractonTokenCashier))
    (:then_1
      (CallFunction|UnbindonPlayerLeftTokenCashier))))

(fn PlayerTeleporttoTokenCashier
  (bind _returnvalue (Game|GetPlayerCharacter 0))
  (bind _arrow (Variables|Default|GetArrow))
  (bind _returnvalue_2 (Transformation|GetWorldTransform _arrow))
  (Variables|/Script/Engine.CharacterMovementComponent|SetGravityScale (Variables|/Script/Engine.Character|GetCharacterMovement (Game|GetPlayerCharacter 0)) 0.0)
  (Transformation|SetWorldTransform (Variables|/Script/Engine.Actor|GetRootComponent (Variables|Default|GetBP%20Player)) (Math|Transform|MakeTransform (.location _returnvalue_2) (.rotation _returnvalue_2) "1.000000,1.000000,1.000000") false false) ; Teletransport player
  (Collision|SetCollisionEnabled (Variables|/Script/Engine.Character|GetCapsuleComponent (Variables|Default|GetBP%20Player)) "NoCollision") ; Allow player enter on the groud
  (if (== (Variables|Default|GetBP%20Player) _returnvalue)
    (Pawn|SetControlRotation (Game|GetPlayerController 0) (Transformation|GetActorRotation _returnvalue)) ; Set player to look foward
    (Variables|/Script/Engine.MovementComponent|SetVelocity (Variables|/Script/Engine.Character|GetCharacterMovement _returnvalue) "0, 0, 0")))

(fn PlayerTeleportBackTokenCashier
  (bind _arrow (Variables|Default|GetArrow))
  (bind _returnvalue (Transformation|GetWorldTransform _arrow))
  (Variables|/Script/Engine.CharacterMovementComponent|SetGravityScale (Variables|/Script/Engine.Character|GetCharacterMovement (Game|GetPlayerCharacter 0)) 1.0)
  (Transformation|SetWorldTransform (Variables|/Script/Engine.Actor|GetRootComponent (Variables|Default|GetBP%20Player)) (Math|Transform|MakeTransform (- (.location _returnvalue) "0.000000,0.000000,-30.000000") (.rotation _returnvalue) "1.000000,1.000000,1.000000") false false) ; Teletransport player
  (Collision|SetCollisionEnabled (Variables|/Script/Engine.Character|GetCapsuleComponent (Variables|Default|GetBP%20Player)) "QueryAndPhysics") ; player can walk on ground
)