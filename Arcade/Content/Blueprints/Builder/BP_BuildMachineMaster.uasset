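; Base Blueprint for builder machines that shows its CollisionMesh only while build mode is active.
; On BeginPlay it caches the first BP_BuilderController found in the level, hides the mesh and binds to the controller's OnBuildModeChanged.
; That event passes the build mode flag straight to the mesh's visibility, without changing its collision settings.
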(event Custom|OnBuildModeChanged
  (params (InBuildMode :type Boolean))
  ;[1 1 1] Listen OnBuildModeChanged
  ;[1 1 1] Turn ON CollisionMesh
  (Rendering|SetVisibility (Variables|Default|GetCollisionMesh) InBuildMode false))

(event EventBeginPlay
  (|CallParentFunction)
  (Utilities|FlowControl|Sequence
    (:then_0
      ;[1 1 1] Get builder controller
      (bind _outactors (Actor|GetAllActorsOfClass "/Game/Blueprints/Builder/BuilderStuff/BP_BuilderController.BP_BuilderController_C"))
      (if (> (Utilities|Array|Length _outactors) 0)
        (Variables|Default|SetBP_BuilderController (Utilities|Array|Get(acopy) _outactors))))
    (:then_1
      ;[1 1 1] Turn OFF CollisionMesh
      (Rendering|SetVisibility (Variables|Default|GetCollisionMesh) false false))
    (:then_2
      ;[1 1 1] Listen OnBuildModeChanged
      (EventDispatchers|BindEventtoOnBuildModeChanged (Variables|Default|GetBP_BuilderController) (delegate Custom|OnBuildModeChanged)))))

(event Collision|EventActorBeginOverlap
  (params (OtherActor :type Actor%20Object%20Reference))
  (|CallParentFunction OtherActor) ; This node is disabled and will not be called.\nDrag off pins to build functionality.
)

(event EventTick
  (params (DeltaSeconds :type Float%20%28single-precision%29))
  (|CallParentFunction DeltaSeconds) ; This node is disabled and will not be called.\nDrag off pins to build functionality.
)

(fn ConstructionScript
  (|CallParentFunction))