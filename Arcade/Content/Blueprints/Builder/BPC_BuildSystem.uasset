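; Player build-system component that previews, places and destroys buildings defined in DT_BuildParts.
; While build mode is on, Tick traces from the camera to move a preview actor along Z=0, and the mouse wheel rotates it in 45-degree steps.
; Placement spawns the real Blueprint if BP_BuilderController allows it, then exits, destroying the preview and the player's held box.
; Destroy input removes traced actors tagged Buildable.
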(event Custom|Preview%20Loop
  ;[1 1 1] Mesh Trace
  (bind (_outhit _returnvalue) (Collision|LineTraceByChannel (Variables|Default|GetTraceStart) (Variables|Default|GetTraceEnd) "TraceTypeQuery1" false 0 "None"))
  (if _returnvalue
    (Utilities|FlowControl|Sequence
      (:then_0
        ;[1 1 1] Create Build Preview Once
        (Utilities|FlowControl|DoOnce false
          (:Completed
            (bind _returnvalue_2 (Game|SpawnActorfromClass (.BluePrintPreview (Utilities|Struct|BreakS_BuildParts (Utilities|Array|Get(acopy) (Variables|Default|GetDT_Buildables) (Variables|Default|GetbuildableIndex)))) (Variables|Default|GetBuild%20Preview%20Transform) "AlwaysSpawn" "MultiplyWithRoot" 0 0))
            (Variables|Default|SetBP_BuildPreview _returnvalue_2))))
      (:then_1
        ;[1 1 1] Check if can build
        (bind (_outhit_2 _returnvalue_3) (Collision|LineTraceByChannel (Variables|Default|GetTraceStart) (Variables|Default|GetTraceEnd) "TraceTypeQuery2" false 0 "None")) ; Collision Trace
        (if _returnvalue_3
          (bind _asbox_collision (Utilities|Casting|CastToBoxComponent (.HitComponent (Collision|BreakHitResult _outhit_2))))
          (if (Components|ComponentHasTag _asbox_collision "BuildCollision")
            _)))
      (:then_2
        ;[1 1 1] Set the Position of the Preview
        (bind _output_get (Variables|Default|SetBuild%20Preview%20Transform (Math|Transform|MakeTransform (Math|Vector|MakeVector (.X (Math|Vector|BreakVector (.Location (Collision|BreakHitResult _outhit)))) (.Y (Math|Vector|BreakVector (.Location (Collision|BreakHitResult _outhit)))) 0.0) (Variables|Default|GetBuildPreviewRotation) "1.000000,1.000000,1.000000")))
        (Transformation|SetActorTransform (Variables|Default|GetBP_BuildPreview) _output_get)))))

(event Custom|Reset%20Build%20Mode
  ;[1 1 1] Reset Player Build
  (Actor|DestroyActor (Variables|Default|GetBP_BoxInHand)) ; Destroy box in hand
  (Variables|Default|SetBP_BoxInHand 0)
  (Variables|/Game/Blueprints/Player/BP_Player.BP_Player_C|SethaveBoxInHands (Variables|Default|GetPlayer%20BP) false)
  ;[1 1 1] Create Build Preview Once
  (Utilities|FlowControl|DoOnce false) ; enters at Reset
)

(event Custom|Stop%20Build%20Mode
  (bind _bp_buildercontroller (Variables|Default|GetBP_BuilderController))
  ;[1 1 1] Input Preview
  (bind _output_get (Variables|Default|SetinBuildMode false))
  (Utilities|FlowControl|Sequence
    (:then_0
      (Default|IsinBuildMode _bp_buildercontroller _output_get)
      (bind _bp_buildpreview (Variables|Default|GetBP_BuildPreview)
        (:then
          (Actor|DestroyActor _bp_buildpreview)
          (Variables|Default|SetBP_BuildPreview 0)
          (CallFunction|ResetBuildMode))
        (:else)))
    (:then_1
      (Default|CanBuildEvent _bp_buildercontroller true))))

(event Custom|Preview
  (bind _bp_buildercontroller (Variables|Default|GetBP_BuilderController))
  ;[1 1 1] Input Preview
  (if (not (Variables|Default|GetinBuildMode))
    (bind _output_get (Variables|Default|SetinBuildMode true))
    (Default|IsinBuildMode (Variables|Default|GetBP_BuilderController) _output_get)
    (else
      (bind _output_get_2 (Variables|Default|SetinBuildMode false))
      (Utilities|FlowControl|Sequence
        (:then_0
          (Default|IsinBuildMode _bp_buildercontroller _output_get_2)
          (bind _bp_buildpreview (Variables|Default|GetBP_BuildPreview)
            (:then
              (Actor|DestroyActor _bp_buildpreview)
              (Variables|Default|SetBP_BuildPreview 0)
              (CallFunction|ResetBuildMode))
            (:else)))
        (:then_1
          (Default|CanBuildEvent _bp_buildercontroller true))))))

(event Input|EnhancedActionEvents|EnhancedInputActionIA_Build
  (params (ActionValue :type Boolean) (ElapsedSeconds :type Float%20%28double-precision%29) (TriggeredSeconds :type Float%20%28double-precision%29) (InputAction :type Input%20Action%20Object%20Reference :default "/Game/Inputs/Building/IA_Build.IA_Build"))
  ;[1 1 1] Input Preview
)

(event Input|EnhancedActionEvents|EnhancedInputActionIA_PlaceBuild
  (params (ActionValue :type Boolean) (ElapsedSeconds :type Float%20%28double-precision%29) (TriggeredSeconds :type Float%20%28double-precision%29) (InputAction :type Input%20Action%20Object%20Reference :default "/Game/Inputs/Building/IA_PlaceBuild.IA_PlaceBuild"))
  ;[1 1 1] Input Build
  (:Started
    (if (Variables|Default|GetinBuildMode)
      (if (Variables|/Game/Blueprints/Builder/BP_BuilderController.BP_BuilderController_C|GetcanBuild (Variables|Default|GetBP_BuilderController))
        (Game|SpawnActorfromClass (.Blueprint (Utilities|Struct|BreakS_BuildParts (Utilities|Array|Get(acopy) (Variables|Default|GetDT_Buildables) (Variables|Default|GetbuildableIndex)))) (Variables|Default|GetBuild%20Preview%20Transform) "AlwaysSpawn" "MultiplyWithRoot" 0 0)
        (CallFunction|StopBuildMode)))))

(event Input|EnhancedActionEvents|EnhancedInputActionIA_RotateBuild
  (params (ActionValue :type Boolean) (ElapsedSeconds :type Float%20%28double-precision%29) (TriggeredSeconds :type Float%20%28double-precision%29) (InputAction :type Input%20Action%20Object%20Reference :default "/Game/Inputs/Building/IA_RotateBuild.IA_RotateBuild")))

(event Input|EnhancedActionEvents|EnhancedInputActionIA_Destroy
  (params (ActionValue :type Boolean) (ElapsedSeconds :type Float%20%28double-precision%29) (TriggeredSeconds :type Float%20%28double-precision%29) (InputAction :type Input%20Action%20Object%20Reference :default "/Game/Inputs/IA_Destroy.IA_Destroy"))
  ;[1 1 1] Destroy building
  (:Started
    (bind (_outhit _returnvalue) (Collision|LineTraceByChannel (Variables|Default|GetTraceStart) (Variables|Default|GetTraceEnd) "TraceTypeQuery1" false 0 "None"))
    (if _returnvalue
      (if (Actor|ActorHasTag (.HitActor (Collision|BreakHitResult _outhit)) "Buildable")
        (Actor|DestroyActor (.HitActor (Collision|BreakHitResult _outhit)))))))

(event EventBeginPlay
  (Utilities|FlowControl|Sequence
    (:then_0
      ;[1 1 1] Get Camera
      (bind _asbp_player (Utilities|Casting|CastToBP_Player (Components|GetOwner)))
      (Variables|Default|SetPlayer%20BP _asbp_player)
      (Variables|Default|SetCamera (Variables|/Game/Blueprints/Player/BP_Player.BP_Player_C|GetCamera _asbp_player)))
    (:then_1
      ;[1 1 1] Get Data Table
      (bind _outrownames (DataTable|GetDataTableRowNames "/Game/Blueprints/Builder/DT_BuildParts.DT_BuildParts"))
      (for _array_element _outrownames
        (bind _returnvalue (Utilities|GetDataTableRow "/Game/Blueprints/Builder/DT_BuildParts.DT_BuildParts" _array_element)
          (:then
            (Utilities|Array|Add (Variables|Default|GetDT_Buildables) _returnvalue)))))
    (:then_2
      ;[1 1 1] Get builder controller
      (bind _outactors (Actor|GetAllActorsOfClass "/Game/Blueprints/Builder/BP_BuilderController.BP_BuilderController_C"))
      (if (> (Utilities|Array|Length _outactors) 0)
        (Variables|Default|SetBP_BuilderController (Utilities|Array|Get(acopy) _outactors))))))

(event EventTick
  (params (DeltaSeconds :type Float%20%28single-precision%29))
  (bind _camera (Variables|Default|GetCamera))
  (bind _returnvalue (Transformation|GetWorldTransform _camera))
  (Utilities|FlowControl|Sequence
    (:then_0
      ;[1 1 1] Set Trace Vector
      (Variables|Default|SetTraceStart (.location _returnvalue))
      (Variables|Default|SetTraceEnd (+ (.location _returnvalue) (* (Math|Vector|GetForwardVector (.rotation _returnvalue)) 7e+02))))
    (:then_1
      ;[1 1 1] Play Preview Loop
      (if (Variables|Default|GetinBuildMode)
        (CallFunction|PreviewLoop)))))

(event Input|MouseEvents|MouseWheelDown
  (params (Key :type Key%20Structure :default "None"))
  ;[1 1 1] Input Rotate Build Preview
  (:Pressed
    (if (Variables|Default|GetinBuildMode)
      (Variables|Default|SetBuildPreviewRotation (Math|Rotator|CombineRotators (.rotation (Variables|Default|GetBuild%20Preview%20Transform)) "0.000000,-45.000000,0.000000")))))

(event Input|MouseEvents|MouseWheelUp
  (params (Key :type Key%20Structure :default "None"))
  ;[1 1 1] Input Rotate Build Preview
  (:Pressed
    (if (Variables|Default|GetinBuildMode)
      (Variables|Default|SetBuildPreviewRotation (Math|Rotator|CombineRotators (.rotation (Variables|Default|GetBuild%20Preview%20Transform)) "0.000000,45.000000,0.000000")))))