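; Player build component that previews, places and destroys buildables defined in DT_BuildParts.
; While build mode is on, Tick traces from the camera and moves a once-spawned preview to the hit point at zero height.
; Mouse wheel rotates it in fixed steps; placing spawns the real Blueprint, clears the held item and exits the mode.
; O and L keys switch between a box in hand and its ground preview, while destroy removes traced "Buildable"-tagged actors.
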(event Custom|Preview%20Loop
  ;[1 1 1] Mesh Trace
  (bind (_outhit _returnvalue) (Collision|LineTraceByChannel (Variables|Default|GetTraceStart) (Variables|Default|GetTraceEnd) "TraceTypeQuery1" false 0 "None"))
  (if _returnvalue
    (Utilities|FlowControl|Sequence
      (:then_0
        ;[1 1 1] Create Build Preview Once
        (Utilities|FlowControl|DoOnce false
          (:Completed
            (bind _returnvalue_2 (Game|SpawnActorfromClass (.BluePrintPreview (Utilities|Struct|BreakS_BuildParts (Utilities|Array|Get(acopy) (Variables|Default|GetDT_Buildables) (Variables|Default|GetbuildableIndex)))) (Variables|Default|GetBuild%20Preview%20Transform) "AlwaysSpawn" "MultiplyWithRoot" 0 0))
            (Variables|Default|SetBP_BuildPreview _returnvalue_2))))
      (:then_1
        ;[1 1 1] Set the Position of the Preview
        (bind _output_get (Variables|Default|SetBuild%20Preview%20Transform (Math|Transform|MakeTransform (Math|Vector|MakeVector (.X (Math|Vector|BreakVector (.Location (Collision|BreakHitResult _outhit)))) (.Y (Math|Vector|BreakVector (.Location (Collision|BreakHitResult _outhit)))) 0.0) (Variables|Default|GetBuildPreviewRotation) "1.000000,1.000000,1.000000")))
        (Transformation|SetActorTransform (Variables|Default|GetBP_BuildPreview) _output_get)))))

(event Custom|Reset%20Build%20Mode
  (Utilities|FlowControl|Sequence
    (:then_0
      ;[1 1 1] Reset Box in Hand
      (Utilities|IsValid (Variables|Default|GetBP_BoxInHand)
        (:Is%20Valid
          (Actor|DestroyActor (Variables|Default|GetBP_BoxInHand)) ; Destroy box in hand
          (Variables|Default|SetBP_BoxInHand 0))))
    (:then_1
      ;[1 1 1] Create Build Preview Once
      (Utilities|FlowControl|DoOnce false) ; enters at Reset
    )))

(event Custom|Stop%20Build%20Mode
  (bind _bp_buildercontroller (Variables|Default|GetBP_BuilderController))
  ;[1 1 1] Input Preview
  (bind _output_get (Variables|Default|SetinBuildMode false)) ; not isnt in build mode
  (Utilities|FlowControl|Sequence
    (:then_0
      (Default|IsinBuildMode _bp_buildercontroller _output_get)
      (bind _bp_buildpreview (Variables|Default|GetBP_BuildPreview)
        (:then
          (Actor|DestroyActor _bp_buildpreview)
          (Variables|Default|SetBP_BuildPreview 0)
          (CallFunction|ResetBuildMode))
        (:else)))
    (:then_1
      (Default|CanBuildEvent _bp_buildercontroller true))))

(event Custom|Preview
  (bind _bp_buildercontroller (Variables|Default|GetBP_BuilderController))
  ;[1 1 1] Input Preview
  (if (not (Variables|Default|GetinBuildMode))
    (bind _output_get (Variables|Default|SetinBuildMode true)) ; now its in build mode
    (Default|IsinBuildMode (Variables|Default|GetBP_BuilderController) _output_get)
    (else
      (bind _output_get_2 (Variables|Default|SetinBuildMode false)) ; not isnt in build mode
      (Utilities|FlowControl|Sequence
        (:then_0
          (Default|IsinBuildMode _bp_buildercontroller _output_get_2)
          (bind _bp_buildpreview (Variables|Default|GetBP_BuildPreview)
            (:then
              (Actor|DestroyActor _bp_buildpreview)
              (Variables|Default|SetBP_BuildPreview 0)
              (CallFunction|ResetBuildMode))
            (:else)))
        (:then_1
          (Default|CanBuildEvent _bp_buildercontroller true))))))

(event Custom|MyTick)

(event Input|EnhancedActionEvents|EnhancedInputActionIA_PlaceBuild
  (params (ActionValue :type Boolean) (ElapsedSeconds :type Float%20%28double-precision%29) (TriggeredSeconds :type Float%20%28double-precision%29) (InputAction :type Input%20Action%20Object%20Reference :default "/Game/Inputs/Building/IA_PlaceBuild.IA_PlaceBuild"))
  ;[1 1 1] Input Build
  (:Started
    (if (Variables|Default|GetinBuildMode)
      (Game|SpawnActorfromClass (.Blueprint (Utilities|Struct|BreakS_BuildParts (Utilities|Array|Get(acopy) (Variables|Default|GetDT_Buildables) (Variables|Default|GetbuildableIndex)))) (Variables|Default|GetBuild%20Preview%20Transform) "AlwaysSpawn" "MultiplyWithRoot" 0 0)
      (Default|RemoveItemonHand (Variables|Default|GetPlayer%20BP))
      (CallFunction|StopBuildMode))))

(event Input|EnhancedActionEvents|EnhancedInputActionIA_Destroy
  (params (ActionValue :type Boolean) (ElapsedSeconds :type Float%20%28double-precision%29) (TriggeredSeconds :type Float%20%28double-precision%29) (InputAction :type Input%20Action%20Object%20Reference :default "/Game/Inputs/Building/IA_Destroy.IA_Destroy"))
  ;[1 1 1] Destroy building
  (:Started
    (bind (_outhit _returnvalue) (Collision|LineTraceByChannel (Variables|Default|GetTraceStart) (Variables|Default|GetTraceEnd) "TraceTypeQuery1" false 0 "None"))
    (if _returnvalue
      (if (Actor|ActorHasTag (.HitActor (Collision|BreakHitResult _outhit)) "Buildable")
        (Actor|DestroyActor (.HitActor (Collision|BreakHitResult _outhit)))))))

(event EventTick
  (params (DeltaSeconds :type Float%20%28single-precision%29))
  (bind _camera (Variables|Default|GetCamera))
  (bind _returnvalue (Transformation|GetWorldTransform _camera))
  (Development|PrintString "Hello")
  (Utilities|FlowControl|Sequence
    (:then_1
      ;[1 1 1] Play Preview Loop
      (if (Variables|Default|GetinBuildMode)
        ;[1 1 1] Set Trace Vector
        (Variables|Default|SetTraceStart (.location _returnvalue))
        (Variables|Default|SetTraceEnd (+ (.location _returnvalue) (* (Math|Vector|GetForwardVector (.rotation _returnvalue)) 7e+02)))
        (CallFunction|PreviewLoop)))))

(event EventBeginPlay
  (Utilities|FlowControl|Sequence
    (:then_0
      ;[1 1 1] Get Camera
      (bind _asbp_player (Utilities|Casting|CastToBP_Player (Components|GetOwner)))
      (Variables|Default|SetPlayer%20BP _asbp_player)
      (Variables|Default|SetCamera (Variables|/Game/Blueprints/Player/BP_Player.BP_Player_C|GetCamera _asbp_player)))
    (:then_1
      ;[1 1 1] Get Data Table
      (bind _outrownames (DataTable|GetDataTableRowNames "/Game/Blueprints/Builder/BuilderStuff/DT_BuildParts.DT_BuildParts"))
      (for _array_element _outrownames
        (bind _returnvalue (Utilities|GetDataTableRow "/Game/Blueprints/Builder/BuilderStuff/DT_BuildParts.DT_BuildParts" _array_element)
          (:then
            (Utilities|Array|Add (Variables|Default|GetDT_Buildables) _returnvalue)))))
    (:then_2
      ;[1 1 1] Get builder controller
      (bind _outactors (Actor|GetAllActorsOfClass "/Game/Blueprints/Builder/BuilderStuff/BP_BuilderController.BP_BuilderController_C"))
      (if (> (Utilities|Array|Length _outactors) 0)
        (Variables|Default|SetBP_BuilderController (Utilities|Array|Get(acopy) _outactors))))
    (:then_3
      (Utilities|Time|SetTimerbyEvent (delegate Custom|MyTick) 0.1 true))))

(event Input|MouseEvents|MouseWheelDown
  (params (Key :type Key%20Structure :default "None"))
  ;[1 1 1] Input Rotate Build Preview
  (:Pressed
    (if (Variables|Default|GetinBuildMode)
      (Variables|Default|SetBuildPreviewRotation (Math|Rotator|CombineRotators (.rotation (Variables|Default|GetBuild%20Preview%20Transform)) "0.000000,-45.000000,0.000000")))))

(event Input|MouseEvents|MouseWheelUp
  (params (Key :type Key%20Structure :default "None"))
  ;[1 1 1] Input Rotate Build Preview
  (:Pressed
    (if (Variables|Default|GetinBuildMode)
      (Variables|Default|SetBuildPreviewRotation (Math|Rotator|CombineRotators (.rotation (Variables|Default|GetBuild%20Preview%20Transform)) "0.000000,45.000000,0.000000")))))

(event Input|KeyboardEvents|L
  (params (Key :type Key%20Structure :default "None"))
  ;[1 1 1] Build Box in ground
  (:Pressed
    (Variables|Default|SetbuildableIndex (Variables|Default|GetbuildBoxInHandIndex))
    (Actor|DestroyActor (Variables|Default|GetBP_BuildPreview))
    (Variables|Default|SetBP_BuildPreview 0)
    (CallFunction|ResetBuildMode)))

(event Input|KeyboardEvents|O
  (params (Key :type Key%20Structure :default "None"))
  (bind _player_bp (Variables|Default|GetPlayer%20BP))
  (bind _boxinhandpoint (Variables|/Game/Blueprints/Player/BP_Player.BP_Player_C|GetBoxInHandPoint _player_bp))
  ;[1 1 1] Take Box back to hand, and place item
  (:Pressed
    (Variables|Default|SetbuildableIndex (Variables|Default|GetbuildItemIndex)) ; Go back to item Index
    (Actor|DestroyActor (Variables|Default|GetBP_BuildPreview)) ; Destroy box preview
    (Variables|Default|SetBP_BuildPreview 0)
    (bind _returnvalue (Game|SpawnActorfromClass "/Game/Blueprints/BoxInHand/BP_BoxInHand.BP_BoxInHand_C" (Transformation|GetWorldTransform _boxinhandpoint) "AlwaysSpawn" "MultiplyWithRoot" 0 0)) ; Spawn Box again
    (Transformation|AttachComponentToComponent _returnvalue _boxinhandpoint "None" "SnapToTarget" "SnapToTarget" "KeepRelative" true)
    (Variables|Default|SetBP_BoxInHand _returnvalue)
    ;[1 1 1] Create Build Preview Once
    (Utilities|FlowControl|DoOnce false) ; enters at Reset
  ))

(event Input|KeyboardEvents|O
  (params (Key :type Key%20Structure :default "None"))
  ;[1 1 1] Faze botao para apertar e lancar a caixa para longe
)