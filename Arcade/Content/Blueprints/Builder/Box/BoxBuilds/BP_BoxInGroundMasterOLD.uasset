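; BP_BoxInGroundMasterOLD is an interactable box on the ground that the player can pick up, apparently an older master version.
; Interact stores the player, calls AddItemOnHand on it, then spawns a BP_BoxInHand at the player's BoxInHandPoint.
; The new box receives the player reference, runs Setup and snaps onto that point, and the ground actor destroys itself.
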(event EventInteract
  (params (bpPlayer :type BP%20Player%20Object%20Reference))
  (bind _output_get (Variables|Default|SetBP_Player bpPlayer))
  (Default|AddItemonHand _output_get)
  (bind _returnvalue (Game|SpawnActorfromClass "/Game/Blueprints/BoxInHand/BP_BoxInHand.BP_BoxInHand_C" (Transformation|GetWorldTransform (Variables|/Game/Blueprints/Player/BP_Player.BP_Player_C|GetBoxInHandPoint (Variables|Default|GetBP_Player))) "AlwaysSpawn" "MultiplyWithRoot" 0 0)) ; Spawn Box
  (Variables|/Game/Blueprints/BoxInHand/BP_BoxInHand.BP_BoxInHand_C|SetBP_Player _returnvalue (Variables|Default|GetBP_Player)) ; Pass ref to box
  (Default|Setup _returnvalue)
  (Transformation|AttachComponentToComponent _returnvalue (Variables|/Game/Blueprints/Player/BP_Player.BP_Player_C|GetBoxInHandPoint (Variables|Default|GetBP_Player)) "None" "SnapToTarget" "SnapToTarget" "KeepRelative" true)
  (Actor|DestroyActor) ; Destroy this obj
)

(fn ConstructionScript)