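; BP_BuildBoxMaster is the base Blueprint for a world box representing a buildable item that the player can pick up.
; A short delay after BeginPlay gates pickup.
; Interact marks the player as holding an item, spawns the in-hand box class chosen from the buildables data by index, attaches it to the player's hand point with that index, then destroys the world box.
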(event Collision|EventActorBeginOverlap
  (params (OtherActor :type Actor%20Object%20Reference))
  (|CallParentFunction OtherActor) ; This node is disabled and will not be called.\nDrag off pins to build functionality.
)

(event EventTick
  (params (DeltaSeconds :type Float%20%28single-precision%29))
  (|CallParentFunction DeltaSeconds) ; This node is disabled and will not be called.\nDrag off pins to build functionality.
)

(event EventBeginPlay
  (|CallParentFunction)
  (Utilities|FlowControl|Delay 0.2)
  (Variables|Default|SetdelayToPickup true))

(event EventInteract
  (params (bpPlayer :type BP%20Player%20Object%20Reference))
  (if (Variables|Default|GetdelayToPickup)
    (bind _output_get (Variables|Default|SetBP_Player bpPlayer))
    (Default|AddItemonHand _output_get)
    (bind _returnvalue (Game|SpawnActorfromClass (Utilities|Array|Get(acopy) (Variables|Default|GetBP_BoxInHand) (.ThisItemBoxIndex (Utilities|Struct|BreakS_BuildParts (Utilities|Array|Get(acopy) (Variables|Default|GetDT_Buildables) (Variables|Default|GetthisBuildableIndex))))) (Transformation|GetWorldTransform (Variables|/Game/Blueprints/Player/BP_Player.BP_Player_C|GetBoxInHandPoint (Variables|Default|GetBP_Player))) "AlwaysSpawn" "MultiplyWithRoot" 0 0)) ; Spawn Box in Hand
    (Variables|/Game/Blueprints/BoxInHand/BP_BoxInHandMaster.BP_BoxInHandMaster_C|SetBP_Player _returnvalue (Variables|Default|GetBP_Player)) ; Pass ref to box
    (Default|Setup _returnvalue (Variables|Default|GetthisBuildableIndex))
    (Transformation|AttachComponentToComponent _returnvalue (Variables|/Game/Blueprints/Player/BP_Player.BP_Player_C|GetBoxInHandPoint (Variables|Default|GetBP_Player)) "None" "SnapToTarget" "SnapToTarget" "KeepRelative" true)
    (Actor|DestroyActor) ; Destroy this obj
  ))

(fn ConstructionScript
  (|CallParentFunction))