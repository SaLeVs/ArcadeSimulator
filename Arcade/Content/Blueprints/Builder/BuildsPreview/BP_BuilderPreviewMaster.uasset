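; Master builder preview actor that signals whether a building can be placed at its current spot.
; On BeginPlay it caches the first BP_BuilderController in the level.
; BuildCollision overlap events check the OverlappedComponent for the "BuildCollision" tag, report buildability to the controller and swap BuildMesh between valid and blocked preview materials.
; A tagged end overlap restores the buildable state without checking for remaining overlaps.
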(event OnComponentBeginOverlap(BuildCollision)
  (params (OverlappedComponent :type Primitive%20Component%20Object%20Reference) (OtherActor :type Actor%20Object%20Reference) (OtherComp :type Primitive%20Component%20Object%20Reference) (OtherBodyIndex :type Integer) (bFromSweep :type Boolean) (SweepResult :type Hit%20Result%20Structure%20%28by%20ref%29))
  (bind _bp_buildercontroller (Variables|Default|GetBP_BuilderController))
  (bind _buildmesh (Variables|Default|GetBuildMesh))
  (if (Components|ComponentHasTag OverlappedComponent "BuildCollision")
    (Default|CanBuildEvent _bp_buildercontroller false) ; cant build
    (Rendering|Material|SetMaterial _buildmesh 0 "/Game/Materials/M_CantBuildingPreview.M_CantBuildingPreview")
    (else
      (Default|CanBuildEvent _bp_buildercontroller true) ; can build
      (Rendering|Material|SetMaterial _buildmesh 0 "/Game/Materials/M_BuildingPreview.M_BuildingPreview"))))

(event OnComponentEndOverlap(BuildCollision)
  (params (OverlappedComponent :type Primitive%20Component%20Object%20Reference) (OtherActor :type Actor%20Object%20Reference) (OtherComp :type Primitive%20Component%20Object%20Reference) (OtherBodyIndex :type Integer))
  (if (Components|ComponentHasTag OverlappedComponent "BuildCollision")
    (Default|CanBuildEvent (Variables|Default|GetBP_BuilderController) true) ; can build
    (Rendering|Material|SetMaterial (Variables|Default|GetBuildMesh) 0 "/Game/Materials/M_BuildingPreview.M_BuildingPreview")))

(event EventBeginPlay
  ;[1 1 1] Get Builder Controller
  (bind _outactors (Actor|GetAllActorsOfClass "/Game/Blueprints/Builder/BP_BuilderController.BP_BuilderController_C"))
  (if (> (Utilities|Array|Length _outactors) 0)
    (Variables|Default|SetBP_BuilderController (Utilities|Array|Get(acopy) _outactors))))

(fn ConstructionScript)