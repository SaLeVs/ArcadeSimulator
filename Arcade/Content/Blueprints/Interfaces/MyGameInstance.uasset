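; Game instance that owns the save system and the player's money balance.
; On Init it loads or creates a BP_SaveLoadGame object, then caches the BP_ExpandController after a short delay.
; SaveAll rebuilds the buildables list from all BP_BuildablesMaster actors and saves player data, with sync or async slot writes.
; GainMoney and SpendMoney adjust the balance and broadcast changes, with SpendMoney refusing spends that would not leave it above zero.
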(event EventInit
  (Utilities|FlowControl|Sequence
    (:then_0
      (CallFunction|LoadGameData false))
    (:then_1
      (Utilities|FlowControl|Delay 0.2)
      (bind _returnvalue (Actor|GetActorOfClass "/Game/Blueprints/ExpandArcade/BP_ExpandController.BP_ExpandController_C"))
      (Variables|Default|SetexpandController _returnvalue))))

(event EventSaveGameData
  (params (Async :type Boolean))
  ;[1 1 1] Save Game
  (if Async
    (|AsyncSaveGametoSlot (Variables|Default|GetSavedData) (Variables|Default|GetSaveSlotName))
    (else
      (SaveGame|SaveGametoSlot (Variables|Default|GetSavedData) (Variables|Default|GetSaveSlotName)))))

(event EventLoadGameData
  (params (Async :type Boolean))
  (bind _saveslotname (Variables|Default|GetSaveSlotName))
  ;[1 1 1] Load Game
  (bind _returnvalue (SaveGame|DoesSaveGameExist (Variables|Default|GetSaveSlotName)))
  (if _returnvalue
    (if Async
      (bind _savegame (|AsyncLoadGamefromSlot _saveslotname)
        (:Completed
          (bind _asbp_save_load_game (Utilities|Casting|CastToBP_SaveLoadGame _savegame))
          (Variables|Default|SetSavedData _asbp_save_load_game)
          (Default|CallOnGameLoaded)))
      (else
        (bind _returnvalue_2 (SaveGame|LoadGamefromSlot _saveslotname))
        (bind _asbp_save_load_game_2 (Utilities|Casting|CastToBP_SaveLoadGame _returnvalue_2))
        (Variables|Default|SetSavedData _asbp_save_load_game_2)))
    (else
      (bind _returnvalue_3 (SaveGame|CreateSaveGameObject "/Game/Blueprints/SaveLoad/BP_SaveLoadGame.BP_SaveLoadGame_C"))
      (Variables|Default|SetSavedData _returnvalue_3))))

(event EventSavePlayer
  (params (PlayerSave :type S%20Player%20Save%20Structure) (Async :type Boolean))
  ;[1 1 1] Custom Save Functions
  (Variables|/Game/Blueprints/SaveLoad/BP_SaveLoadGame.BP_SaveLoadGame_C|SetPlayerSave (Variables|Default|GetSavedData) PlayerSave)
  (CallFunction|SaveGameData Async))

(event EventSaveBuildables
  (params (Async :type Boolean))
  ;[1 1 1] Custom Save Functions
  (Utilities|Array|Clear (Variables|/Game/Blueprints/SaveLoad/BP_SaveLoadGame.BP_SaveLoadGame_C|GetBuildablesSave (Variables|Default|GetSavedData))) ; Clear and readd all objs
  (bind _outactors (Actor|GetAllActorsOfClass "/Game/Blueprints/Builder/BP_BuildablesMaster.BP_BuildablesMaster_C"))
  (for _array_element _outactors
    (bind _asbp_buildables_master (Utilities|Casting|CastToBP_BuildablesMaster _array_element))
    (bind _buildablesave (Default|GetBuildableSaveData _asbp_buildables_master))
    (Utilities|Array|AddUnique (Variables|/Game/Blueprints/SaveLoad/BP_SaveLoadGame.BP_SaveLoadGame_C|GetBuildablesSave (Variables|Default|GetSavedData)) _buildablesave))
  (CallFunction|SaveGameData false))

(event EventSaveAll
  (params (Async :type Boolean))
  (Utilities|FlowControl|Sequence
    (:then_0
      (CallFunction|SaveBuildables false))
    (:then_1
      (bind _bpplayer (Variables|Default|GetbpPlayer) ; Save player pos
        (:then
          (bind _playersave (Default|GetPlayerSaveData _bpplayer))
          (Class|BPISaveGame|SavePlayer(Message) (Game|GetGameInstance) _playersave Async))
        (:else)))
    (:then_2
      (Development|PrintString "Saved All"))))

(event EventGainMoney
  (params (moneyToGain :type Float%20%28double-precision%29))
  (Variables|Default|SetplayerMoney (+ (Variables|Default|GetplayerMoney) moneyToGain))
  (Default|CallOnMoneyChanged))

(fn GetGameData
  (return (Variables|Default|GetSavedData)))

(fn SpendMoney
  (params (moneyToSpend :type Float%20%28double-precision%29))
  (if (> (- (Variables|Default|GetplayerMoney) moneyToSpend) 0.0) ; True = can spend\nFalse = can't spend
    (Variables|Default|SetplayerMoney (- (Variables|Default|GetplayerMoney) moneyToSpend)) ; Decrease
    (Default|CallOnMoneyChanged)
    (return true)
    (else
      (return false))))