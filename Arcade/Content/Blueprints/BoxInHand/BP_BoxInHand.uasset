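; BP_BoxInHand is the Blueprint for a box in the player's hand that links a buildable item to the player's build system.
; Its Setup event registers the box on the player's BPCBuildSystem component and passes the item index as both the build item and buildable index.
; It also hands over its own box index, then starts the build preview.
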(event Custom|Setup
  (params (itemIndex :type Integer))
  (Variables|Default|SetBPC_BuildSystem (Variables|/Game/Blueprints/Player/BP_Player.BP_Player_C|GetBPC_BuildSystem (Variables|Default|GetBP_Player))) ; Ref to player buildSystem
  (Variables|/Game/Blueprints/Builder/BuilderStuff/BPC_BuildSystem.BPC_BuildSystem_C|SetBP_BoxInHand (Variables|Default|GetBPC_BuildSystem) self) ; Ref this to player
  (Variables|/Game/Blueprints/Builder/BuilderStuff/BPC_BuildSystem.BPC_BuildSystem_C|SetbuildItemIndex (Variables|Default|GetBPC_BuildSystem) itemIndex) ; Set the ITEM build index
  (Variables|/Game/Blueprints/Builder/BuilderStuff/BPC_BuildSystem.BPC_BuildSystem_C|SetbuildableIndex (Variables|Default|GetBPC_BuildSystem) itemIndex) ; Set the build index
  (Variables|/Game/Blueprints/Builder/BuilderStuff/BPC_BuildSystem.BPC_BuildSystem_C|SetbuildBoxInHandIndex (Variables|Default|GetBPC_BuildSystem) (Variables|Default|GetthisBoxInHandIndex)) ; Set this box index to build system
  (Default|Preview (Variables|Default|GetBPC_BuildSystem)) ; Start build preview in player
)

(fn ConstructionScript)