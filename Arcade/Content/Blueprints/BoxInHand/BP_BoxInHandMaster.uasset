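; BP_BoxInHandMaster is the master Blueprint for a box held in the player's hand that drives build placement.
; On BeginPlay it caches every DT_BuildParts row in DTBuildables.
; Setup registers the box with the player's BPCBuildSystem, passes ItemIndex as both item and buildable index, copies that row's box index, then starts the build preview.
; ItemIndex indexes the cached array directly, so it depends on the table's row order.
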(event Custom|Setup
  (params (itemIndex :type Integer))
  (Variables|Default|SetBPC_BuildSystem (Variables|/Game/Blueprints/Player/BP_Player.BP_Player_C|GetBPC_BuildSystem (Variables|Default|GetBP_Player))) ; Ref to player buildSystem
  (Variables|/Game/Blueprints/Builder/BuilderStuff/BPC_BuildSystem.BPC_BuildSystem_C|SetBP_BoxInHand (Variables|Default|GetBPC_BuildSystem) self) ; Ref this to player
  (Variables|/Game/Blueprints/Builder/BuilderStuff/BPC_BuildSystem.BPC_BuildSystem_C|SetbuildItemIndex (Variables|Default|GetBPC_BuildSystem) itemIndex) ; Set the ITEM build index
  (Variables|/Game/Blueprints/Builder/BuilderStuff/BPC_BuildSystem.BPC_BuildSystem_C|SetbuildableIndex (Variables|Default|GetBPC_BuildSystem) itemIndex) ; Set the build index
  (Variables|/Game/Blueprints/Builder/BuilderStuff/BPC_BuildSystem.BPC_BuildSystem_C|SetbuildBoxInHandIndex (Variables|Default|GetBPC_BuildSystem) (.ThisItemBoxIndex (Utilities|Struct|BreakS_BuildParts (Utilities|Array|Get(acopy) (Variables|Default|GetDT_Buildables) itemIndex)))) ; Set this box index to build system
  (Default|Preview (Variables|Default|GetBPC_BuildSystem)) ; Start build preview in player
)

(event EventBeginPlay
  ;[1 1 1] Get Data Table
  (bind _outrownames (DataTable|GetDataTableRowNames "/Game/Blueprints/Builder/BuilderStuff/DT_BuildParts.DT_BuildParts"))
  (for _array_element _outrownames
    (bind _returnvalue (Utilities|GetDataTableRow "/Game/Blueprints/Builder/BuilderStuff/DT_BuildParts.DT_BuildParts" _array_element)
      (:then
        (Utilities|Array|Add (Variables|Default|GetDT_Buildables) _returnvalue)))))

(fn ConstructionScript)