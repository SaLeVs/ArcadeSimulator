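; BP_Mop is a mop item Blueprint with a use and disuse action that lowers and raises the actor.
; MopUse runs a debug-drawn Visibility line trace straight down, then moves the actor down without sweep; the trace result is not used.
; MopDisuse moves it back up by the same distance.
; The construction script and NewFunction are empty.
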(event EventMopDisuse
  (Transformation|SetActorLocation (- (Transformation|GetActorLocation) "0.000000,0.000000,-70.000000") false false))

(event EventMopUse
  (Collision|LineTraceByChannel (Transformation|GetActorLocation) (- (Transformation|GetActorLocation) "0.000000,0.000000,500.000000") "TraceTypeQuery1" false 0 "ForDuration")
  (Transformation|SetActorLocation (- (Transformation|GetActorLocation) "0.000000,0.000000,70.000000") false false))

(fn ConstructionScript)

(fn NewFunction
  (return 0))