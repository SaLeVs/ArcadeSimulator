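; BP_Computer is an in-world computer the player uses through a widget component.
; Entering its Box trigger focuses the widget in Game and UI input mode, shows the mouse cursor and blends the view to the computer over one second.
; Leaving restores game-only input, hides the cursor and blends back to the player character.
; The begin overlap only checks actor validity, so any actor can trigger it for player 0.
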(event OnComponentBeginOverlap(Box)
  (params (OverlappedComponent :type Primitive%20Component%20Object%20Reference) (OtherActor :type Actor%20Object%20Reference) (OtherComp :type Primitive%20Component%20Object%20Reference) (OtherBodyIndex :type Integer) (bFromSweep :type Boolean) (SweepResult :type Hit%20Result%20Structure%20%28by%20ref%29))
  (Utilities|IsValid OtherActor
    (:Is%20Valid
      (bind _output_get (Variables|Default|SetPlayerController (Game|GetPlayerController 0)))
      (Input|SetInputModeGameandUI _output_get (UserInterface|GetUserWidgetObject (Variables|Default|GetWidget)) "DoNotLock" true false)
      (Variables|/Script/Engine.PlayerController|SetbShowMouseCursor (Variables|Default|GetPlayerController) true)
      (Game|Player|SetViewTargetwithBlend (Variables|Default|GetPlayerController) self 1.0 "VTBlend_Linear" 0.0 false))))

(event OnComponentEndOverlap(Box)
  (params (OverlappedComponent :type Primitive%20Component%20Object%20Reference) (OtherActor :type Actor%20Object%20Reference) (OtherComp :type Primitive%20Component%20Object%20Reference) (OtherBodyIndex :type Integer))
  (Utilities|IsValid (Game|GetPlayerController 0)
    (:Is%20Valid
      (Input|SetInputModeGameOnly (Variables|Default|GetPlayerController) false)
      (Variables|/Script/Engine.PlayerController|SetbShowMouseCursor (Variables|Default|GetPlayerController) false)
      (Game|Player|SetViewTargetwithBlend (Variables|Default|GetPlayerController) (Game|GetPlayerCharacter 0) 1.0 "VTBlend_Linear" 0.0 false))))

(fn ConstructionScript)