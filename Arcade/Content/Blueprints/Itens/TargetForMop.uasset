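; Dirt spot actor that the player cleans by holding a wet mop over it.
; When BP_Mop overlaps the Box and the game instance reports a bucket-dipped mop with water left, the Cube gets a dynamic material instance.
; Opacity fades in timed steps while overlap continues, checked through a flag cleared on end overlap.
; A completed fade destroys the actor and deducts water from the game instance's mop.
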(event OnComponentBeginOverlap(Box)
  (params (OverlappedComponent :type Primitive%20Component%20Object%20Reference) (OtherActor :type Actor%20Object%20Reference) (OtherComp :type Primitive%20Component%20Object%20Reference) (OtherBodyIndex :type Integer) (bFromSweep :type Boolean) (SweepResult :type Hit%20Result%20Structure%20%28by%20ref%29))
  (bind _asmy_game_instance (Utilities|Casting|CastToMyGameInstance (Game|GetGameInstance)))
  (if (and (Variables|/Game/Blueprints/Interfaces/MyGameInstance.MyGameInstance_C|GetPlayerPassTheMopOnBucket? _asmy_game_instance) (> (Variables|/Game/Blueprints/Interfaces/MyGameInstance.MyGameInstance_C|GetWaterOnMop _asmy_game_instance) 0.0))
    (Utilities|Casting|CastToBP_Mop OtherActor)
    (Variables|Default|SetIsMopColiding? true)
    (bind _returnvalue (Rendering|Material|CreateDynamicMaterialInstance "/Game/Materials/WashMop/DirtMaterial.DirtMaterial" "Opacity" "None" :!class /Script/Engine.KismetMaterialLibrary))
    (bind _output_get (Variables|Default|SetMyDirtMaterial _returnvalue))
    (Rendering|Material|SetMaterial (Variables|Default|GetCube) 0 _output_get)
    (Rendering|Material|SetScalarParameterValue (Variables|Default|GetMyDirtMaterial) "Opacity" 0.8 :!class /Script/Engine.MaterialInstanceDynamic)
    (Utilities|FlowControl|Delay 1.0)
    (if (Variables|Default|GetIsMopColiding?)
      (Rendering|Material|SetScalarParameterValue (Variables|Default|GetMyDirtMaterial) "Opacity" 0.4 :!class /Script/Engine.MaterialInstanceDynamic)
      (Utilities|FlowControl|Delay 1.0)
      (if (Variables|Default|GetIsMopColiding?)
        (Rendering|Material|SetScalarParameterValue (Variables|Default|GetMyDirtMaterial) "Opacity" 0.0 :!class /Script/Engine.MaterialInstanceDynamic)
        (Actor|DestroyActor)
        (bind _output_get_2 (Variables|/Game/Blueprints/Interfaces/MyGameInstance.MyGameInstance_C|SetWaterOnMop _asmy_game_instance (- (Variables|/Game/Blueprints/Interfaces/MyGameInstance.MyGameInstance_C|GetWaterOnMop _asmy_game_instance) 0.5)))
        (Development|PrintString (Utilities|String|ToString(Float) _output_get_2))
        (else
          (Rendering|Material|SetScalarParameterValue (Variables|Default|GetMyDirtMaterial) "Opacity" 0.4 :!class /Script/Engine.MaterialInstanceDynamic)))
      (else
        (Rendering|Material|SetScalarParameterValue (Variables|Default|GetMyDirtMaterial) "Opacity" 0.8 :!class /Script/Engine.MaterialInstanceDynamic)))))

(event OnComponentEndOverlap(Box)
  (params (OverlappedComponent :type Primitive%20Component%20Object%20Reference) (OtherActor :type Actor%20Object%20Reference) (OtherComp :type Primitive%20Component%20Object%20Reference) (OtherBodyIndex :type Integer))
  (Variables|Default|SetIsMopColiding? false))

(fn ConstructionScript)