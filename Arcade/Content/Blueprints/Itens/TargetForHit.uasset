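; TargetForHit is an item actor that records hits on its configurable static mesh by painting them into a render target at the impact point.
; On BeginPlay it briefly applies an unwrap material and uses a scene capture to bake the mesh into a texture.
; DrawToRenderTarget feeds that texture, position and size to a brush material, drawing into a hit mask that drives the mesh materials' OpacityMask layer-blend parameter.
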(event EventBeginPlay
  (for _index (range 0 (- (Rendering|Material|GetNumMaterials (Variables|Default|GetStaticMesh)) 1))
    (bind _returnvalue (Rendering|Material|CreateDynamicMaterialInstance (Variables|Default|GetStaticMesh) _index (Variables|Default|GetSourceMaterial) "None" :!class /Script/Engine.PrimitiveComponent))
    (Utilities|Array|Add (Variables|Default|GetMaterial%20Instances) _returnvalue))
  (Utilities|FlowControl|Sequence
    (:then_0
      (bind _returnvalue_2 (Rendering|CreateRenderTarget2D 1024 1024 "RTF_RGBA16f"))
      (bind _output_get (Variables|Default|SetRT%20Unrwrap _returnvalue_2))
      (Variables|/Script/Engine.SceneCaptureComponent2D|SetTextureTarget (Variables|Default|GetSceneCaptureComponent2D) _output_get)
      (Rendering|SceneCapture|ShowOnlyActorComponents (Variables|Default|GetSceneCaptureComponent2D) self false))
    (:then_1
      (bind _returnvalue_3 (Rendering|CreateRenderTarget2D 1024 1024 "RTF_RGBA16f"))
      (Variables|Default|SetRT%20Hity _returnvalue_3)
      (for _array_element (Variables|Default|GetMaterial%20Instances)
        (Class|MaterialInstanceDynamic|SetTextureParameterValuebyInfo _array_element (Utilities|Struct|MakeMaterialParameterInfo "OpacityMask" "BlendParameter" 0) (Variables|Default|GetRT%20Hity)))
      (Rendering|ClearRenderTarget2D (Variables|Default|GetRT%20Hity)))
    (:then_2
      (Transformation|SetWorldRotation (Variables|Default|GetSceneCaptureComponent2D) "-90.000000,-90.000000,0.000000" false false)
      (for _index_2 (range 0 (- (Rendering|Material|GetNumMaterials (Variables|Default|GetStaticMesh)) 1))
        (Rendering|Material|SetMaterial (Variables|Default|GetStaticMesh) _index_2 "/Game/Materials/WashHit/M_Unwrap.M_Unwrap"))
      (Rendering|SceneCapture|CaptureScene (Variables|Default|GetSceneCaptureComponent2D) :!class /Script/Engine.SceneCaptureComponent2D)
      (for (_array_element_2 _array_index) (Variables|Default|GetMaterial%20Instances)
        (Rendering|Material|SetMaterial (Variables|Default|GetStaticMesh) _array_index _array_element_2))
      (bind _returnvalue_4 (Rendering|Material|CreateDynamicMaterialInstance "/Game/Materials/WashHit/M_Brush.M_Brush" "None" "None" :!class /Script/Engine.KismetMaterialLibrary))
      (bind _output_get_2 (Variables|Default|SetMI%20Brush _returnvalue_4))
      (Rendering|Material|SetTextureParameterValue _output_get_2 "Unwrapped" (Variables|Default|GetRT%20Unrwrap)))))

(fn ConstructionScript
  (Components|StaticMesh|SetStaticMesh (Variables|Default|GetStaticMesh) (Variables|Default|GetSourceMesh)))

(fn DrawtoRenderTarget
  (params (Impact%20Point :type Vector) (Brush%20Size :type Float%20%28double-precision%29))
  (Rendering|Material|SetScalarParameterValue (Variables|Default|GetMI%20Brush) "Size" Brush%20Size :!class /Script/Engine.MaterialInstanceDynamic)
  (Rendering|Material|SetVectorParameterValue (Variables|Default|GetMI%20Brush) "Position" (Math|Conversions|ToLinearColor(Vector) Impact%20Point) :!class /Script/Engine.MaterialInstanceDynamic)
  (Rendering|DrawMaterialtoRenderTarget (Variables|Default|GetRT%20Hity) (Variables|Default|GetMI%20Brush)))