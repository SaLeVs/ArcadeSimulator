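; Master pickup item that puts a box in the player's hands when touched.
; Its Box overlap accepts only components tagged Player on a BP_Player, and does nothing if that player already holds a box.
; Otherwise it flags the hands as full, spawns BP_BoxInHand at BoxInHandPoint, passes it the player reference and runs Setup.
; The new box is attached to that point and the pickup destroys itself.
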(event OnComponentBeginOverlap(Box)
  (params (OverlappedComponent :type Primitive%20Component%20Object%20Reference) (OtherActor :type Actor%20Object%20Reference) (OtherComp :type Primitive%20Component%20Object%20Reference) (OtherBodyIndex :type Integer) (bFromSweep :type Boolean) (SweepResult :type Hit%20Result%20Structure%20%28by%20ref%29))
  ;[1 1 1] Touched player, spawn a box in hand
  (if (Components|ComponentHasTag OtherComp "Player")
    (bind _asbp_player (Utilities|Casting|CastToBP_Player OtherActor))
    (bind _output_get (Variables|Default|SetBP_Player _asbp_player))
    (if (not (Variables|/Game/Blueprints/Player/BP_Player.BP_Player_C|GethaveBoxInHands _output_get)) ; If hands empty
      (Variables|/Game/Blueprints/Player/BP_Player.BP_Player_C|SethaveBoxInHands (Variables|Default|GetBP_Player) true) ; Now, have box in hands
      (bind _returnvalue (Game|SpawnActorfromClass "/Game/Blueprints/Itens/BP_BoxInHand.BP_BoxInHand_C" (Transformation|GetWorldTransform (Variables|/Game/Blueprints/Player/BP_Player.BP_Player_C|GetBoxInHandPoint (Variables|Default|GetBP_Player))) "AlwaysSpawn" "MultiplyWithRoot" 0 0)) ; Spawn Box
      (Variables|/Game/Blueprints/Itens/BP_BoxInHand.BP_BoxInHand_C|SetBP_Player _returnvalue (Variables|Default|GetBP_Player)) ; Pass ref to box
      (Default|Setup _returnvalue)
      (Transformation|AttachComponentToComponent _returnvalue (Variables|/Game/Blueprints/Player/BP_Player.BP_Player_C|GetBoxInHandPoint (Variables|Default|GetBP_Player)) "None" "SnapToTarget" "SnapToTarget" "KeepRelative" true)
      (Actor|DestroyActor) ; Destroy this obj
    )))

(fn ConstructionScript)