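; BP_TutorialClearItens is a one-time tutorial trigger that resets the build machines when the player passes through its Box.
; On a BP_Player overlap it destroys every BP_BuildMachineMaster actor, then spawns Arcade, Pinball and Claw machines at hardcoded transforms.
; After a short delay it calls SetDoorRotation on the tutorial door and sets PlayerPassed, which blocks later triggers.
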(event OnComponentBeginOverlap(Box)
  (params (OverlappedComponent :type Primitive%20Component%20Object%20Reference) (OtherActor :type Actor%20Object%20Reference) (OtherComp :type Primitive%20Component%20Object%20Reference) (OtherBodyIndex :type Integer) (bFromSweep :type Boolean) (SweepResult :type Hit%20Result%20Structure%20%28by%20ref%29))
  (if (not (Variables|Default|GetplayerPassed))
    (Utilities|Casting|CastToBP_Player OtherActor)
    (bind _outactors (Actor|GetAllActorsOfClass "/Game/Blueprints/Builder/Machines/MachineBuilds/BP_BuildMachineMaster.BP_BuildMachineMaster_C"))
    (Actor|DestroyActor _outactors)
    (Game|SpawnActorfromClass "/Game/Blueprints/Builder/Machines/MachineBuilds/Arcade/BP_BuildMachine_ArcadeV1.BP_BuildMachine_ArcadeV1_C" (Math|Transform|MakeTransform "-5595.000000,1315.000000,0.000000" "0.000000,-179.999999,0.000000" "1.000000,1.000000,1.000000") "AdjustIfPossibleButAlwaysSpawn" "MultiplyWithRoot" 0 0)
    (Game|SpawnActorfromClass "/Game/Blueprints/Builder/Machines/MachineBuilds/Pinball/BP_BuildMachine_PinballV1.BP_BuildMachine_PinballV1_C" (Math|Transform|MakeTransform "-5960.000000,970.000000,0.000000" "0.000000,-89.999999,0.000000" "1.000000,1.000000,1.000000") "AdjustIfPossibleButAlwaysSpawn" "MultiplyWithRoot" 0 0)
    (Game|SpawnActorfromClass "/Game/Blueprints/Builder/Machines/MachineBuilds/Claw/BP_BuildMachine_ClawV3.BP_BuildMachine_ClawV3_C" (Math|Transform|MakeTransform "-5590.000000,575.000000,0.000000" "0, 0, 0" "1.000000,1.000000,1.000000") "AdjustIfPossibleButAlwaysSpawn" "MultiplyWithRoot" 0 0)
    (Utilities|FlowControl|Delay 0.5)
    (Default|SetDoorRotation (Variables|Default|GetbpTutorialDoor))
    (Variables|Default|SetplayerPassed true)))

(fn ConstructionScript)