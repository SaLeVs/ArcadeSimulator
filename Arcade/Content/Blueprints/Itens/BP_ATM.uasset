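; BP_ATM is an ATM actor that switches the player into a cashier input mode.
; A collision volume tracks whether the player is in range, setting the flag on any overlap without an actor check.
; When UseMoney fires in range, it teleports the overlapping actor to PlayerPoint and swaps the Enhanced Input movement context for the cashier one.
; Pressing X, bound directly on the actor, restores movement and clears the range flag.
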(event OnComponentEndOverlap(Collision)
  (params (OverlappedComponent :type Primitive%20Component%20Object%20Reference) (OtherActor :type Actor%20Object%20Reference) (OtherComp :type Primitive%20Component%20Object%20Reference) (OtherBodyIndex :type Integer))
  (Variables|Default|SetIsPlayerOnRadius? false))

(event OnComponentBeginOverlap(Collision)
  (params (OverlappedComponent :type Primitive%20Component%20Object%20Reference) (OtherActor :type Actor%20Object%20Reference) (OtherComp :type Primitive%20Component%20Object%20Reference) (OtherBodyIndex :type Integer) (bFromSweep :type Boolean) (SweepResult :type Hit%20Result%20Structure%20%28by%20ref%29))
  (Variables|Default|SetIsPlayerOnRadius? true))

(event EventBeginPlay
  (Input|EnableInput (Game|GetPlayerController 0)))

(event EventUseMoney
  (bind _returnvalue (Game|GetPlayerController 0))
  (bind _returnvalue_2 (PlayerController|LocalPlayerSubsystems|GetEnhancedInputLocalPlayerSubsystem _returnvalue))
  (if (Variables|Default|GetIsPlayerOnRadius?)
    (Transformation|Teleport (stale OnComponentBeginOverlap(Collision) OtherActor) (Transformation|GetWorldLocation (Variables|Default|GetPlayerPoint)) "0, 0, 0")
    (Input|RemoveMappingContext _returnvalue_2 "/Game/Inputs/IMC_PlayerMovement.IMC_PlayerMovement" "(bIgnoreAllPressedKeysUntilRelease=True,bForceImmediately=False,bNotifyUserSettings=False)")
    (Input|AddMappingContext _returnvalue_2 "/Game/Inputs/IMC_PlayerOnCashier.IMC_PlayerOnCashier" 0 "(bIgnoreAllPressedKeysUntilRelease=True,bForceImmediately=False,bNotifyUserSettings=False)")))

(event Input|KeyboardEvents|X
  (params (Key :type Key%20Structure :default "None"))
  (bind _returnvalue (Game|GetPlayerController 0))
  (bind _returnvalue_2 (PlayerController|LocalPlayerSubsystems|GetEnhancedInputLocalPlayerSubsystem _returnvalue))
  (:Pressed
    (Input|RemoveMappingContext _returnvalue_2 "/Game/Inputs/IMC_PlayerOnCashier.IMC_PlayerOnCashier" "(bIgnoreAllPressedKeysUntilRelease=True,bForceImmediately=False,bNotifyUserSettings=False)")
    (Input|AddMappingContext _returnvalue_2 "/Game/Inputs/IMC_PlayerMovement.IMC_PlayerMovement" 0 "(bIgnoreAllPressedKeysUntilRelease=True,bForceImmediately=False,bNotifyUserSettings=False)")
    (Variables|Default|SetIsPlayerOnRadius? false)))

(fn ConstructionScript)