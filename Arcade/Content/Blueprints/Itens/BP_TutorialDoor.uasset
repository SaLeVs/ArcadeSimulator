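; Tutorial door actor that swings open and shut by yawing the whole actor.
; SetDoorRotation and ResetDoorRotation offset the Door component's world yaw by 140 degrees in opposite directions and apply it with SetActorRotation.
; Each passes the target through a single RInterpTo with a large fixed delta time, so the door snaps rather than animates.
; Both offsets are relative to the current rotation, so repeated calls accumulate.
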(fn ConstructionScript)

(fn SetDoorRotation
  (bind _door (Variables|Default|GetDoor))
  (bind _returnvalue (Transformation|GetWorldRotation _door))
  (bind _returnvalue_2 (+ (.yaw _returnvalue) -1.4e+02))
  (bind _returnvalue_3 (Math|Interpolation|RInterpTo (Math|Rotator|MakeRotator (.roll _returnvalue) (.pitch _returnvalue) (.yaw _returnvalue)) (Math|Rotator|MakeRotator (.roll _returnvalue) (.pitch _returnvalue) _returnvalue_2) 1e+01 1e+01))
  (Transformation|SetActorRotation (Math|Rotator|MakeRotator (.roll _returnvalue_3) (.pitch _returnvalue_3) (.yaw _returnvalue_3))))

(fn ResetDoorRotation
  (bind _door (Variables|Default|GetDoor))
  (bind _returnvalue (Transformation|GetWorldRotation _door))
  (bind _returnvalue_2 (+ (.yaw _returnvalue) 1.4e+02))
  (bind _returnvalue_3 (Math|Interpolation|RInterpTo (Math|Rotator|MakeRotator (.roll _returnvalue) (.pitch _returnvalue) (.yaw _returnvalue)) (Math|Rotator|MakeRotator (.roll _returnvalue) (.pitch _returnvalue) _returnvalue_2) 1e+01 1e+01))
  (Transformation|SetActorRotation (Math|Rotator|MakeRotator (.roll _returnvalue_3) (.pitch _returnvalue_3) (.yaw _returnvalue_3))))