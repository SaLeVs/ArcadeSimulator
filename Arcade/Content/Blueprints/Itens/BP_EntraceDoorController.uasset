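; Entrance door controller that rotates a linked tutorial door as NPCs enter and leave its Box trigger.
; Overlap begin and end events raise or lower a count of BP_NPCMaster actors and print it for debugging.
; Each event branches on that count to enter or reset its own DoOnce gate, which guards the call to set or reset the door's rotation.
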(event OnComponentBeginOverlap(Box)
  (params (OverlappedComponent :type Primitive%20Component%20Object%20Reference) (OtherActor :type Actor%20Object%20Reference) (OtherComp :type Primitive%20Component%20Object%20Reference) (OtherBodyIndex :type Integer) (bFromSweep :type Boolean) (SweepResult :type Hit%20Result%20Structure%20%28by%20ref%29))
  (bind _npccount (Variables|Default|GetnpcCount))
  (Utilities|Casting|CastToBP_NPCMaster OtherActor)
  (Math|Integer|IncrementInt (Variables|Default|GetnpcCount)
    (:%20%20
      (Development|PrintString (Utilities|String|ToString(Integer) _npccount))
      (if (<= _npccount 0)
        (goto _label Reset)
        (else
          (Utilities|FlowControl|DoOnce false :!label _label
            (:Completed
              (Default|SetDoorRotation (Variables|Default|GetbpTutorialDoor)))))))))

(event OnComponentEndOverlap(Box)
  (params (OverlappedComponent :type Primitive%20Component%20Object%20Reference) (OtherActor :type Actor%20Object%20Reference) (OtherComp :type Primitive%20Component%20Object%20Reference) (OtherBodyIndex :type Integer))
  (bind _npccount (Variables|Default|GetnpcCount))
  (Utilities|Casting|CastToBP_NPCMaster OtherActor)
  (Math|Integer|DecrementInt (Variables|Default|GetnpcCount)
    (:%20%20
      (Development|PrintString (Utilities|String|ToString(Integer) _npccount))
      (if (<= _npccount 0)
        (goto _label Reset)
        (else
          (Utilities|FlowControl|DoOnce false :!label _label
            (:Completed
              (Default|ResetDoorRotation (Variables|Default|GetbpTutorialDoor)))))))))

(fn ConstructionScript)