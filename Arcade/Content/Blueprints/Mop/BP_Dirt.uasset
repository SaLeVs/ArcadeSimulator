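; BP_Dirt is a dirt actor that fades out as it is mopped and then removes itself.
; Each OnMopClear call lowers DirtValue by a fixed step and writes it to the Opacity parameter of the mesh material.
; A DoOnce creates and assigns the dynamic material instance on the first clear, and DestroyDirt destroys the actor once the value is nearly zero.
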(event Custom|OnMopClear
  (if (> (Variables|Default|GetdirtValue) 0.0)
    (Utilities|FlowControl|Sequence ; Can Clear This
      (:then_0
        (Utilities|FlowControl|DoOnce false ; Change the Mat (once)
          (:Completed
            (bind _returnvalue (Rendering|Material|CreateDynamicMaterialInstance "/Game/Materials/DirtMaterial.DirtMaterial" "Opacity" "None" :!class /Script/Engine.KismetMaterialLibrary))
            (bind _output_get (Variables|Default|SetMyDirtMaterial _returnvalue))
            (Rendering|Material|SetMaterial (Variables|Default|GetDirtMesh) 0 _output_get))))
      (:then_1
        (bind _output_get_2 (Variables|Default|SetdirtValue (- (Variables|Default|GetdirtValue) 0.1))) ; Change Opacity
        (Rendering|Material|SetScalarParameterValue (Variables|Default|GetMyDirtMaterial) "Opacity" _output_get_2 :!class /Script/Engine.MaterialInstanceDynamic)
        (if (<= (Variables|Default|GetdirtValue) 0.01)
          (CallFunction|DestroyDirt) ; Last input
        )))
    (else
      (CallFunction|DestroyDirt))))

(event Custom|DestroyDirt
  (Actor|DestroyActor) ; Finished Clear
)

(fn ConstructionScript)