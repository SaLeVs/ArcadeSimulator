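; BP_Mop is a mop the player picks up through Interact, uses and drops.
; Pickup disables physics and snaps it to the player's MopPoint if the hand is free; every Interact also binds to BPCMopSystem's use and drop events.
; Use lowers or raises the mop by a fixed offset, with a downward debug trace whose result is unused.
; Drop detaches it, frees the hand and restores physics.
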(event Custom|MopUse
  (params (isUsingMop :type Boolean))
  (if isUsingMop
    (Collision|LineTraceByChannel (Transformation|GetActorLocation) (- (Transformation|GetActorLocation) "0.000000,0.000000,500.000000") "TraceTypeQuery1" false 0 "ForDuration")
    (Transformation|SetActorLocation (- (Transformation|GetActorLocation) "0.000000,0.000000,70.000000") false false)
    (else
      (Transformation|SetActorLocation (- (Transformation|GetActorLocation) "0.000000,0.000000,-70.000000") false false))))

(event Custom|MopDrop
  (Transformation|DetachFromActor "KeepWorld" "KeepWorld" "KeepWorld")
  (Variables|/Game/Blueprints/Player/BP_Player.BP_Player_C|SethaveItemOnHand (stale EventInteract bpPlayer) false)
  (Physics|SetSimulatePhysics (Variables|Default|GetCube) true)
  (Physics|SetSimulatePhysics (Variables|Default|GetBox) true))

(event EventInteract
  (params (bpPlayer :type BP%20Player%20Object%20Reference))
  (bind _bpc_mopsystem (Variables|/Game/Blueprints/Player/BP_Player.BP_Player_C|GetBPC_MopSystem bpPlayer))
  (Utilities|FlowControl|Sequence
    (:then_0
      (if (not (Variables|/Game/Blueprints/Player/BP_Player.BP_Player_C|GethaveItemOnHand bpPlayer))
        (Variables|/Game/Blueprints/Player/BP_Player.BP_Player_C|SethaveItemOnHand bpPlayer true)
        (Physics|SetSimulatePhysics (Variables|Default|GetCube) false)
        (Physics|SetSimulatePhysics (Variables|Default|GetBox) false)
        (Transformation|AttachComponentToComponent (Variables|/Game/Blueprints/Player/BP_Player.BP_Player_C|GetMopPoint bpPlayer) "None" "SnapToTarget" "SnapToTarget" "KeepRelative" true)
        (Development|PrintString "Hello")))
    (:then_1
      (EventDispatchers|BindEventtoOnMopUse _bpc_mopsystem (delegate Custom|MopUse)))
    (:then_2
      (EventDispatchers|BindEventtoOnDropMop _bpc_mopsystem (delegate Custom|MopDrop)))))

(fn ConstructionScript)

(fn NewFunction
  (return 0))