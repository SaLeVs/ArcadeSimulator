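; BP_BucketOfWater is a bucket the player picks up with a hold interaction and carries at their MopPoint.
; Pickup registers the held item, disables mesh physics, snaps the bucket to that point and adds the IMC_Mop input context.
; It binds to the player mop system's OnDropMop event, which detaches the bucket, clears the held item, restores physics and removes the input context.
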(event Custom|MopDrop
  (Transformation|DetachFromActor "KeepWorld" "KeepWorld" "KeepWorld")
  (Default|RemoveItemonHand (Variables|Default|GetBP_Player))
  (CallFunction|TogglePhysic true) ; Turn On Phyisic
  (Input|RemoveMappingContext (PlayerController|LocalPlayerSubsystems|GetEnhancedInputLocalPlayerSubsystem (Game|GetPlayerController 0)) "/Game/Inputs/InputsMop/IMC_Mop.IMC_Mop" "(bIgnoreAllPressedKeysUntilRelease=True,bForceImmediately=False,bNotifyUserSettings=False)"))

(event EventInteractHold
  (params (bpPlayer :type BP%20Player%20Object%20Reference))
  (Variables|Default|SetBP_Player bpPlayer)
  (Utilities|FlowControl|Sequence
    (:then_0
      (Default|AddItemonHand (Variables|Default|GetBP_Player))
      (CallFunction|TogglePhysic false))
    (:then_1
      (Transformation|AttachComponentToComponent (Variables|/Game/Blueprints/Player/BP_Player.BP_Player_C|GetMopPoint (Variables|Default|GetBP_Player)) "None" "SnapToTarget" "SnapToTarget" "KeepRelative" true)
      (Input|AddMappingContext (PlayerController|LocalPlayerSubsystems|GetEnhancedInputLocalPlayerSubsystem (Game|GetPlayerController 0)) "/Game/Inputs/InputsMop/IMC_Mop.IMC_Mop" 0 "(bIgnoreAllPressedKeysUntilRelease=True,bForceImmediately=False,bNotifyUserSettings=False)"))
    (:then_2
      (EventDispatchers|BindEventtoOnDropMop (Variables|/Game/Blueprints/Player/BP_Player.BP_Player_C|GetBPC_MopSystem (Variables|Default|GetBP_Player)) (delegate Custom|MopDrop)) ; Subscribe to Event
    )))

(fn ConstructionScript)

(fn TogglePhysic
  (params (toggle :type Boolean))
  (bind _bucketmesh (Variables|Default|GetBucketMesh))
  (if toggle
    (Physics|SetSimulatePhysics _bucketmesh true)
    (else
      (Physics|SetSimulatePhysics _bucketmesh false))))