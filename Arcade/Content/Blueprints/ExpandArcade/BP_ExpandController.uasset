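; BP_ExpandController grows an arcade map in steps by moving a wall.
; ExpandMap teleports WallToMove to the location of the next actor in PoinsToMoveWall with zero rotation, increments ExpandedTimes and returns true.
; It returns false once every point is used.
; BeginPlay is empty, and the delayed debug test calls in the event graph are disconnected.
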(event EventBeginPlay)

(fn ConstructionScript)

(fn ExpandMap
  (if (>= (Variables|Default|GetexpandedTimes) (Utilities|Array|Length (Variables|Default|GetpoinsToMoveWall)))
    (return false) ; Couldnt Expand
    (else
      (Transformation|Teleport (Variables|Default|GetWallToMove) (.location (Transformation|GetActorTransform (Utilities|Array|Get(acopy) (Variables|Default|GetpoinsToMoveWall) (Variables|Default|GetexpandedTimes)))) "0, 0, 0")
      (Variables|Default|SetexpandedTimes (+ (Variables|Default|GetexpandedTimes) 1))
      (return true) ; Expanded Done!
    )))